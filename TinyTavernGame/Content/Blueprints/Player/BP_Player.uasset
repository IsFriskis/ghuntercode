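; Player Blueprint handling audio listener setup, position sharing, area ambience, footsteps and impact feedback.
; Tick writes the capsule position to Niagara and material parameter collections and re-sets the ambient Niagara asset from MapAreaID.
; CE_Dust triggers MetaSound-style footsteps by floor type.
; CE_ImpactDie combines an impact actor, post-process flash, camera shake and brief hit-stop via custom time dilation.
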(event `self.ReceiveBeginPlay`
  ;[0 1 0.1185] Begin Play
  (`PlayerController.SetAudioListenerAttenuationOverride` (`GameplayStatics.GetPlayerController` 0) (`self.Mesh`) (0.0 0.0 0.0))
  (`ActorComponent.Activate` (`self.PlayerPointLight`) false))

(event `self.ReceiveTick`
  (params (DeltaSeconds :type "Float (single-precision)"))
  (bind _mapareaid (`self.MapAreaID`))
  ;[1 0.8538 0] Tick
  (bind _returnvalue (`NiagaraFunctionLibrary.GetNiagaraParameterCollection` "/Game/Assets/Enviroment/VFX/Arañitas/NPC_PlayerPosition.NPC_PlayerPosition"))
  (`NiagaraParameterCollectionInstance.SetVectorParameter` _returnvalue "PlayerPosition" (- (`SceneComponent.K2_GetComponentLocation` (`self.CapsuleComponent`)) (0.0 0.0 35.0)))
  (`KismetMaterialLibrary.SetVectorParameterValue` "/Game/Assets/Enviroment/Materials/MPC_PlayerInfo.MPC_PlayerInfo" "PlayerPos" (`KismetMathLibrary.Conv_VectorToLinearColor` (`SceneComponent.K2_GetComponentLocation` (`self.CapsuleComponent`))))
  ;[1 1 1] Select VFX for ZoneMap
  (if (== _mapareaid 0)
    (`NiagaraComponent.SetAsset` (`self.NiagaraComponent`) "/Game/Assets/Enviroment/VFX/VFXVientoHojas/NS_Wind.NS_Wind" true)
    (elif (== _mapareaid 1)
      (`NiagaraComponent.SetAsset` (`self.NiagaraComponent`) "/Game/Assets/Enviroment/VFX/VFXEsporas/NS_ambience_spores.NS_ambience_spores" true)
      (elif (== _mapareaid 2)
        (`NiagaraComponent.SetAsset` (`self.NiagaraComponent`) "/Game/Assets/Enviroment/VFX/VFXVientoHojas/NS_Wind.NS_Wind" true)))))

(event `CE_Dust`
  (params (FloorIndex :type Integer))
  (bind _ms_footsteps (`self.MS_FootSteps`))
  ;[1 1 1] Dust
  (`AudioParameterControllerInterface.SetTriggerParameter` _ms_footsteps "Execute")
  (`AudioParameterControllerInterface.SetIntParameter` _ms_footsteps "TypeOfFloor" FloorIndex))

(event `CE_ImpactDie`
  (bind (_returnvalue_location _returnvalue_rotation) (`KismetMathLibrary.BreakTransform` (`self.GetTransform`)))
  ;[1 0.03768 0] Impact Die
  (`|ExecutionSequence`
    (:`then_0`
      (set `PostProcessComponent.BlendWeight` 1.0 (`self.PostProcess`))
      (`|SpawnActorFromClass` "/Game/Blueprints/Character/Commons/BP_ImpactNS.BP_ImpactNS_C" (`KismetMathLibrary.MakeTransform` _returnvalue_location _returnvalue_rotation) "Undefined" "MultiplyWithRoot" null null)
      (`KismetSystemLibrary.Delay` 0.1)
      (set `PostProcessComponent.BlendWeight` 0.0 (`self.PostProcess`)))
    (:`then_2`
      (`PlayerController.ClientStartCameraShake` :`self` (`GameplayStatics.GetPlayerController` 0) :`Shake` "/Game/Blueprints/Character/Commons/BP_HitCameraShake.BP_HitCameraShake_C" :`PlaySpace` "World")
      (set `self.CustomTimeDilation` 0.0)
      (`KismetSystemLibrary.Delay` 0.25)
      (set `self.CustomTimeDilation` 1.0))))

(fn `UserConstructionScript`)