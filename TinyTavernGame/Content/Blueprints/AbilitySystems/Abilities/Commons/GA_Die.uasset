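; Gameplay ability that handles death for the player and other combat characters.
; It applies GE_Die and tags, disables movement and plays the CombatInterface death montage with camera shake and a brief time-dilation freeze on the player.
; Player deaths turn off capsule collision and, on montage blend-out, apply inventory penalties, show WBP_Death and pause the game.
; Other deaths call CEImpactDie on BP_Player and simply end the ability after blend-out.
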(event `self.K2_ActivateAbility`
  (bind _returnvalue (`self.GetAvatarActorFromActorInfo`))
  (bind _returnvalue_2 (`GameplayStatics.GetPlayerController` 0))
  (`|ExecutionSequence`
    (:`then_0`
      (bind _asplayer_character (cast `PlayerCharacter` (`self.GetAvatarActorFromActorInfo`))
        (:`then`
          (bind _output_get (set `self. Player` _asplayer_character))
          (bind _capsulecomponent (`Character.CapsuleComponent` _output_get))
          (`PrimitiveComponent.SetCollisionEnabled` _capsulecomponent "NoCollision")
          (`PrimitiveComponent.SetCollisionObjectType` _capsulecomponent "ECC_Camera"))
        (:`CastFailed`
          (bind _asbp_player (cast `/Game/Blueprints/Player/BP_Player` (`GameplayStatics.GetPlayerPawn` 0)))
          (`/Game/Blueprints/Player/BP_Player.CE_ImpactDie` _asbp_player))))
    (:`then_1`
      (bind _returnvalue_3 (`self.BP_ApplyGameplayEffectToOwner` "/Game/Blueprints/AbilitySystems/Effects/Commons/GE_Die.GE_Die_C"))
      (set `self.Active GE_HitReact` _returnvalue_3)
      (`AbilitySystemBlueprintLibrary.AddLooseGameplayTags` (`self.GetAvatarActorFromActorInfo`) (`self.Tag Container`))
      ;[1 1 1] Disable Movement
      (bind _ascharacter (cast `Character` _returnvalue))
      (`CharacterMovementComponent.DisableMovement` (`Character.CharacterMovement` _ascharacter))
      ;[1 1 1] Get Die Animation
      (bind _ascombat_interface (cast `CombatInterface` _returnvalue))
      (bind _returnvalue_4 (`CombatInterface.GetDieMontage` _ascombat_interface))
      (`AbilityTask_PlayMontageAndWait.CreatePlayMontageAndWaitProxy` "None" _returnvalue_4
        (:`then`
          ;[1 1 1] Pasar a C
          (`PlayerController.ClientStartCameraShake` :`self` (`GameplayStatics.GetPlayerController` 0) :`Shake` "/Game/Blueprints/Character/Commons/BP_HitCameraShake.BP_HitCameraShake_C" :`PlaySpace` "World")
          (`KismetSystemLibrary.Delay` 0.1)
          (set `Actor.CustomTimeDilation` 0.0 (`self. Player`))
          (`KismetSystemLibrary.Delay` 0.1)
          (set `Actor.CustomTimeDilation` 1.0 (`self. Player`)))
        (:`OnBlendOut`
          ;[1 1 1] If Player Dies, Show game over, remove Extra Plates and Remove a percentage of ammunition
          (bind _asplayer_character_2 (cast `PlayerCharacter` (`self.GetAvatarActorFromActorInfo`))
            (:`then`
              (`PlayerController.K2_ClientPlayForceFeedback` (`GameplayStatics.GetPlayerController` 0) "/Game/Blueprints/Inputs/ForceFeedback/FF_DeathVibration.FF_DeathVibration" "None" false false false)
              (`self.CE_PlayerInventory`)
              (`PrimitiveComponent.SetCollisionEnabled` (`Character.CapsuleComponent` _asplayer_character_2) "NoCollision")
              (bind _returnvalue_5 (`|CreateWidget` "/Game/Blueprints/UI/Menus/GameOver/WBP_Death.WBP_Death_C" _returnvalue_2))
              (`UserWidget.AddToViewport` _returnvalue_5 0)
              (`WidgetBlueprintLibrary.SetInputMode_UIOnlyEx` _returnvalue_2 null)
              (set `PlayerController.bShowMouseCursor` true _returnvalue_2)
              (`GameplayStatics.SetGamePaused` true)
              (`self.BP_RemoveGameplayEffectFromOwnerWithHandle` (`self.Active GE_HitReact`))
              (`self.K2_EndAbility`))
            (:`CastFailed`
              (`self.BP_RemoveGameplayEffectFromOwnerWithHandle` (`self.Active GE_HitReact`))
              (`self.K2_EndAbility`))))))))

(event `CE_PlayerInventory`
  (bind _astt_game_instance (cast `TT_GameInstance` (`GameplayStatics.GetGameInstance`)))
  (`TT_GameInstance.DeathConsequences` _astt_game_instance 0.15))