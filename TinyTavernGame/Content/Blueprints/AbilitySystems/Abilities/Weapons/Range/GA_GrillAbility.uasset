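; Gameplay ability that fires the player's shotgun-style grill weapon, ending immediately when out of ammunition.
; Each shot applies a cooldown, plays sounds and a firing montage with rumble and camera shake, then runs a quad-collision task as the hitbox.
; Hit enemies get a VFX cue and SetByCaller grill damage, plus a burn effect when the triggering event's magnitude is non-zero.
; Drunk enemies take multiplied grill and burn damage.
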(event `self.K2_ActivateAbilityFromEvent`
  (params (EventData :type "GameplayEventData Structure (by ref)"))
  (bind _returnvalue (`self.MakeOutgoingGameplayEffectSpec` "/Game/Blueprints/AbilitySystems/Effects/Weapons/Ranged/GE_BurnEffect.GE_BurnEffect_C"))
  (bind _returnvalue_2 (`self.MakeOutgoingGameplayEffectSpec` "/Game/Blueprints/AbilitySystems/Effects/Weapons/Ranged/GE_GrillDamage.GE_GrillDamage_C"))
  (bind _returnvalue_3 (`self.GetAvatarActorFromActorInfo`))
  (bind _returnvalue_4 (`GameplayStatics.GetPlayerController` 0))
  (bind _returnvalue_5 (`Actor.K2_GetActorLocation` _returnvalue_3))
  (bind _returnvalue_6 (!= (`.EventMagnitude` (break `GameplayEventData` EventData)) 0.0))
  (bind _asplayer_character (cast `PlayerCharacter` _returnvalue_3))
  (bind _returnvalue_7 (`self.NoAmmunition` _asplayer_character))
  (if _returnvalue_7
    (`self.K2_EndAbility`)
    (else
      (`GameplayStatics.PlaySoundAtLocation` "/Game/Assets/Music/GrillSFX/S_grill_shotgun.S_grill_shotgun" _returnvalue_5 (struct) 1.0 1.0 0.0 null null null null)
      (`GameplayStatics.PlaySoundAtLocation` "/Game/Assets/Music/GrillSFX/S_GrillShoot.S_GrillShoot" _returnvalue_5 (struct) 1.0 1.0 0.0 null null null null)
      (`self.ApplyCooldownEffect` (`self.CooldownBetweenShots`))
      (`AbilityTask_PlayMontageAndWait.CreatePlayMontageAndWaitProxy` "SingleShot" (`self.FiringAnimation`) 1.0 "Default" false
        (:`then`
          (`PlayerController.K2_ClientPlayForceFeedback` _returnvalue_4 "/Game/Blueprints/Inputs/ForceFeedback/FF_GrillVibration.FF_GrillVibration" "None" false false false)
          (`PlayerController.ClientStartCameraShake` :`self` _returnvalue_4 :`Shake` "/Game/Blueprints/Character/Commons/BP_HitCameraShake.BP_HitCameraShake_C" :`Scale` 0.33 :`PlaySpace` "World")
          (bind (_asynctaskproxy _hits) (`AbilityTask_QuadCollisionCheck.QuadCollisionAbilityTask` "GrillCollision" (`Actor.K2_GetActorLocation` _returnvalue_3) (`self.Range`) (`self.HitboxAngle`) (`self.Width`) (`|MakeArray` null :!type "Actor Class Reference"))
            (:`OnCompleted`
              (`self.K2_EndAbility`))
            (:`OnHit`
              (bind _asenemy_base (cast `EnemyBase` _hits))
              (bind _output_get (set `self.As Enemy Base` _asenemy_base))
              (`GameplayCueFunctionLibrary.ExecuteGameplayCueOnActor` _output_get (struct :`TagName` "GameplayCue.Enemy.GrillVFX") (`AbilitySystemBlueprintLibrary.MakeGameplayCueParameters` 0.0))
              (bind _returnvalue_8 (`AbilitySystemBlueprintLibrary.GetAbilitySystemComponent` _output_get))
              (if (`BlueprintGameplayTagLibrary.HasTag` (`GameplayTagAssetInterface.GetOwnedGameplayTags` _returnvalue_8) (struct :`TagName` "States.Drunk") true)
                (bind _returnvalue_9 (`AbilitySystemBlueprintLibrary.AssignTagSetByCallerMagnitude` _returnvalue_2 (struct :`TagName` "States.Cook.Grilled") (* (`self.DrunkDamageMultiplier`) (`self.WeaponDamage`))))
                (`AbilitySystemComponent.BP_ApplyGameplayEffectSpecToTarget` _returnvalue_8 _returnvalue_9 _returnvalue_8)
                (if _returnvalue_6
                  (bind _returnvalue_10 (`AbilitySystemBlueprintLibrary.AssignTagSetByCallerMagnitude` _returnvalue (struct :`TagName` "States.Cook.Grilled") (* (`self.DrunkDamageMultiplier`) (`self.BurnDamagePerTick`))))
                  (`AbilitySystemComponent.BP_ApplyGameplayEffectSpecToTarget` _returnvalue_8 _returnvalue_10 _returnvalue_8))
                (else
                  (bind _returnvalue_11 (`AbilitySystemBlueprintLibrary.AssignTagSetByCallerMagnitude` _returnvalue_2 (struct :`TagName` "States.Cook.Grilled") (`self.WeaponDamage`)))
                  (`AbilitySystemComponent.BP_ApplyGameplayEffectSpecToTarget` _returnvalue_8 _returnvalue_11 _returnvalue_8)
                  (if _returnvalue_6
                    (bind _returnvalue_12 (`AbilitySystemBlueprintLibrary.AssignTagSetByCallerMagnitude` _returnvalue (struct :`TagName` "States.Cook.Grilled") (`self.BurnDamagePerTick`)))
                    (`AbilitySystemComponent.BP_ApplyGameplayEffectSpecToTarget` _returnvalue_8 _returnvalue_12 _returnvalue_8)))))))))))