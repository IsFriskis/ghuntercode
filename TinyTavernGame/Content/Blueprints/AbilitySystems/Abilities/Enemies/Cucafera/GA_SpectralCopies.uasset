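; Enemy gameplay ability that spawns spectral ghost copies of the premium Cucafera around the caster.
; It plays the Campaneo montage, then after a short delay emits smoke and sound and spawns ghosts at random reachable navmesh points nearby.
; When the caster is a premium Cucafera, each ghost is registered in its ally array and parented to it.
; On ability end, it swaps loose gameplay tags to make the caster flee desperately.
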(event `self.K2_ActivateAbility`
  (bind (_returnvalue_roll _returnvalue_pitch _returnvalue_yaw) (`KismetMathLibrary.BreakRotator` (`KismetMathLibrary.RandomRotator` false)))
  (bind _as_enemy_base (`self.As Enemy Base`))
  (bind _mothercucafera (`self.MotherCucafera`))
  (bind _as_enemy_base_2 (`self.As Enemy Base`))
  (bind _returnvalue (`Actor.K2_GetActorLocation` _as_enemy_base))
  (bind (_randomlocation _returnvalue_2) (`NavigationSystemV1.K2_GetRandomReachablePointInRadius` (`Actor.K2_GetActorLocation` (`self.As Enemy Base`)) 600.0 (`self.Nav Data`) null))
  (bind _asenemy_base (cast `EnemyBase` (`self.GetOwningActorFromActorInfo`)))
  (set `self.As Enemy Base` _asenemy_base)
  (if (== (`GameplayStatics.GetObjectClass` _as_enemy_base_2) "/Game/Blueprints/Character/Enemies/Cucafera/BP_CucaferaPremium.BP_CucaferaPremium_C")
    (bind _asenemy_cucafera (cast `EnemyCucafera` _as_enemy_base_2))
    (set `self.MotherCucafera` _asenemy_cucafera))
  (`AbilityTask_PlayMontageAndWait.CreatePlayMontageAndWaitProxy` "None" "/Game/Assets/Enemies/Cucafera/Anims/AM_Cucafera_Campaneo.AM_Cucafera_Campaneo" 1.6
    (:`then`
      (`AbilityTask_Delay.DelayTask` "None" 0.2
        (:`OnCompleted`
          (`GameplayStatics.PlaySoundAtLocation` "/Game/Assets/Music/Enemy/Cucafera/S_CucaferaSmoke.S_CucaferaSmoke" _returnvalue (struct) 1.0 1.0 0.0 null null null null)
          (`NiagaraFunctionLibrary.SpawnSystemAtLocation` "/Game/Assets/Enemies/Cucafera/Variantes/Spectral/NS_CucaferaSmoke.NS_CucaferaSmoke" _returnvalue (`Actor.K2_GetActorRotation` _as_enemy_base))
          (if _returnvalue_2
            (while (!= (`self.SpawnedEnemies`) (`self.Ghosts`))
              (bind _returnvalue_3 (`|SpawnActorFromClass` "/Game/Blueprints/Character/Enemies/Cucafera/BP_CucaferaPremiunGhost.BP_CucaferaPremiunGhost_C" (`KismetMathLibrary.MakeTransform` (`KismetMathLibrary.MakeVector` (.x _randomlocation) (.y _randomlocation) (.z (.location (`Actor.GetTransform` _asenemy_base)))) (`KismetMathLibrary.MakeRotator` 0.0 0.0 _returnvalue_yaw)) "AdjustIfPossibleButAlwaysSpawn" "MultiplyWithRoot" null null))
              (set `/Game/Blueprints/Character/Enemies/Cucafera/BP_CucaferaPremium.FirstHit` false _returnvalue_3)
              (set `/Game/Blueprints/Character/Enemies/Cucafera/BP_CucaferaPremiunGhost.Ghost_Num` (`self.Ghosts`) _returnvalue_3)
              (set `self.SpawnedEnemies` (+ (`self.SpawnedEnemies`) 1))
              (`/Engine/EditorBlueprintResources/StandardMacros.IsValid` _mothercucafera
                (:`Is Valid`
                  (`KismetArrayLibrary.Array_Add` (`EnemyCucafera.GhostAlliesArray` _mothercucafera) _returnvalue_3)
                  (bind _asbp_cucafera_premium (cast `/Game/Blueprints/Character/Enemies/Cucafera/BP_CucaferaPremium` _mothercucafera))
                  (`/Game/Blueprints/Character/Enemies/Cucafera/BP_CucaferaPremiunGhost.SetParent` _returnvalue_3 _asbp_cucafera_premium)
                  (`self.K2_EndAbility`))))
            ;[1 0.03003 0] It is necesarry to have this delay until next tick otherwise the ability wont stop
            (`KismetSystemLibrary.DelayUntilNextTick`)
            (`self.K2_EndAbility`)
            (else
              (`self.K2_EndAbility`))))))))

(event `self.K2_OnEndAbility`
  (params (bWasCancelled :type Boolean))
  ;[1 1 1] Add DesperatelyFlee and EndAbility
  (`AbilitySystemBlueprintLibrary.AddLooseGameplayTags` (`self.GetOwningActorFromActorInfo`) (`self.Gameplay Tags_0`))
  (`AbilitySystemBlueprintLibrary.RemoveLooseGameplayTags` (`self.As Enemy Base`) (`self.Gameplay Tags`))
  (`self.K2_EndAbility`))