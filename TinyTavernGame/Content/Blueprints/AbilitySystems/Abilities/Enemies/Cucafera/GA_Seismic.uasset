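; Gameplay ability for the seismic attack of the Cucafera enemy, fired as its Campaneo montage blends out.
; Four parallel SweepArcCollisions tasks start from front and back mesh sockets, each spawning a Niagara shockwave.
; A player hit applies damage, deactivates that arc's VFX and ends its named task.
; Any arc completing, interrupting or cancelling removes gameplay tags and ends the whole ability.
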(event `self.K2_ActivateAbility`
  (bind _mesh (`Character.Mesh` (`self.Enemy`)))
  (bind _mesh_2 (`Character.Mesh` (`self.Enemy`)))
  (bind _mesh_3 (`Character.Mesh` (`self.Enemy`)))
  (bind _mesh_4 (`Character.Mesh` (`self.Enemy`)))
  (bind _asenemy_cucafera (cast `EnemyCucafera` (`self.GetOwningActorFromActorInfo`)))
  (set `self.Enemy` _asenemy_cucafera)
  (bind _asbp_cucafera_seismic (cast `/Game/Blueprints/Character/Enemies/Cucafera/BP_CucaferaSeismic` (`self.Enemy`)))
  (`AbilitySystemBlueprintLibrary.RemoveLooseGameplayTags` _asbp_cucafera_seismic (`self.Gameplay Tags`))
  (`AbilityTask_PlayMontageAndWait.CreatePlayMontageAndWaitProxy` "None" "/Game/Assets/Enemies/Cucafera/Anims/AM_Cucafera_Campaneo.AM_Cucafera_Campaneo"
    (:`OnBlendOut`
      (`|ExecutionSequence`
        (:`then_0`
          (bind (_asynctaskproxy _actorhit) (`AbilityTask_Sweep_ArcCollision.SweepArcCollisions` "Arc1" "FrontPoint1" (`self.Arch Wide`) (`self.Left Angle`) (`self.Right Angle`) (`self.Distance`) (`self.Speed`))
            (:`then`
              (bind _returnvalue (`NiagaraFunctionLibrary.SpawnSystemAtLocation` "/Game/Assets/Enemies/Cucafera/NS_CucaferaSysmic.NS_CucaferaSysmic" (`SceneComponent.GetSocketLocation` _mesh_2 "FrontPoint1") (`SceneComponent.GetSocketRotation` _mesh_2 "FrontPoint1")))
              (set `self.Vfx1` _returnvalue))
            (:`OnCompleted`
              (`AbilitySystemBlueprintLibrary.RemoveLooseGameplayTags` (`self.Enemy`) (`self.Gameplay Tags`) :!label _label)
              (`self.K2_EndAbility`))
            (:`OnInterrupted`
              (goto _label))
            (:`OnCancelled`
              (goto _label))
            (:`OnHit`
              (bind _asplayer_character (cast `PlayerCharacter` _actorhit))
              (bind _returnvalue_2 (`AbilitySystemBlueprintLibrary.GetAbilitySystemComponent` _asplayer_character))
              (`AbilitySystemComponent.BP_ApplyGameplayEffectToTarget` :`self` _returnvalue_2 :`GameplayEffectClass` "/Game/Blueprints/AbilitySystems/Effects/Damage/GE_Damage_1.GE_Damage_1_C" :`Target` _returnvalue_2)
              (`ActorComponent.Deactivate` (`self.Vfx1`))
              (`self.EndTaskByInstanceName` "Arc1"))))
        (:`then_1`
          (bind (_asynctaskproxy_2 _actorhit_2) (`AbilityTask_Sweep_ArcCollision.SweepArcCollisions` "Arc2" "FrontPoint2" (`self.Arch Wide`) (`self.Left Angle`) (`self.Right Angle`) (`self.Distance`) (`self.Speed`))
            (:`then`
              (bind _returnvalue_3 (`NiagaraFunctionLibrary.SpawnSystemAtLocation` "/Game/Assets/Enemies/Cucafera/NS_CucaferaSysmic.NS_CucaferaSysmic" (`SceneComponent.GetSocketLocation` _mesh_3 "FrontPoint2") (`SceneComponent.GetSocketRotation` _mesh_3 "FrontPoint2")))
              (set `self.Vfx2` _returnvalue_3))
            (:`OnCompleted`
              (`AbilitySystemBlueprintLibrary.RemoveLooseGameplayTags` (`self.Enemy`) (`self.Gameplay Tags`) :!label _label_2)
              (`self.K2_EndAbility`))
            (:`OnInterrupted`
              (goto _label_2))
            (:`OnCancelled`
              (goto _label_2))
            (:`OnHit`
              (bind _asplayer_character_2 (cast `PlayerCharacter` _actorhit_2))
              (bind _returnvalue_4 (`AbilitySystemBlueprintLibrary.GetAbilitySystemComponent` _asplayer_character_2))
              (`AbilitySystemComponent.BP_ApplyGameplayEffectToTarget` :`self` _returnvalue_4 :`GameplayEffectClass` "/Game/Blueprints/AbilitySystems/Effects/Damage/GE_Damage_1.GE_Damage_1_C" :`Target` _returnvalue_4)
              (`ActorComponent.Deactivate` (`self.Vfx2`))
              (`self.EndTaskByInstanceName` "Arc2"))))
        (:`then_2`
          (bind (_asynctaskproxy_3 _actorhit_3) (`AbilityTask_Sweep_ArcCollision.SweepArcCollisions` "Arc3" "BackPoint1" (`self.Arch Wide`) (`self.Left Angle`) (`self.Right Angle`) (`self.Distance`) (`self.Speed`))
            (:`then`
              (bind _returnvalue_5 (`NiagaraFunctionLibrary.SpawnSystemAtLocation` "/Game/Assets/Enemies/Cucafera/NS_CucaferaSysmic.NS_CucaferaSysmic" (`SceneComponent.GetSocketLocation` _mesh_4 "BackPoint1") (`SceneComponent.GetSocketRotation` _mesh_4 "BackPoint1")))
              (set `self.Vfx3` _returnvalue_5))
            (:`OnCompleted`
              (`AbilitySystemBlueprintLibrary.RemoveLooseGameplayTags` (`self.Enemy`) (`self.Gameplay Tags`) :!label _label_3)
              (`self.K2_EndAbility`))
            (:`OnInterrupted`
              (goto _label_3))
            (:`OnCancelled`
              (goto _label_3))
            (:`OnHit`
              (bind _asplayer_character_3 (cast `PlayerCharacter` _actorhit_3))
              (bind _returnvalue_6 (`AbilitySystemBlueprintLibrary.GetAbilitySystemComponent` _asplayer_character_3))
              (`AbilitySystemComponent.BP_ApplyGameplayEffectToTarget` :`self` _returnvalue_6 :`GameplayEffectClass` "/Game/Blueprints/AbilitySystems/Effects/Damage/GE_Damage_1.GE_Damage_1_C" :`Target` _returnvalue_6)
              (`ActorComponent.Deactivate` (`self.Vfx3`))
              (`self.EndTaskByInstanceName` "Arc3"))))
        (:`then_3`
          (bind (_asynctaskproxy_4 _actorhit_4) (`AbilityTask_Sweep_ArcCollision.SweepArcCollisions` "Arc4" "BackPoint2" (`self.Arch Wide`) (`self.Left Angle`) (`self.Right Angle`) (`self.Distance`) (`self.Speed`))
            (:`then`
              (bind _returnvalue_7 (`NiagaraFunctionLibrary.SpawnSystemAtLocation` "/Game/Assets/Enemies/Cucafera/NS_CucaferaSysmic.NS_CucaferaSysmic" (`SceneComponent.GetSocketLocation` _mesh "BackPoint2") (`SceneComponent.GetSocketRotation` _mesh "BackPoint2")))
              (set `self.Vfx4` _returnvalue_7))
            (:`OnCompleted`
              (`AbilitySystemBlueprintLibrary.RemoveLooseGameplayTags` (`self.Enemy`) (`self.Gameplay Tags`) :!label _label_4)
              (`self.K2_EndAbility`))
            (:`OnInterrupted`
              (goto _label_4))
            (:`OnCancelled`
              (goto _label_4))
            (:`OnHit`
              (bind _asplayer_character_4 (cast `PlayerCharacter` _actorhit_4))
              (bind _returnvalue_8 (`AbilitySystemBlueprintLibrary.GetAbilitySystemComponent` _asplayer_character_4))
              (`AbilitySystemComponent.BP_ApplyGameplayEffectToTarget` :`self` _returnvalue_8 :`GameplayEffectClass` "/Game/Blueprints/AbilitySystems/Effects/Damage/GE_Damage_1.GE_Damage_1_C" :`Target` _returnvalue_8)
              (`ActorComponent.Deactivate` (`self.Vfx4`))
              (`self.EndTaskByInstanceName` "Arc4"))))))
    (:`OnInterrupted`
      (`self.K2_EndAbility` :!label _label_5))
    (:`OnCancelled`
      (goto _label_5))))

(event `self.K2_OnEndAbility`
  (params (bWasCancelled :type Boolean))
  (`AbilitySystemBlueprintLibrary.RemoveLooseGameplayTags` null (`self.Gameplay Tags_0`))
  (`self.K2_EndAbility`))