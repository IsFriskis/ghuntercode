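; Cucafera enemy Gameplay Ability that fires an oriented seismic wave from its mouth at the player.
; An aim task turns the enemy toward the player, then the sonic boom montage plays.
; On blend out, an arc collision sweep task runs from the mouth socket alongside a Niagara effect.
; A player hit applies a damage effect through the player's own ASC, stops the effect and ends the ability.
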(event `self.K2_ActivateAbility`
  (bind _mesh (`Character.Mesh` (`self.As Enemy Cucafera`)))
  (bind _asenemy_cucafera (cast `EnemyCucafera` (`self.GetOwningActorFromActorInfo`)))
  (set `self.As Enemy Cucafera` _asenemy_cucafera)
  (bind _asplayer_character (cast `PlayerCharacter` (`GameplayStatics.GetPlayerCharacter` 0)))
  (bind _output_get (set `self.As Player Character` _asplayer_character))
  (`AbilityTask_Aim.AimAbilityTask` "None" _output_get 0.2 10.0 125.0 true
    (:`OnCompleted`
      (`AbilityTask_PlayMontageAndWait.CreatePlayMontageAndWaitProxy` "None" "/Game/Assets/Enemies/Cucafera/Anims/AM_Cucafera_Sonic_Boom.AM_Cucafera_Sonic_Boom" 1.5
        (:`OnBlendOut`
          (bind (_asynctaskproxy _actorhit) (`AbilityTask_Sweep_ArcCollision.SweepArcCollisions` "None" "MouthFirePoint" (`self.Arch Wide`) (`self.Left Angle`) (`self.Right Angle`) (`self.Distance`) (`self.Speed`))
            (:`then`
              (bind _returnvalue (`NiagaraFunctionLibrary.SpawnSystemAtLocation` "/Game/Assets/Enemies/Cucafera/NS_CucaferaSysmic2.NS_CucaferaSysmic2" (`SceneComponent.GetSocketLocation` _mesh "MouthFirePoint") (`SceneComponent.GetSocketRotation` _mesh "MouthFirePoint")))
              (set `self.VfxArc` _returnvalue))
            (:`OnCompleted`
              (`self.K2_EndAbility` :!label _label))
            (:`OnInterrupted`
              (`self.K2_EndAbility` :!label _label_2))
            (:`OnCancelled`
              (goto _label_2))
            (:`OnHit`
              (bind _asplayer_character_2 (cast `PlayerCharacter` _actorhit))
              (bind _returnvalue_2 (`AbilitySystemBlueprintLibrary.GetAbilitySystemComponent` _asplayer_character_2))
              (`AbilitySystemComponent.BP_ApplyGameplayEffectToTarget` :`self` _returnvalue_2 :`GameplayEffectClass` "/Game/Blueprints/AbilitySystems/Effects/Damage/GE_Damage_2.GE_Damage_2_C" :`Target` _returnvalue_2)
              (`ActorComponent.Deactivate` (`self.VfxArc`))
              (goto _label))))
        (:`OnInterrupted`
          (`self.K2_EndAbility` :!label _label_3))
        (:`OnCancelled`
          (goto _label_3))))
    (:`OnInterrupted`
      (`self.K2_EndAbility` :!label _label_4))
    (:`OnCancelled`
      (goto _label_4))))

(event `self.K2_OnEndAbility`
  (params (bWasCancelled :type Boolean))
  (`AbilitySystemBlueprintLibrary.RemoveLooseGameplayTags` (`self.As Enemy Cucafera`) (`self.Gameplay Tags`))
  (`self.K2_EndAbility`))