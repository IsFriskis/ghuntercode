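; Gameplay ability where a Cucafera enemy screams to alert nearby jumper Cucaferas.
; It plays the scream montage and, after a short delay, shakes the player camera and runs a radius collision task.
; Each hit enemy with the Jumper tag gains a loose Alert tag, and ending the ability removes loose tags from the owner.
; The Niagara distortion effect spawn is left disconnected and never runs.
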(event `self.K2_ActivateAbility`
  (bind _asenemy_cucafera (cast `EnemyCucafera` (`self.GetOwningActorFromActorInfo`)))
  (set `self.As Enemy Cucafera` _asenemy_cucafera)
  (`AbilityTask_PlayMontageAndWait.CreatePlayMontageAndWaitProxy` "None" "/Game/Assets/Enemies/Cucafera/Anims/AM_Cucafera_Scream.AM_Cucafera_Scream" 1.0 "None" false
    (:`then`
      (`AbilityTask_Delay.DelayTask` "None" 0.5
        (:`OnCompleted`
          (`PlayerController.ClientStartCameraShake` :`self` (`GameplayStatics.GetPlayerController` 0) :`Shake` "/Game/Assets/Enemies/Cucafera/Variantes/Guardian/BP_CucaferaScream_Shake.BP_CucaferaScream_Shake_C" :`Scale` 0.7 :`PlaySpace` "World")
          (bind (_asynctaskproxy _actor) (`AbilityTask_OnCollision.OnCollisionAbilityTask` "None" (`self.SocketRot`) (0.0 0.0 0.0) 1000.0 (`self.Ignore Actors`))
            (:`OnCompleted`
              (`self.EndAbility` :!label _label))
            (:`OnInterrupted`
              (goto _label))
            (:`OnCancelled`
              (goto _label))
            (:`OnHit`
              (bind _asenemy_base (cast `EnemyBase` _actor))
              (if (`GameplayTagAssetInterface.HasMatchingGameplayTag` (`AbilitySystemBlueprintLibrary.GetAbilitySystemComponent` _asenemy_base) (struct :`TagName` "Enemy.Cucafera.Jumper"))
                (`AbilitySystemBlueprintLibrary.AddLooseGameplayTags` _asenemy_base (`self.Alert`))))))))
    (:`OnInterrupted`
      (`self.EndAbility` :!label _label_2))
    (:`OnCancelled`
      (goto _label_2))))

(fn `EndAbility`
  (`AbilitySystemBlueprintLibrary.RemoveLooseGameplayTags` (`self.GetOwningActorFromActorInfo`) (`self.Remove Tag`))
  (`self.K2_EndAbility`))