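; Gameplay ability for the Cucafera enemy's bite attack against the player.
; It briefly aims at the player, ending afterwards if the player's starting location was off the navmesh, then plays the bite montage.
; As that blends out, a timed collision task at the mouth applies damage with snap VFX.
; A recovery montage follows with a second damaging check around the body and shell VFX, then the ability ends, removing its loose tags.
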(event `self.K2_ActivateAbility`
  (bind _as_enemy_base (`self.As Enemy Base`))
  (bind _mesh (`Character.Mesh` _as_enemy_base))
  (bind _returnvalue (`SceneComponent.GetSocketLocation` (`Character.Mesh` (`self.As Enemy Base`)) "MouthFirePoint"))
  (bind _asenemy_base (cast `EnemyBase` (`self.GetOwningActorFromActorInfo`)))
  (set `self.As Enemy Base` _asenemy_base)
  (bind _asplayer_character (cast `PlayerCharacter` (`GameplayStatics.GetPlayerCharacter` 0)))
  (bind _output_get (set `self.PlayerCharacter` _asplayer_character))
  ;[0 1 0.02555] Apunta de la carga
  (set `self.OutOfNavMesh?` (`.ReturnValue` (`NavigationSystemV1.K2_ProjectPointToNavigation` (`Actor.K2_GetActorLocation` _output_get) (`self.Nav Data`))))
  (bind (_asynctaskproxy _location) (`AbilityTask_Aim.AimAbilityTask` "None" (`self.PlayerCharacter`) 0.5 0.0 5.0 true)
    (:`OnCompleted`
      (set `self.AimEndPosition` _location)
      (if (`self.OutOfNavMesh?`)
        (if (not (`.ReturnValue` (`NavigationSystemV1.K2_ProjectPointToNavigation` _location (`self.Nav Data`))))
          (set `self.AimEndPosition` (`Actor.K2_GetActorLocation` (`self.PlayerCharacter`))))
        (`AbilityTask_PlayMontageAndWait.CreatePlayMontageAndWaitProxy` "None" "/Game/Assets/Enemies/Cucafera/Anims/AM_Cucafera_Bite.AM_Cucafera_Bite" 1.0 "None" false
          (:`OnBlendOut`
            (bind (_asynctaskproxy_2 _actor) (`AbilityTask_OnCollision.OnCollisionAbilityTask` "None" _returnvalue (0.0 0.0 0.0) 150.0 (`self.Ignore Actors in Peck`) 0.5)
              (:`then`
                (`NiagaraFunctionLibrary.SpawnSystemAtLocation` "/Game/Assets/Enemies/Cucafera/NS_SnapBite.NS_SnapBite" _returnvalue))
              (:`OnCompleted`
                (`AbilityTask_PlayMontageAndWait.CreatePlayMontageAndWaitProxy` "None" "/Game/Assets/Enemies/Cucafera/Anims/AM_Cucafera_BiteRecovery.AM_Cucafera_BiteRecovery" 1.0 "None" false
                  (:`OnBlendOut`
                    (bind (_asynctaskproxy_3 _actor_2) (`AbilityTask_OnCollision.OnCollisionAbilityTask` "None" (`Actor.K2_GetActorLocation` _as_enemy_base) (0.0 0.0 0.0) 150.0 (`self.Ignore Actors in Peck`) 0.67 true)
                      (:`then`
                        (bind _returnvalue_2 (`NiagaraFunctionLibrary.SpawnSystemAtLocation` "/Game/Assets/Enemies/Cucafera/Variantes/Guardian/NS_cucaferashell.NS_cucaferashell" (`SceneComponent.GetSocketLocation` _mesh "caparazonBotTwin_c_sknSocket") (`SceneComponent.GetSocketRotation` _mesh "caparazonBotTwin_c_sknSocket")))
                        (`AbilityTask_Delay.DelayTask` "None" 0.3
                          (:`OnCompleted`
                            (`ActorComponent.Deactivate` _returnvalue_2))))
                      (:`OnCompleted`
                        (`self.End Ability` :!label _label))
                      (:`OnCancelled`
                        (goto _label))
                      (:`OnHit`
                        ;[1 1 1] Dmg Player
                        (bind _asplayer_character_2 (cast `PlayerCharacter` _actor_2))
                        (bind _returnvalue_3 (`AbilitySystemBlueprintLibrary.AssignTagSetByCallerMagnitude` (`self.MakeOutgoingGameplayEffectSpec` "/Game/Blueprints/AbilitySystems/Effects/Damage/GE_Damage_2.GE_Damage_2_C") (struct :`TagName` "States.Damaged") 1.0))
                        (bind _returnvalue_4 (`AbilitySystemBlueprintLibrary.GetAbilitySystemComponent` _asplayer_character_2))
                        (`AbilitySystemComponent.BP_ApplyGameplayEffectSpecToTarget` _returnvalue_4 _returnvalue_3 _returnvalue_4))))
                  (:`OnInterrupted`
                    (`self.End Ability` :!label _label_2))
                  (:`OnCancelled`
                    (goto _label_2))))
              (:`OnInterrupted`
                (`self.End Ability` :!label _label_3))
              (:`OnCancelled`
                (goto _label_3))
              (:`OnHit`
                ;[1 1 1] Dmg Player
                (bind _asplayer_character_3 (cast `PlayerCharacter` _actor))
                (bind _returnvalue_5 (`AbilitySystemBlueprintLibrary.AssignTagSetByCallerMagnitude` (`self.MakeOutgoingGameplayEffectSpec` "/Game/Blueprints/AbilitySystems/Effects/Damage/GE_Damage_2.GE_Damage_2_C") (struct :`TagName` "States.Damaged") 1.0))
                (bind _returnvalue_6 (`AbilitySystemBlueprintLibrary.GetAbilitySystemComponent` _asplayer_character_3))
                (`AbilitySystemComponent.BP_ApplyGameplayEffectSpecToTarget` _returnvalue_6 _returnvalue_5 _returnvalue_6))))
          (:`OnInterrupted`
            (`self.End Ability` :!label _label_4))
          (:`OnCancelled`
            (goto _label_4)))
        (else
          (`self.End Ability` :!label _label_5))))
    (:`OnInterrupted`
      (goto _label_5))
    (:`OnCancelled`
      (goto _label_5))))

(event `self.K2_OnEndAbility`
  (params (bWasCancelled :type Boolean))
  (`self.End Ability`))

(fn `End Ability`
  (`AbilitySystemBlueprintLibrary.RemoveLooseGameplayTags` (`self.GetOwningActorFromActorInfo`) (`self.Remove Tag`))
  (`self.K2_EndAbility`))