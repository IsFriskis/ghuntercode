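; Gameplay ability for the Cucafera enemy that raises the guardian walls belonging to its group.
; On activation it gets the owner's CucaferaGroup and makes every wall in GuardianWallsArray visible, with actor collision on and the mesh blocking all channels.
; It ends one tick later, and its EndAbility function removes loose gameplay tags from the owner without replication.
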(event `self.K2_ActivateAbility`
  (bind _asenemy_cucafera (cast `EnemyCucafera` (`self.GetOwningActorFromActorInfo`)))
  (bind _output_get (set `self.As Enemy Cucafera` _asenemy_cucafera))
  (bind _ascucafera_group (cast `CucaferaGroup` (`EnemyBase.GetGroup` _output_get)))
  (for _array_element (`CucaferaGroup.GuardianWallsArray` _ascucafera_group)
    (bind _asguardian_wall (cast `GuardianWall` _array_element))
    (`Actor.SetActorEnableCollision` _asguardian_wall true)
    (`Actor.SetActorHiddenInGame` _asguardian_wall false)
    (bind _wallstaticmesh (`GuardianWall.WallStaticMesh` _asguardian_wall))
    (`PrimitiveComponent.SetCollisionEnabled` _wallstaticmesh "QueryAndPhysics")
    (`PrimitiveComponent.SetCollisionResponseToAllChannels` _wallstaticmesh "ECR_Block"))
  (`KismetSystemLibrary.DelayUntilNextTick`)
  (`self.K2_EndAbility`))

(event `self.K2_OnEndAbility`
  (params (bWasCancelled :type Boolean))
  (`self.EndAbility`))

(fn `EndAbility`
  (`AbilitySystemBlueprintLibrary.RemoveLooseGameplayTags` (`self.GetOwningActorFromActorInfo`) (`self.Gameplay Tags`))
  (`self.K2_EndAbility`))