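; Gameplay ability for the Basilisco Brute enemy: an aimed charge at the player followed by a peck.
; It aims only onward if the player projects onto the navmesh, falling back near the player if the aimed point does not.
; Chained montages and custom tasks drive a motion-warped charge that damages the player and stuns enemies, then a mouth-socket collision peck that damages the player.
; Ending removes a loose gameplay tag.
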(event `self.K2_ActivateAbility`
  (bind _as_enemy_base (`self.As Enemy Base`))
  (bind _mesh (`Character.Mesh` _as_enemy_base))
  (bind _asplayer_character (cast `PlayerCharacter` (`GameplayStatics.GetPlayerCharacter` 0)))
  (bind _output_get (set `self.PlayerCharacter` _asplayer_character))
  ;[0 1 0.02555] Apunta de la carga
  (set `self.OutOfNavMesh?` (`.ReturnValue` (`NavigationSystemV1.K2_ProjectPointToNavigation` (`Actor.K2_GetActorLocation` _output_get) (`self.Nav Data`))))
  (bind (_asynctaskproxy _location) (`AbilityTask_Aim.AimAbilityTask` "None" (`self.PlayerCharacter`) 0.2 0.0 0.0 true false 600.0)
    (:`OnCompleted`
      (set `self.AimEndPosition` _location)
      (if (`self.OutOfNavMesh?`)
        (if (not (`.ReturnValue` (`NavigationSystemV1.K2_ProjectPointToNavigation` _location (`self.Nav Data`))))
          (set `self.AimEndPosition` (+ (`Actor.K2_GetActorLocation` (`self.PlayerCharacter`)) 20.0)))
        (`AbilityTask_PlayMontageAndWait.CreatePlayMontageAndWaitProxy` "None"
          (:`OnCompleted`
            ;[0 1 0.02745] Realiza la carga al punto de apuntado
            (bind _asenemy_base (cast `EnemyBase` (`self.GetOwningActorFromActorInfo`) :!label _label))
            (bind _output_get_2 (set `self.As Enemy Base` _asenemy_base))
            (`MotionWarpingComponent.AddOrUpdateWarpTarget` (`EnemyBase.EnemyMotionWarpingComponent` _output_get_2) (make `MotionWarpingTarget` "Basilisk_Charge" (`self.AimEndPosition`)))
            (bind (_asynctaskproxy_2 _actorshit) (`AbilityTask_Charge.ChargeAbilityTask` (`self.charge`) (`self.AimEndPosition`) true true 75.0 true 2000.0 (`self.Ignore Actors in charge`) true (`self.Actors to Destroy`))
              (:`then`
                (`AbilityTask_PlayMontageAndWait.CreatePlayMontageAndWaitProxy` "None"
                  (:`OnCompleted`
                    ;[1 1 1] Seteamos los actores que ignora durante el picotazo
                    (bind _outactors (`GameplayStatics.GetAllActorsOfClass` "/Game/Blueprints/Character/Enemies/Gamusino/BP_Gamusino.BP_Gamusino_C" :!label _label_2))
                    (set `self.Ignore Actors in Peck` _outactors)
                    ;[1 0.01866 0] Lanza la animación del picotazo
                    (`AbilityTask_PlayMontageAndWait.CreatePlayMontageAndWaitProxy` "None"
                      (:`OnCompleted`
                        ;[0 1 0.02745] Detecta la colisión durante la animación
                        (bind (_asynctaskproxy_3 _actor) (`AbilityTask_OnCollision.OnCollisionAbilityTask` "PeckAbility" (`SceneComponent.GetSocketLocation` _mesh (`SkinnedMeshComponent.GetSocketBoneName` _mesh "Mouth")) (100.0 0.0 0.0) 150.0 (`self.Ignore Actors in Peck`))
                          (:`then`
                            (`Controller.StopMovement` (`AIBlueprintHelperLibrary.GetAIController` _as_enemy_base))
                            (`AbilityTask_PlayMontageAndWait.CreatePlayMontageAndWaitProxy` "None"
                              (:`OnCompleted`
                                _)
                              (:`OnBlendOut`
                                _)
                              (:`OnInterrupted`
                                _)
                              (:`OnCancelled`
                                _))
                            (`self.End Ability` :!label _label_3))
                          (:`OnInterrupted`
                            (goto _label_3))
                          (:`OnCancelled`
                            (goto _label_3))
                          (:`OnHit`
                            ;[0.07751 0.2856 1] Aplica efectos al player si se detecta colisión
                            (bind _asplayer_character_2 (cast `PlayerCharacter` _actor))
                            (bind _returnvalue (`AbilitySystemBlueprintLibrary.GetAbilitySystemComponent` _asplayer_character_2))
                            (`AbilitySystemComponent.BP_ApplyGameplayEffectToTarget` :`self` _returnvalue :`GameplayEffectClass` "/Game/Blueprints/AbilitySystems/Effects/Damage/GE_Damage_1.GE_Damage_1_C" :`Target` _returnvalue))))
                      (:`OnInterrupted`
                        (`self.End Ability` :!label _label_4))
                      (:`OnCancelled`
                        (goto _label_4))))
                  (:`OnBlendOut`
                    (goto _label_2))
                  (:`OnInterrupted`
                    (`self.End Ability` :!label _label_5))
                  (:`OnCancelled`
                    (goto _label_5))))
              (:`OnInterrupted`
                (`self.End Ability` :!label _label_6))
              (:`OnCancelled`
                (goto _label_6))
              (:`OnHitActor`
                ;[0.07751 0.2856 1] Aplica effectos a los actores con los que colisiona
                ;;[1 1 1] Aplica effectos a los enemigos
                (bind _asenemy_base_2 (cast `EnemyBase` _actorshit)
                  (:`then`
                    (bind _returnvalue_2 (`AbilitySystemBlueprintLibrary.SetDuration` (`self.MakeOutgoingGameplayEffectSpec` "/Game/Blueprints/AbilitySystems/Effects/Enemies/GE_EnemyStun.GE_EnemyStun_C") 1.0))
                    (bind _returnvalue_3 (`AbilitySystemBlueprintLibrary.GetAbilitySystemComponent` _asenemy_base_2))
                    (`AbilitySystemComponent.BP_ApplyGameplayEffectSpecToTarget` _returnvalue_3 _returnvalue_2 _returnvalue_3))
                  (:`CastFailed`
                    ;;[1 1 1] Aplica efectos al player
                    (bind _asplayer_character_3 (cast `PlayerCharacter` _actorshit))
                    (bind _returnvalue_4 (`AbilitySystemBlueprintLibrary.GetAbilitySystemComponent` _asplayer_character_3))
                    (`AbilitySystemComponent.BP_ApplyGameplayEffectToTarget` :`self` _returnvalue_4 :`GameplayEffectClass` "/Game/Blueprints/AbilitySystems/Effects/Damage/GE_Damage_1.GE_Damage_1_C" :`Target` _returnvalue_4))))))
          (:`OnBlendOut`
            (goto _label))
          (:`OnInterrupted`
            (`self.End Ability` :!label _label_7))
          (:`OnCancelled`
            (goto _label_7)))
        (else
          (`self.End Ability` :!label _label_8))))
    (:`OnInterrupted`
      (goto _label_8))
    (:`OnCancelled`
      (goto _label_8))))

(event `self.K2_OnEndAbility`
  (params (bWasCancelled :type Boolean))
  (`self.End Ability`))

(fn `End Ability`
  (`AbilitySystemBlueprintLibrary.RemoveLooseGameplayTags` (`self.GetOwningActorFromActorInfo`) (`self.Remove Tag`))
  (`self.K2_EndAbility`))