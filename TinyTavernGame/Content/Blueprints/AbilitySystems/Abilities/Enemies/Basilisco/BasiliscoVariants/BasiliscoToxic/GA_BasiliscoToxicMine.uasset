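; Gameplay ability for the Toxic Basilisco enemy that lays a mine just in front of it with a peck.
; After a brief delay it plays the peck montage, then fires the mine gameplay cue, spawns BP_BasiliscoMine lowered ahead of the enemy unless blocked, and plays a recovery montage.
; Recovery completion or either montage being interrupted or cancelled ends the ability through EndAbility1, which first removes loose gameplay tags from the owner.
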(event `self.K2_ActivateAbility`
  (bind _asenemy_base (cast `EnemyBase` (`self.GetOwningActorFromActorInfo`)))
  (`AbilityTask_Delay.DelayTask` "None" 0.1
    (:`then`
      (`AbilityTask_PlayMontageAndWait.CreatePlayMontageAndWaitProxy` "None" "/Game/Assets/Enemies/Basilisco/Anim/Montages/AM_BasiliscoToxic_Peck.AM_BasiliscoToxic_Peck" 1.5
        (:`OnCompleted`
          (`GameplayCueFunctionLibrary.ExecuteGameplayCueOnActor` _asenemy_base (struct :`TagName` "GameplayCue.Basilisco.MineCue") (`AbilitySystemBlueprintLibrary.MakeGameplayCueParameters` 0.0))
          (`|SpawnActorFromClass` "/Game/Blueprints/Character/Enemies/Basilisco/Variantes/B_Toxic/BP_BasiliscoMine.BP_BasiliscoMine_C" (`KismetMathLibrary.MakeTransform` (+ (+ (`Actor.K2_GetActorLocation` _asenemy_base) (* (`SceneComponent.GetForwardVector` (`Actor.RootComponent` _asenemy_base)) 100.0)) (0.0 0.0 -50.0))) "AdjustIfPossibleButDontSpawnIfColliding" "MultiplyWithRoot" null null)
          (`AbilityTask_PlayMontageAndWait.CreatePlayMontageAndWaitProxy` "None" "/Game/Assets/Enemies/Basilisco/Anim/Montages/AM_Basilisco_PeckRecovery.AM_Basilisco_PeckRecovery" 0.7
            (:`OnCompleted`
              _)
            (:`OnInterrupted`
              _)
            (:`OnCancelled`
              _))
          (`self.EndAbility1`))
        (:`OnInterrupted`
          (`self.EndAbility1` :!label _label))
        (:`OnCancelled`
          (goto _label))))))

(event `self.K2_OnEndAbility`
  (params (bWasCancelled :type Boolean)))

(fn `EndAbility1`
  (`AbilitySystemBlueprintLibrary.RemoveLooseGameplayTags` (`self.GetOwningActorFromActorInfo`) (`self.Remove Tag`))
  (`self.K2_EndAbility`))