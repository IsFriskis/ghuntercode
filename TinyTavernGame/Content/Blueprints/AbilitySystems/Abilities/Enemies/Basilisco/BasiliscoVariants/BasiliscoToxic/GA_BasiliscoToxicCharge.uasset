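; Gameplay ability for the Toxic Basilisco enemy's charge attack against the player.
; An aim task locks a target point, falling back to the player's position if off the navmesh; the ability aborts if the player started off-navmesh.
; After an anticipation montage, it sets a motion-warp target and runs a charge task with the charge montage.
; Player hits apply a damage effect; the enemy-stun branch is unconnected.
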(event `self.K2_ActivateAbility`
  (bind _asplayer_character (cast `PlayerCharacter` (`GameplayStatics.GetPlayerCharacter` 0)))
  (bind _output_get (set `self.PlayerCharacter` _asplayer_character))
  ;[0 1 0.02555] Apunta de la carga
  (set `self.OutOfNavMesh?` (`.ReturnValue` (`NavigationSystemV1.K2_ProjectPointToNavigation` (`Actor.K2_GetActorLocation` _output_get) (`self.Nav Data`))))
  (bind (_asynctaskproxy _location) (`AbilityTask_Aim.AimAbilityTask` "None" _output_get 0.7 0.0 2000.0 true false 550.0)
    (:`OnCompleted`
      (set `self.AimEndPosition` _location)
      (if (`self.OutOfNavMesh?`)
        (if (not (`.ReturnValue` (`NavigationSystemV1.K2_ProjectPointToNavigation` _location (`self.Nav Data`))))
          (set `self.AimEndPosition` (+ (`Actor.K2_GetActorLocation` (`self.PlayerCharacter`)) 20.0)))
        (`AbilityTask_PlayMontageAndWait.CreatePlayMontageAndWaitProxy` "None" "/Game/Assets/Enemies/Basilisco/Anim/Montages/AM_Basilisco_CargaAnticipacion.AM_Basilisco_CargaAnticipacion"
          (:`OnCompleted`
            ;[0 1 0.02745] Realiza la carga al punto de apuntado
            (bind _asenemy_base (cast `EnemyBase` (`self.GetOwningActorFromActorInfo`) :!label _label))
            (bind _output_get_2 (set `self.As Enemy Base` _asenemy_base))
            (`MotionWarpingComponent.AddOrUpdateWarpTarget` (`EnemyBase.EnemyMotionWarpingComponent` _output_get_2) (make `MotionWarpingTarget` "Basilisk_Charge" (`self.AimEndPosition`)))
            (bind (_asynctaskproxy_2 _actorshit) (`AbilityTask_Charge.ChargeAbilityTask` (`self.charge`) (`self.AimEndPosition`) true false 75.0 false 2000.0 (`self.Ignore Actors in charge`) false (`self.Actors to Destroy`))
              (:`then`
                (`AbilityTask_PlayMontageAndWait.CreatePlayMontageAndWaitProxy` "None" "/Game/Assets/Enemies/Basilisco/Anim/Montages/AM_Basilisco_Carga.AM_Basilisco_Carga" 1.4 "None" false
                  (:`OnCompleted`
                    (bind _outactors (`GameplayStatics.GetAllActorsOfClass` "/Game/Blueprints/Character/Enemies/Gamusino/BP_Gamusino.BP_Gamusino_C"))
                    (set `self.Ignore Actors in Peck` _outactors)
                    (`self.End Ability`))
                  (:`OnInterrupted`
                    (`self.End Ability` :!label _label_2))
                  (:`OnCancelled`
                    (goto _label_2))))
              (:`OnInterrupted`
                (`self.End Ability` :!label _label_3))
              (:`OnCancelled`
                (goto _label_3))
              (:`OnHitActor`
                ;[0.07751 0.2856 1] Aplica effectos a los actores con los que colisiona
                (bind _asplayer_character_2 (cast `PlayerCharacter` _actorshit))
                (bind _returnvalue (`AbilitySystemBlueprintLibrary.GetAbilitySystemComponent` _asplayer_character_2))
                ;;[1 1 1] Aplica efectos al player
                (`AbilitySystemComponent.BP_ApplyGameplayEffectToTarget` :`self` _returnvalue :`GameplayEffectClass` "/Game/Blueprints/AbilitySystems/Effects/Damage/GE_Damage_1.GE_Damage_1_C" :`Target` _returnvalue))))
          (:`OnBlendOut`
            (goto _label))
          (:`OnInterrupted`
            (`self.End Ability` :!label _label_4))
          (:`OnCancelled`
            (goto _label_4)))
        (else
          (`self.End Ability` :!label _label_5))))
    (:`OnInterrupted`
      (goto _label_5))
    (:`OnCancelled`
      (goto _label_5))))

(event `self.K2_OnEndAbility`
  (params (bWasCancelled :type Boolean))
  (`self.End Ability`))

(fn `End Ability`
  (`AbilitySystemBlueprintLibrary.RemoveLooseGameplayTags` (`self.GetOwningActorFromActorInfo`) (`self.Remove Tag`))
  (`self.K2_EndAbility`))