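; Gameplay ability for the Basilisco Dragon enemy's mortar-style "Jam" attack on the player.
; It plays the mortar montage and, on blend out, spawns a projectile at the mouth socket and records the player's position.
; After a short delay, it spawns a jam slam above that position, offset randomly along the player's movement direction to lead the target.
; Completion or montage interruption removes a loose gameplay tag and ends the ability.
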(event `self.K2_ActivateAbility`
  (bind _asplayer_character (cast `PlayerCharacter` (`GameplayStatics.GetPlayerCharacter` 0)))
  (set `self.PlayerCharacter` _asplayer_character)
  (bind _asenemy_base (cast `EnemyBase` (`self.GetOwningActorFromActorInfo`)))
  (set `self.Enemy` _asenemy_base)
  (`AbilityTask_PlayMontageAndWait.CreatePlayMontageAndWaitProxy` "None" "/Game/Assets/Enemies/Basilisco/Anim/Montages/AM_Basilisco_Mortero.AM_Basilisco_Mortero" 0.7
    (:`OnBlendOut`
      (`|SpawnActorFromClass` "/Game/Blueprints/Character/Enemies/Basilisco/Variantes/B_Dragon/BP_BasiliscoProjectile.BP_BasiliscoProjectile_C" (`KismetMathLibrary.MakeTransform` (`SceneComponent.GetSocketLocation` (`Character.Mesh` (`self.Enemy`)) "Mouth")) "Undefined" "MultiplyWithRoot" null null)
      (set `self.AimEndPosition` (`Actor.K2_GetActorLocation` (`self.PlayerCharacter`)))
      (`AbilityTask_Delay.DelayTask` "None" 0.25
        (:`then`
          (`|SpawnActorFromClass` "/Game/Blueprints/Character/Enemies/Basilisco/Variantes/B_Dragon/BP_JamSlamBasilisco.BP_JamSlamBasilisco_C" (`KismetMathLibrary.MakeTransform` (+ (* (`KismetMathLibrary.Normal` (`MovementComponent.Velocity` (`Pawn.GetMovementComponent` (`self.PlayerCharacter`)))) (`KismetMathLibrary.RandomFloatInRange` 100.0 400.0)) (+ (`self.AimEndPosition`) (0.0 0.0 700.0)))) "Undefined" "MultiplyWithRoot" null null)
          (`self.EndAbility1`))))
    (:`OnInterrupted`
      (`self.EndAbility1` :!label _label))
    (:`OnCancelled`
      (goto _label))))

(event `self.K2_OnEndAbility`
  (params (bWasCancelled :type Boolean))
  (`self.K2_EndAbility`))

(fn `EndAbility1`
  (`AbilitySystemBlueprintLibrary.RemoveLooseGameplayTags` (`self.GetOwningActorFromActorInfo`) (`self.Remove Tag`))
  (`self.K2_EndAbility`))