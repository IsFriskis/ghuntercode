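; Gameplay ability for the Basilisco Brute enemy's peck attack.
; When the peck montage completes, a collision task checks an area offset from the peck VFX socket's bone, ignoring the owner, and shakes the first player's camera.
; Player hits receive a set-by-caller damage effect, and a slower recovery montage follows the task.
; Completion or any interruption removes loose gameplay tags from the owner and ends the ability.
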(event `self.K2_ActivateAbility`
  (bind _mesh (`Character.Mesh` (`self.EnemyBase`)))
  (bind _asenemy_base (cast `EnemyBase` (`self.GetOwningActorFromActorInfo`)))
  (set `self.EnemyBase` _asenemy_base)
  (`AbilityTask_PlayMontageAndWait.CreatePlayMontageAndWaitProxy` "None" "/Game/Assets/Enemies/Basilisco/Anim/Montages/AM_Basilisco_Peck.AM_Basilisco_Peck"
    (:`OnCompleted`
      (`KismetArrayLibrary.Array_Add` (`self.Ignore Actors`) (`self.EnemyBase`))
      (bind (_asynctaskproxy _actor) (`AbilityTask_OnCollision.OnCollisionAbilityTask` "PeckAbility" (`SceneComponent.GetSocketLocation` _mesh (`SkinnedMeshComponent.GetSocketBoneName` _mesh "Peck_VFX_Socket")) (100.0 0.0 0.0) 200.0 (`self.Ignore Actors`))
        (:`then`
          (`PlayerController.ClientStartCameraShake` :`self` (`GameplayStatics.GetPlayerController` 0) :`Shake` "/Game/Blueprints/Character/Commons/BP_HitCameraShake.BP_HitCameraShake_C" :`Scale` 0.3 :`PlaySpace` "World"))
        (:`OnCompleted`
          (`AbilityTask_PlayMontageAndWait.CreatePlayMontageAndWaitProxy` "None" "/Game/Assets/Enemies/Basilisco/Anim/Montages/AM_Basilisco_PeckRecovery.AM_Basilisco_PeckRecovery" 0.8
            (:`OnCompleted`
              _)
            (:`OnInterrupted`
              _)
            (:`OnCancelled`
              _))
          (`self.EndAbility1`))
        (:`OnInterrupted`
          (`self.EndAbility1` :!label _label))
        (:`OnCancelled`
          (goto _label))
        (:`OnHit`
          (bind _asplayer_character (cast `PlayerCharacter` _actor))
          (bind _returnvalue (`AbilitySystemBlueprintLibrary.AssignTagSetByCallerMagnitude` (`self.MakeOutgoingGameplayEffectSpec` "/Game/Blueprints/AbilitySystems/Effects/Damage/GE_Damage_3.GE_Damage_3_C") (struct :`TagName` "States.Damaged") 2.0))
          (bind _returnvalue_2 (`AbilitySystemBlueprintLibrary.GetAbilitySystemComponent` _asplayer_character))
          (`AbilitySystemComponent.BP_ApplyGameplayEffectSpecToTarget` _returnvalue_2 _returnvalue _returnvalue_2))))
    (:`OnInterrupted`
      (`self.EndAbility1` :!label _label_2))
    (:`OnCancelled`
      (goto _label_2))))

(event `self.K2_OnEndAbility`
  (params (bWasCancelled :type Boolean))
  (`self.K2_EndAbility`))

(fn `EndAbility1`
  (`AbilitySystemBlueprintLibrary.RemoveLooseGameplayTags` (`self.GetOwningActorFromActorInfo`) (`self.Remove Tag`))
  (`self.K2_EndAbility`))