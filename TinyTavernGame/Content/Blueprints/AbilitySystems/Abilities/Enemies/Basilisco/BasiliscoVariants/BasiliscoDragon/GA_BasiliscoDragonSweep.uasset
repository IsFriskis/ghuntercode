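; Gameplay ability for the Basilisco Dragon enemy's tail sweep attack, which damages players the tail hits.
; It plays the sweep montage while a ticking socket collision task checks between the start and end tail sockets using an impact radius.
; Player hits receive a damage effect through the player's own ability system component.
; When the montage finishes, blends out or aborts, it adds a UseTail tag and ends.
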(event `self.K2_ActivateAbility`
  ;[1 1 1] Obtenemos el Actor que va a realizar la habilidad
  (bind _asenemy_basilisco (cast `EnemyBasilisco` (`self.GetOwningActorFromActorInfo`)))
  (set `self.Basilico` _asenemy_basilisco)
  ;[1 1 1] Reproduce la animación del coletazo
  (`AbilityTask_PlayMontageAndWait.CreatePlayMontageAndWaitProxy` "None" "/Game/Assets/Enemies/Basilisco/Anim/Montages/AM_Basilisco_TailSweep.AM_Basilisco_TailSweep"
    (:`then`
      ;[1 1 1] Detecta las colisiones durante la animación en función del tamaño del impact radius
      (bind (_asynctaskproxy _actor) (`AbilityTask_OnCollision_Socket.OnCollisionSocketAbilityTask` "None" (`self.Impact Radius`) false (`self.Ignore Actors`) 10000.0 true (`Character.Mesh` (`self.Basilico`)) "StartTailSocket" "EndTailSocket")
        (:`OnCompleted`
          (`self.EndAbility` :!label _label))
        (:`OnInterrupted`
          (goto _label))
        (:`OnCancelled`
          (goto _label))
        (:`OnHit`
          ;[1 1 1] Aplica un effecto al player si lo detecta durante la colisión
          (bind _asplayer_character (cast `PlayerCharacter` _actor))
          (bind _returnvalue (`AbilitySystemBlueprintLibrary.GetAbilitySystemComponent` _asplayer_character))
          (`AbilitySystemComponent.BP_ApplyGameplayEffectToTarget` :`self` _returnvalue :`GameplayEffectClass` "/Game/Blueprints/AbilitySystems/Effects/Damage/GE_Damage_2.GE_Damage_2_C" :`Target` _returnvalue))))
    (:`OnCompleted`
      ;[1 1 1] Se le añade una tag para identificar que acaba de usar  este ataque
      (`AbilitySystemBlueprintLibrary.AddLooseGameplayTags` (`self.Basilico`) (`self.UseTail?`) :!label _label_2)
      (`self.EndAbility`))
    (:`OnBlendOut`
      (goto _label_2))
    (:`OnInterrupted`
      (goto _label_2))
    (:`OnCancelled`
      (goto _label_2))))

(event `self.K2_OnEndAbility`
  (params (bWasCancelled :type Boolean))
  (`AbilitySystemBlueprintLibrary.RemoveLooseGameplayTags` null (`self.Gameplay Tags`))
  (`self.EndAbility`))

(fn `EndAbility`
  (`AbilitySystemBlueprintLibrary.RemoveLooseGameplayTags` (`self.Basilico`) (`self.Gameplay Tags`))
  (`self.K2_EndAbility`))