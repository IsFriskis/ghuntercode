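; Gameplay ability for the toxic Basilisco enemy variant that releases a spore area around itself.
; It plays the spores montage and, only on completion, spawns a scaled-up toxic spores actor with a circle Niagara effect and puffball sound at the Basilisco's location.
; Interruption or cancellation ends the ability without spawning anything.
; Ending the ability removes loose gameplay tags from the owner.
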(event `self.K2_ActivateAbility`
  (`AbilityTask_PlayMontageAndWait.CreatePlayMontageAndWaitProxy` "None" "/Game/Assets/Enemies/Basilisco/Anim/Montages/AM_Basilisco_Spores.AM_Basilisco_Spores"
    (:`OnCompleted`
      (bind _asenemy_basilisco (cast `EnemyBasilisco` (`self.GetOwningActorFromActorInfo`)))
      (bind _returnvalue (`Actor.K2_GetActorLocation` _asenemy_basilisco))
      (`|SpawnActorFromClass` "/Game/Blueprints/Character/Enemies/Basilisco/Variantes/B_Toxic/BP_ToxicSpores.BP_ToxicSpores_C" (`KismetMathLibrary.MakeTransform` _returnvalue (struct) (14.0 14.0 14.0)) "Undefined" "MultiplyWithRoot" null null)
      (`NiagaraFunctionLibrary.SpawnSystemAtLocation` "/Game/Assets/Enemies/Basilisco/VFX/NS_BasiliscoSporesCircle.NS_BasiliscoSporesCircle" _returnvalue)
      (`GameplayStatics.PlaySoundAtLocation` "/Game/Assets/Music/Enviroment/Puffball.Puffball" _returnvalue (struct) 1.0 1.0 0.0 null null null null)
      (`self.EndAbility`))
    (:`OnInterrupted`
      (`self.EndAbility` :!label _label))
    (:`OnCancelled`
      (goto _label))))

(event `self.K2_OnEndAbility`
  (params (bWasCancelled :type Boolean))
  (`AbilitySystemBlueprintLibrary.RemoveLooseGameplayTags` null (`self.Gameplay Tags`))
  (`self.EndAbility`))

(fn `EndAbility`
  (`AbilitySystemBlueprintLibrary.RemoveLooseGameplayTags` (`self.GetOwningActorFromActorInfo`) (`self.RemoveTag`))
  (`self.K2_EndAbility`))