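; Gameplay ability that plays the Basilisco enemy's hit reaction with hitstop, mesh shake and a white flash.
; After a short delay it freezes the enemy via CustomTimeDilation, while a looping timer jitters mesh X and applies an overlay material to mesh and children.
; Burn or boil cue tags suppress the shake and minimize hitstop.
; The ability cancels itself after the flash; ending clears the overlay and removes loose tags.
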(event `self.K2_ActivateAbility`
  (bind _returnvalue (`AbilitySystemBlueprintLibrary.GetAbilitySystemComponent` (`self.Enemy`)))
  (`AbilityTask_Delay.DelayTask` "None" 0.1
    (:`OnCompleted`
      (bind _asenemy_base (cast `EnemyBase` (`self.GetAvatarActorFromActorInfo`)))
      (bind _output_get (set `self.Enemy` _asenemy_base))
      (set `self.Character Movement` (`Character.CharacterMovement` _output_get))
      (cast `CombatInterface` (`self.GetAvatarActorFromActorInfo`))
      (bind _returnvalue_2 (`KismetSystemLibrary.K2_SetTimerDelegate` (delegate `Shake`) 0.05 true))
      (if (or (`GameplayTagAssetInterface.HasMatchingGameplayTag` _returnvalue (struct :`TagName` "GameplayCue.Combat.BurnVFX")) (`GameplayTagAssetInterface.HasMatchingGameplayTag` _returnvalue (struct :`TagName` "GameplayCue.Enemy.BoilVFX")))
        (set `self.Shake Distance` 0.0)
        ;[1 1 1] Pasar a C
        (set `self.Hitstop time` 0.001)
        (set `self.MatChange Time` 0.1)
        (else
          (set `self.Shake Distance` 30.0)
          (bind _output_get_2 (set `self.Hitstop time` (`self.Hitstop time`)))
          (set `self.MatChange Time` _output_get_2)))
      ;;[1 0.3426 0.2428] Hitstop
      (set `Actor.CustomTimeDilation` 0.0 (`self.Enemy`))
      (`AbilityTask_Delay.DelayTask` "None" (`self.Hitstop time`)
        (:`OnCompleted`
          (set `Actor.CustomTimeDilation` 1.0 (`self.Enemy`)))))))

(event `self.K2_OnEndAbility`
  (params (bWasCancelled :type Boolean))
  (`self.ChangeOverlay` null)
  (`AbilitySystemBlueprintLibrary.RemoveLooseGameplayTags` (`self.Enemy`) (`self.Gameplay Tags`)))

(event `Shake`
  (bind _mesh (`Character.Mesh` (`self.Enemy`)))
  (bind (_relativelocation_x _relativelocation_y _relativelocation_z) (`KismetMathLibrary.BreakVector` (`SceneComponent.RelativeLocation` _mesh)))
  ;[1 1 1] Pasar a C
  (`|ExecutionSequence`
    (:`then_0`
      ;;[1 1 1] Change Overlay Material
      (`self.ChangeOverlay` "/Game/Assets/VFX/M_HitReact_White_Inst.M_HitReact_White_Inst")
      (`AbilityTask_Delay.DelayTask` "None" (`self.MatChange Time`)
        (:`OnCompleted`
          (`self.ChangeOverlay` null)
          (`KismetSystemLibrary.K2_ClearAndInvalidateTimerHandle` (stale `self.K2_ActivateAbility` _returnvalue_2))
          (`self.K2_CancelAbility`))))
    (:`then_1`
      ;;[0.2135 0.03981 0.1851] Mesh Shake
      (bind _isa (`/Engine/EditorBlueprintResources/StandardMacros.FlipFlop`)
        (:`A`
          _)
        (:`B`
          _))
      (`SceneComponent.K2_SetRelativeLocation` _mesh (`KismetMathLibrary.MakeVector` (+ _relativelocation_x (`KismetMathLibrary.SelectFloat` (* (`self.Shake Distance`) -1.0) (`self.Shake Distance`) _isa)) _relativelocation_y _relativelocation_z) false false))))

(fn `ChangeOverlay`
  (params (OverlayMaterial :type "MaterialInstance Object Reference"))
  (bind _children (`SceneComponent.GetChildrenComponents` (`Character.Mesh` (`self.Enemy`)) false))
  (`MeshComponent.SetOverlayMaterial` (`Character.Mesh` (`self.Enemy`)) OverlayMaterial)
  (if (> (`KismetArrayLibrary.Array_Length` _children) 0)
    (bind _output_get (set `self.Children` _children))
    (for _array_element _output_get
      (bind _asstatic_mesh_component (cast `StaticMeshComponent` _array_element)
        (:`then`
          (`MeshComponent.SetOverlayMaterial` _asstatic_mesh_component OverlayMaterial))
        (:`CastFailed`
          (bind _asskeletal_mesh_component (cast `SkeletalMeshComponent` _array_element))
          (`MeshComponent.SetOverlayMaterial` _asskeletal_mesh_component OverlayMaterial))))))