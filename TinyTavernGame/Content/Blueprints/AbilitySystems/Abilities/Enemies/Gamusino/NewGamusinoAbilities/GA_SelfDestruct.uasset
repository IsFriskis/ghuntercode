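; Gameplay ability for the Gamusino enemy's suicide jump at the player.
; It plays an anticipation montage, runs an aim task on the player, then feeds the resulting location to the "Bomba" motion warp target for the jump montage.
; Movement switches to Flying for the jump and back to Walking afterwards, and loose gameplay tags are removed when the ability ends.
; The NavMesh checks and fallback to the player's location are disconnected.
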(event `self.K2_ActivateAbility`
  ;[1 1 1] Almacenamos el Player
  (bind _asplayer_character (cast `PlayerCharacter` (`GameplayStatics.GetPlayerCharacter` 0)))
  (set `self.Player` _asplayer_character)
  (`AbilityTask_PlayMontageAndWait.CreatePlayMontageAndWaitProxy` "None" "/Game/Assets/Enemies/Gamusino/Animations/AM_Gamusino_SuicideAnticipation.AM_Gamusino_SuicideAnticipation" 1.35
    (:`OnCompleted`
      ;[0.21 0 1] Obtiene el punto final de la carga
      (bind (_asynctaskproxy _location) (`AbilityTask_Aim.AimAbilityTask` "None" (`self.Player`) 0.0 0.0 0.0 true true 700.0 (`self.Tolerance`))
        (:`OnCompleted`
          (set `self.Location` _location)
          ;[1 0.251 0.2353] Usamos Motion Warping para ajustar el punto final de la animación de la carga
          (bind _asbp_gamusino (cast `/Game/Blueprints/Character/Enemies/Gamusino/BP_Gamusino` (`self.GetOwningActorFromActorInfo`)))
          (bind _output_get (set `self.As BP Gamusino` _asbp_gamusino))
          (`MotionWarpingComponent.AddOrUpdateWarpTarget` (`EnemyBase.EnemyMotionWarpingComponent` _output_get) (make `MotionWarpingTarget` "Bomba" (`self.Location`)))
          (`CharacterMovementComponent.SetMovementMode` (`Character.CharacterMovement` (`self.As BP Gamusino`)) "MOVE_Flying" 0)
          (`AbilityTask_PlayMontageAndWait.CreatePlayMontageAndWaitProxy` "None" "/Game/Assets/Enemies/Gamusino/Animations/AM_GamusinoSuicideJump.AM_GamusinoSuicideJump"
            (:`OnCompleted`
              _)
            (:`OnInterrupted`
              _)
            (:`OnCancelled`
              _))
          (`CharacterMovementComponent.SetMovementMode` (`Character.CharacterMovement` (`self.As BP Gamusino`)) "MOVE_Walking" 0)
          (`self.K2_EndAbility`))
        (:`OnInterrupted`
          ;[0 0.8641 1] Control de comportamiento en función de  NavMesh
          (`self.K2_EndAbility` :!label _label))
        (:`OnCancelled`
          (goto _label))))
    (:`OnInterrupted`
      (`self.K2_EndAbility` :!label _label_2))
    (:`OnCancelled`
      (goto _label_2))))

(event `self.K2_OnEndAbility`
  (params (bWasCancelled :type Boolean))
  (`AbilitySystemBlueprintLibrary.RemoveLooseGameplayTags` (`self.GetOwningActorFromActorInfo`) (`self.Gameplay Tags`)))

(fn `HasMatchingTag`
  (locals (MatchingTag :type Boolean :default false))
  (set `local.MatchingTag` (`GameplayTagAssetInterface.HasMatchingGameplayTag` (`AbilitySystemBlueprintLibrary.GetAbilitySystemComponent` (`self.GetOwningActorFromActorInfo`)) (struct :`TagName` "States.Cook.Grilled")))
  (return))