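; Gameplay ability for the Gamusino enemy's kamikaze explosion, which hurts the player and breaks destroyables.
; On activation it plays explosion sound and VFX, spawns a blood death actor, shakes the camera and applies invulnerability to itself.
; A radial collision task then applies SetByCaller damage to the player or destroys hit Destroyable actors with break VFX.
; The ability ends when that task completes, and its end event removes loose gameplay tags.
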(event `self.K2_ActivateAbility`
  (bind _returnvalue (`self.GetOwningActorFromActorInfo`))
  (bind _returnvalue_2 (`Actor.K2_GetActorLocation` _returnvalue))
  (bind _returnvalue_3 (`Actor.K2_GetActorRotation` _returnvalue))
  (bind _asplayer_character (cast `PlayerCharacter` (`GameplayStatics.GetPlayerPawn` 0)))
  (bind _output_get (set `self.Player` _asplayer_character))
  (`GameplayStatics.SpawnSoundAtLocation` "/Game/Assets/Music/Enemy/S_Kamikaze_Explosion.S_Kamikaze_Explosion" _returnvalue_2 (struct) 1.0 1.0 0.0 null null)
  (`|SpawnActorFromClass` "/Game/Blueprints/Character/Commons/BP_BloodDEATH.BP_BloodDEATH_C" (`KismetMathLibrary.MakeTransform` _returnvalue_2 _returnvalue_3) "Undefined" "MultiplyWithRoot" null null)
  (`PlayerController.ClientStartCameraShake` :`self` (`GameplayStatics.GetPlayerController` 0) :`Shake` "/Game/Blueprints/Character/Commons/BP_HitCameraShake.BP_HitCameraShake_C" :`Scale` 2.0 :`PlaySpace` "World")
  (`NiagaraFunctionLibrary.SpawnSystemAtLocation` "/Game/Assets/Enemies/Gamusino/Variantes/Kamikaze/NS_KamikazeExplosion.NS_KamikazeExplosion" _returnvalue_2 _returnvalue_3)
  (`AbilitySystemComponent.BP_ApplyGameplayEffectToSelf` :`self` (`AbilitySystemBlueprintLibrary.GetAbilitySystemComponent` (`self.GetOwningActorFromActorInfo`)) :`GameplayEffectClass` "/Game/Blueprints/AbilitySystems/Effects/Enemies/GE_EnemyInvulnerability.GE_EnemyInvulnerability_C")
  (bind (_asynctaskproxy _actor) (`AbilityTask_OnCollision.OnCollisionAbilityTask` "None" (`Actor.K2_GetActorLocation` (`self.GetOwningActorFromActorInfo`)) (0.0 0.0 0.0) 200.0 (`self.Ignore Actors`))
    (:`OnCompleted`
      (`self.K2_EndAbility`))
    (:`OnHit`
      (bind _asplayer_character_2 (cast `PlayerCharacter` _actor)
        (:`then`
          (bind _returnvalue_4 (`AbilitySystemBlueprintLibrary.AssignTagSetByCallerMagnitude` (`self.MakeOutgoingGameplayEffectSpec` "/Game/Blueprints/AbilitySystems/Effects/Damage/GE_Damage_2.GE_Damage_2_C") (struct :`TagName` "States.Damaged") 1.0))
          (bind _returnvalue_5 (`AbilitySystemBlueprintLibrary.GetAbilitySystemComponent` _asplayer_character_2))
          (`AbilitySystemComponent.BP_ApplyGameplayEffectSpecToTarget` _returnvalue_5 _returnvalue_4 _returnvalue_5))
        (:`CastFailed`
          (bind _asdestroyable (cast `Destroyable` _actor))
          (`NiagaraFunctionLibrary.SpawnSystemAtLocation` "/Game/Assets/Actors/Hazards/Destroyable/NS_BreakDestroyable.NS_BreakDestroyable" (`Actor.K2_GetActorLocation` _asdestroyable))
          (`Actor.K2_DestroyActor` _asdestroyable))))))

(event `self.K2_OnEndAbility`
  (params (bWasCancelled :type Boolean))
  (`AbilitySystemBlueprintLibrary.RemoveLooseGameplayTags` (`self.GetOwningActorFromActorInfo`) (`self.Gameplay Tags`))
  (`self.K2_EndAbility`))

(fn `HasMatchingTag`
  (locals (MatchingTag :type Boolean :default false))
  (set `local.MatchingTag` (`GameplayTagAssetInterface.HasMatchingGameplayTag` (`AbilitySystemBlueprintLibrary.GetAbilitySystemComponent` (`self.GetOwningActorFromActorInfo`)) (struct :`TagName` "States.Cook.Grilled")))
  (return))