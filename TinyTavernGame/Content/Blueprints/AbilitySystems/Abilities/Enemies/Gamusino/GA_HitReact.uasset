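; Gameplay ability that plays the PlayerCharacter's hit reaction, despite sitting under the Enemies/Gamusino folder.
; On activation it caches materials, applies invulnerability and hit-react effects, breaks any active shield, and plays the combat interface's montage.
; Camera shake, force feedback and a brief time-dilation hitstop accompany a looping timer that flashes hit materials and jitters the mesh.
; Montage end clears the timer and effect; ending the ability restores materials.
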(event `self.K2_OnEndAbility`
  (params (bWasCancelled :type Boolean))
  (bind _mesh (`Character.Mesh` (`self.Player`)))
  (for (_ _array_index) (`MeshComponent.GetMaterials` _mesh)
    (`PrimitiveComponent.SetMaterial` _mesh _array_index (`|GetArrayItem` (`self.OriginalMaterials`) _array_index))
    (`AbilitySystemBlueprintLibrary.RemoveLooseGameplayTags` (`self.Player`) (`self.Gameplay Tags`) :!label _label))
  (if (`self.HasChildMaterials`)
    (for _array_element (`SceneComponent.GetChildrenComponents` (`Character.Mesh` (`self.Player`)) false)
      (bind _asstatic_mesh_component (cast `StaticMeshComponent` _array_element))
      (for (_ _array_index_2) (`MeshComponent.GetMaterials` _asstatic_mesh_component)
        (`PrimitiveComponent.SetMaterial` _asstatic_mesh_component _array_index_2 null)
        (goto _label)))))

(event `Shake`
  (bind _mesh (`Character.Mesh` (`self.Player`)))
  (bind _mesh_2 (`Character.Mesh` (`self.Player`)))
  (bind _mesh_3 (`Character.Mesh` (`self.Player`)))
  (bind (_relativelocation_x _relativelocation_y _relativelocation_z) (`KismetMathLibrary.BreakVector` (`SceneComponent.RelativeLocation` _mesh)))
  (`|ExecutionSequence`
    (:`then_0`
      ;[1 0.6949 0.2601] Poner Material Hit
      (for (_ _array_index) (`MeshComponent.GetMaterials` _mesh_3)
        (`PrimitiveComponent.SetMaterial` _mesh_3 _array_index "/Game/Assets/VFX/M_HitReact_Inst.M_HitReact_Inst"))
      (if (`self.HasChildMaterials`)
        (for _array_element (`SceneComponent.GetChildrenComponents` (`Character.Mesh` (`self.Player`)) false)
          (bind _asstatic_mesh_component (cast `StaticMeshComponent` _array_element))
          (for (_ _array_index_2) (`MeshComponent.GetMaterials` _asstatic_mesh_component)
            (`PrimitiveComponent.SetMaterial` _asstatic_mesh_component _array_index_2 "/Game/Assets/VFX/M_HitReact_Inst.M_HitReact_Inst"))
          (`AbilityTask_Delay.DelayTask` "None" (`self.Hitstop time`) :!label _label_2
            (:`OnCompleted`
              ;[0.3462 0.755 1] Volver a Materail original
              (for (_ _array_index_3) (`MeshComponent.GetMaterials` _mesh_2)
                (`PrimitiveComponent.SetMaterial` _mesh_2 _array_index_3 (`|GetArrayItem` (`self.OriginalMaterials`) _array_index_3)))
              (if (`self.HasChildMaterials`)
                (for _array_element_2 (`SceneComponent.GetChildrenComponents` (`Character.Mesh` (`self.Player`)) false)
                  (bind _asstatic_mesh_component_2 (cast `StaticMeshComponent` _array_element_2))
                  (for (_ _array_index_4) (`MeshComponent.GetMaterials` _asstatic_mesh_component_2)
                    (`PrimitiveComponent.SetMaterial` _asstatic_mesh_component_2 _array_index_4 null)))))))
        (else
          (goto _label_2))))
    (:`then_1`
      ;[0.2135 0.03981 0.1851] Mesh Shake
      (bind _isa (`/Engine/EditorBlueprintResources/StandardMacros.FlipFlop`)
        (:`A`
          _)
        (:`B`
          _))
      (`SceneComponent.K2_SetRelativeLocation` _mesh (`KismetMathLibrary.MakeVector` (+ _relativelocation_x (`KismetMathLibrary.SelectFloat` (* (`self.Shake Distance`) -1.0) (`self.Shake Distance`) _isa)) _relativelocation_y _relativelocation_z) false false))))

(event `self.K2_ActivateAbility`
  (bind _returnvalue (`GameplayStatics.GetPlayerController` 0))
  (bind _mesh (`Character.Mesh` (`self.Player`)))
  (bind _children (`SceneComponent.GetChildrenComponents` _mesh false))
  (bind _asplayer_character (cast `PlayerCharacter` (`self.GetAvatarActorFromActorInfo`)))
  (bind _output_get (set `self.Player` _asplayer_character))
  (set `self.Character Movement` (`Character.CharacterMovement` _output_get))
  ;[1 1 1] Pick Hit React Montage
  (bind _ascombat_interface (cast `CombatInterface` (`self.GetAvatarActorFromActorInfo`)))
  (bind _returnvalue_2 (`CombatInterface.GetHitReactMontage` _ascombat_interface))
  (set `self.Hit React Montage` _returnvalue_2)
  (set `self.OriginalMaterials` (`MeshComponent.GetMaterials` _mesh))
  (bind _output_get_2 (set `self.HasChildMaterials` (> (`KismetArrayLibrary.Array_Length` _children) 0)))
  (if _output_get_2
    (for _array_element _children
      (bind _asstatic_mesh_component (cast `StaticMeshComponent` _array_element))
      (bind _output_get_3 (set `self.As Static Mesh Component` _asstatic_mesh_component))
      (for _array_element_2 (`MeshComponent.GetMaterials` _output_get_3)
        (`BlueprintMapLibrary.Map_Add` (`self.Children Materials`) (`self.As Static Mesh Component`) _array_element_2))
      (`AbilitySystemComponent.BP_ApplyGameplayEffectToSelf` :`self` (`AbilitySystemBlueprintLibrary.GetAbilitySystemComponent` (`self.Player`)) :`GameplayEffectClass` "/Game/Blueprints/AbilitySystems/Effects/Commons/GE_PlayerHitInvunerable.GE_PlayerHitInvunerable_C" :!label _label_3)
      (if (`GameplayTagAssetInterface.HasMatchingGameplayTag` (`AbilitySystemBlueprintLibrary.GetAbilitySystemComponent` (`self.Player`)) (struct :`TagName` "States.PlayerShield"))
        (`AbilitySystemBlueprintLibrary.RemoveLooseGameplayTags` (`self.Player`) (`self.ShieldTag`))
        (`GameplayCueFunctionLibrary.ExecuteGameplayCueOnActor` (`self.Player`) (struct :`TagName` "GameplayCue.PlayerShieldBroken") (`AbilitySystemBlueprintLibrary.MakeGameplayCueParameters` 0.0)))
      (bind _returnvalue_3 (`self.BP_ApplyGameplayEffectToOwner` "/Game/Blueprints/AbilitySystems/Effects/Commons/GE_HitReact.GE_HitReact_C"))
      (set `self.Active GE_HitReact` _returnvalue_3)
      (`AbilityTask_PlayMontageAndWait.CreatePlayMontageAndWaitProxy` "None" (`self.Hit React Montage`)
        (:`then`
          (`PlayerController.ClientStartCameraShake` :`self` _returnvalue :`Shake` "/Game/Blueprints/Character/Commons/BP_HitCameraShake.BP_HitCameraShake_C" :`PlaySpace` "World")
          (`PlayerController.K2_ClientPlayForceFeedback` _returnvalue "/Game/Blueprints/Inputs/ForceFeedback/FF_GrillVibration.FF_GrillVibration" "None" false false false)
          (bind _returnvalue_4 (`KismetSystemLibrary.K2_SetTimerDelegate` (delegate `Shake`) 0.05 true))
          (set `self.Timer Event` _returnvalue_4)
          ;[1 0.3426 0.2428] Hitstop
          (`AbilityTask_Delay.DelayTask` "None" 0.1
            (:`OnCompleted`
              (set `Actor.CustomTimeDilation` 0.0 (`self.Player`))
              (`AbilityTask_Delay.DelayTask` "None" 0.1
                (:`OnCompleted`
                  (set `Actor.CustomTimeDilation` 1.0 (`self.Player`)))))))
        (:`OnCompleted`
          (`self.BP_RemoveGameplayEffectFromOwnerWithHandle` (`self.Active GE_HitReact`) 30 :!label _label_4)
          (`KismetSystemLibrary.K2_ClearAndInvalidateTimerHandle` (`self.Timer Event`))
          (`self.K2_EndAbility`))
        (:`OnInterrupted`
          (goto _label_4))
        (:`OnCancelled`
          (goto _label_4))))
    (else
      (goto _label_3))))