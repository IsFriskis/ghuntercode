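; Gamusino enemy charge ability: a pre-charge montage and VFX, an aim task on the player, then a charge and recovery montage.
; It cancels if the player is off the NavMesh, and retargets near the player if the aimed point is off it.
; Motion Warping fits the charge montage to the target point while a charge task detects hits.
; Hitting the player applies damage and an erratic dodge montage; hitting another Gamusino currently does nothing.
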(event `self.K2_ActivateAbility`
  ;[1 1 1] Almacenamos el Player
  (bind _asplayer_character (cast `PlayerCharacter` (`GameplayStatics.GetPlayerCharacter` 0)))
  (bind _output_get (set `self.Player` _asplayer_character))
  ;[0 0.3327 1] Detectamos si el player esta en la NavMesh
  (set `self.IsOutOfMesh` (`.ReturnValue` (`NavigationSystemV1.K2_ProjectPointToNavigation` (`Actor.K2_GetActorLocation` _output_get) (`self.Nav Data`))))
  ;[1 0.251 0.2353] Animación de Pre-Carga
  (`AbilityTask_PlayMontageAndWait.CreatePlayMontageAndWaitProxy` "None" "/Game/Assets/Enemies/Gamusino/Animations/AM_GamusinoTacklePre.AM_GamusinoTacklePre" 2.5
    (:`then`
      (`NiagaraFunctionLibrary.SpawnSystemAtLocation` null (`Actor.K2_GetActorLocation` (`self.GetOwningActorFromActorInfo`)))
      ;[0.21 0 1] Obtiene el punto final de la carga
      (bind (_asynctaskproxy _location) (`AbilityTask_Aim.AimAbilityTask` "None" (`self.Player`) 1.0 0.0 0.0 true true 500.0 (`self.Tolerance`))
        (:`OnCompleted`
          (set `self.Location` _location)
          ;[0 0.8641 1] Control de comportamiento en función de  NavMesh
          ;;[1 1 1] Si el player esta fuera de la NavMesh cancela la habilidad
          (if (`self.IsOutOfMesh`)
            ;;[1 1 1] Si el punto de carga esta fuera de la NavMesh Recalculamos el punto de la carga para qque termine en el player y se le aplica un offset para que alcance bien al player
            (if (not (`.ReturnValue` (`NavigationSystemV1.K2_ProjectPointToNavigation` _location (`self.Nav Data`))))
              (set `self.Location` (+ (`Actor.K2_GetActorLocation` (`self.Player`)) 20.0)))
            ;[1 0.251 0.2353] Usamos Motion Warping para ajustar el punto final de la animación de la carga
            (bind _asbp_gamusino (cast `/Game/Blueprints/Character/Enemies/Gamusino/BP_Gamusino` (`self.GetOwningActorFromActorInfo`)))
            (bind _output_get_2 (set `self.As BP Gamusino` _asbp_gamusino))
            (`MotionWarpingComponent.AddOrUpdateWarpTarget` (`EnemyBase.EnemyMotionWarpingComponent` _output_get_2) (make `MotionWarpingTarget` "Gamusino_Charge" (`self.Location`)))
            ;[0.21 0 1] Parametrización y Realización de la carga
            (bind (_asynctaskproxy_2 _actorshit) (`AbilityTask_Charge.ChargeAbilityTask` (`self.Task Instance Name`) (`self.Location`) true false 50.0 true 0.0 (`self.Ignore Actors`) false (`self.Actors to Destroy`))
              (:`then`
                ;[1 0.251 0.2353] Animación de la carga
                (`AbilityTask_PlayMontageAndWait.CreatePlayMontageAndWaitProxy` "None" "/Game/Assets/Enemies/Gamusino/Animations/AM_GamusinoTackleCarga.AM_GamusinoTackleCarga"
                  (:`OnCompleted`
                    (`self.EndTaskByInstanceName` (`self.Task Instance Name`))
                    ;[1 0.251 0.2353] Animación del Recovery de la carga
                    (`AbilityTask_PlayMontageAndWait.CreatePlayMontageAndWaitProxy` "None" "/Game/Assets/Enemies/Gamusino/Animations/AM_GamusinoTackleRecovery.AM_GamusinoTackleRecovery"
                      (:`OnCompleted`
                        _)
                      (:`OnBlendOut`
                        _)
                      (:`OnInterrupted`
                        _)
                      (:`OnCancelled`
                        _))
                    (`self.EndAbility` :!label _label))
                  (:`OnInterrupted`
                    (bind _asenemy_base (cast `EnemyBase` (`self.GetOwningActorFromActorInfo`) :!label _label_2))
                    (bind _charactermovement (`Character.CharacterMovement` _asenemy_base))
                    (`CharacterMovementComponent.SetMovementMode` _charactermovement "MOVE_Flying" 0)
                    (`AbilityTask_PlayMontageAndWait.CreatePlayMontageAndWaitProxy` "None" "/Game/Assets/Enemies/Gamusino/Animations/AM_GamusinoErraticDodge.AM_GamusinoErraticDodge" 1.5
                      (:`then`
                        _)
                      (:`OnCompleted`
                        _)
                      (:`OnBlendOut`
                        _)
                      (:`OnInterrupted`
                        _)
                      (:`OnCancelled`
                        _))
                    (`CharacterMovementComponent.SetMovementMode` _charactermovement "MOVE_Walking" 0)
                    (goto _label))
                  (:`OnCancelled`
                    (`self.EndAbility`))))
              (:`OnInterrupted`
                ;[0 1 0.05313] Effectos que se aplicarán en función del Actor con el que colisiona
                ;;[1 1 1] Effecto que aplica si el Actor Hit es un Gamusino
                (`self.EndAbility` :!label _label_3))
              (:`OnCancelled`
                (goto _label_3))
              (:`OnHitActor`
                (bind _output_get_3 (set `self.Actor Hit` _actorshit))
                (bind _asenemy_gamusino (cast `EnemyGamusino` _output_get_3)
                  (:`CastFailed`
                    ;;[1 1 1] Efecto que aplica si el Actor Hit es el Player
                    (bind _asplayer_character_2 (cast `PlayerCharacter` (`self.Actor Hit`)))
                    (bind _returnvalue (`AbilitySystemBlueprintLibrary.GetAbilitySystemComponent` _asplayer_character_2))
                    (`AbilitySystemComponent.BP_ApplyGameplayEffectToTarget` :`self` _returnvalue :`GameplayEffectClass` "/Game/Blueprints/AbilitySystems/Effects/Damage/GE_Damage_1.GE_Damage_1_C" :`Target` _returnvalue)
                    (goto _label_2)))))
            (else
              (`self.EndAbility`))))
        (:`OnInterrupted`
          (`self.EndAbility` :!label _label_4))
        (:`OnCancelled`
          (goto _label_4))))))

(event `self.K2_OnEndAbility`
  (params (bWasCancelled :type Boolean))
  (`self.EndAbility`))

(fn `EndAbility`
  (`AbilitySystemBlueprintLibrary.RemoveLooseGameplayTags` (`self.GetOwningActorFromActorInfo`) (`self.Gameplay Tags`))
  (`self.K2_EndAbility`))