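; Gameplay ability for the Gamusino enemy that throws a muddy projectile at the player.
; It runs a short aim task oriented to the player and starts the shot montage alongside it.
; On montage completion or blend-out it spawns the projectile at the mouth socket's XY, taking height, roll and yaw from the player, then ends.
; Interruption or cancellation ends it without spawning, and ending removes loose gameplay tags from the enemy.
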(event `self.K2_ActivateAbility`
  (bind _asenemy_base (cast `EnemyBase` (`self.GetOwningActorFromActorInfo`))
    (:`then`
      (bind _output_get (set `self.As Enemy Base` _asenemy_base))
      (bind _asplayer_character (cast `PlayerCharacter` (`GameplayStatics.GetPlayerCharacter` 0)))
      (`AbilityTask_Aim.AimAbilityTask` "None" _asplayer_character 0.2 0.0 0.0 true true
        (:`then`
          (`AbilityTask_PlayMontageAndWait.CreatePlayMontageAndWaitProxy` "None" "/Game/Assets/Enemies/Gamusino/Animations/Gamusino_Shot_RM_Montage.Gamusino_Shot_RM_Montage"
            (:`OnCompleted`
              (bind (_returnvalue_x _returnvalue_y) (`KismetMathLibrary.BreakVector` (`SceneComponent.GetSocketLocation` (`Character.Mesh` _output_get) "Mouth")))
              (bind (_returnvalue_x_2 _returnvalue_y_2 _returnvalue_z) (`KismetMathLibrary.BreakVector` (`Actor.K2_GetActorLocation` _asplayer_character)))
              (bind (_returnvalue_roll _returnvalue_pitch _returnvalue_yaw) (`KismetMathLibrary.BreakRotator` (`Actor.K2_GetActorRotation` _asplayer_character)))
              (`|SpawnActorFromClass` "/Game/Blueprints/Character/Enemies/Gamusino/Variantes/G_Muddy/BP_MuddyPorjectile.BP_MuddyPorjectile_C" (`KismetMathLibrary.MakeTransform` (`KismetMathLibrary.MakeVector` _returnvalue_x _returnvalue_y _returnvalue_z) (`KismetMathLibrary.MakeRotator` _returnvalue_roll 0.0 _returnvalue_yaw)) "AlwaysSpawn" "MultiplyWithRoot" null null :!label _label))
            (:`OnBlendOut`
              (goto _label))
            (:`OnInterrupted`
              _)
            (:`OnCancelled`
              _))
          (`self.K2_EndAbility`))))
    (:`CastFailed`
      (`self.K2_EndAbility`))))

(event `self.K2_OnEndAbility`
  (params (bWasCancelled :type Boolean))
  (`AbilitySystemBlueprintLibrary.RemoveLooseGameplayTags` (`self.As Enemy Base`) (`self.Gameplay Tags`)))