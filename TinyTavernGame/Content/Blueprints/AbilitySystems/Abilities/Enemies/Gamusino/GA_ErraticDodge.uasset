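; Gameplay ability for the Gamusino enemy that performs an erratic dodge as two consecutive jumps before ending.
; Each ErraticJump runs an aim task to pick a landing point, feeds it to a motion warping target, plays the dodge montage, then restores Walking movement.
; Interruption or cancellation ends the ability, also forcing a fixed actor rotation during aiming.
; Ending removes loose gameplay tags from the enemy.
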(event `self.K2_ActivateAbility`
  ;[1 1 1] Obtenemos el Actor que va a realizar los saltos
  (bind _asenemy_base (cast `EnemyBase` (`self.GetOwningActorFromActorInfo`)))
  (set `self.As Enemy Base` _asenemy_base)
  ;[1 1 1] Numero de saltos que va a realizar
  (`self.ErraticJump`)
  (`self.ErraticJump`)
  ;[1 1 1] Finalizar habilidad
  (`self.End Ability`))

(fn `End Ability`
  (`AbilitySystemBlueprintLibrary.RemoveLooseGameplayTags` (`self.As Enemy Base`) (`self.Gameplay Tags`))
  (`self.K2_EndAbility`))