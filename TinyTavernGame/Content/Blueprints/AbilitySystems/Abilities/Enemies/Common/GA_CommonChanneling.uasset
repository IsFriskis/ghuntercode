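; Shared enemy channeling ability that plays a type-specific montage at a burrow and removes the enemy from play.
; It motion-warps toward the blackboard burrow's center; Cucafera adds Niagara effects and Basilisco switches to flying.
; A montage notify decrements the group count and ends the ability, destroying the enemy, unless a QTE is active, which tags it Escaped instead.
; Interruption outside a QTE cancels without destroying; older per-enemy chains remain unconnected.
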(event `self.K2_ActivateAbility`
  (bind _as_enemy_base (`self.As Enemy Base`))
  (bind _returnvalue (`EnemyBase.GetGroup` _as_enemy_base))
  (bind _returnvalue_2 (`SceneComponent.GetSocketLocation` (`EnemyBurrow.MeshComponent` (`self.As Enemy Burrow`)) "BurrowCenter"))
  (bind _returnvalue_3 (`GameplayTagAssetInterface.HasMatchingGameplayTag` (`AbilitySystemBlueprintLibrary.GetAbilitySystemComponent` _as_enemy_base) (struct :`TagName` "Events.Enemy.InQTE")))
  (bind _asenemy_base (cast `EnemyBase` (`self.GetOwningActorFromActorInfo`))
    (:`then`
      (bind _output_get (set `self.As Enemy Base` _asenemy_base))
      (bind _asenemy_burrow (cast `EnemyBurrow` (`BlackboardComponent.GetValueAsObject` (`AIBlueprintHelperLibrary.GetBlackboard` (`AIBlueprintHelperLibrary.GetAIController` _output_get)) (`self.Key Name`))))
      (set `self.As Enemy Burrow` _asenemy_burrow)
      (`MotionWarpingComponent.AddOrUpdateWarpTargetFromLocation` (`EnemyBase.EnemyMotionWarpingComponent` (`self.As Enemy Base`)) "E_Channeling" _returnvalue_2)
      (bind _returnvalue_4 (`EnemyBase.GetEnemyType` (`self.As Enemy Base`)))
      (`|SwitchGameplayTag` _returnvalue_4
        (:`Default`
          (`self.K2_EndAbility`))
        (:`Enemy.Gamusino`
          (set `self.MontageToPlay` "/Game/Assets/Enemies/Gamusino/Animations/AM_Gamusino_Chanelling.AM_Gamusino_Chanelling")
          (`|PlayMontage` (`Character.Mesh` (`self.As Enemy Base`)) (`self.MontageToPlay`) :!label _label
            (:`OnInterrupted`
              (if (not _returnvalue_3)
                (`self.K2_CancelAbility`)))
            (:`OnNotifyBegin`
              (if _returnvalue_3
                (`AbilitySystemBlueprintLibrary.AddLooseGameplayTags` (`self.As Enemy Base`) (`BlueprintGameplayTagLibrary.MakeGameplayTagContainerFromTag` (struct :`TagName` "States.Escaped")))
                (else
                  (set `EnemyGroup.enemiesInGroupCount` (- (`EnemyGroup.enemiesInGroupCount` _returnvalue) 1) _returnvalue)))
              (`self.K2_EndAbility`))))
        (:`Enemy.Cucafera`
          (set `self.MontageToPlay` "/Game/Assets/Enemies/Cucafera/Anims/AM_CucaferaChannelingTest.AM_CucaferaChannelingTest")
          (`NiagaraFunctionLibrary.SpawnSystemAtLocation` "/Game/Blueprints/Actors/Tornado/NS_Cucaferachanneling.NS_Cucaferachanneling" _returnvalue_2)
          (goto _label))
        (:`Enemy.Basilisco`
          (set `self.MontageToPlay` "/Game/Assets/Enemies/Basilisco/Anim/Montages/AM_BasiliscoChannelingTest.AM_BasiliscoChannelingTest")
          (`CharacterMovementComponent.SetMovementMode` (`Character.CharacterMovement` (`self.As Enemy Base`)) "MOVE_Flying" 0)
          (goto _label))))
    (:`CastFailed`
      (`self.K2_CancelAbility`))))

(event `self.K2_OnEndAbility`
  (params (bWasCancelled :type Boolean))
  (if (`GameplayTagAssetInterface.HasMatchingGameplayTag` (`AbilitySystemBlueprintLibrary.GetAbilitySystemComponent` (`self.As Enemy Base`)) (struct :`TagName` "States.Escaped"))
    _
    (elif (not bWasCancelled)
      (`Actor.K2_DestroyActor` (`self.As Enemy Base`)))))