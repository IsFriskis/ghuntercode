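; Gameplay ability for a PuffBall hazard that releases an instant spore burst and damages the player.
; On activation it adds loose tags, drives the PuffBall's StartingSpores and SpawningSpores flags, and plays a sound.
; After a short delay it spawns the burst effect and runs a radial collision task, applying GE_HealthHazardInstant to any PlayerCharacter hit.
; Task completion resets the flags, removes the tags and ends the ability.
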(event `self.K2_ActivateAbility`
  (bind _returnvalue (`self.GetOwningActorFromActorInfo`))
  (bind _returnvalue_location (`KismetMathLibrary.BreakTransform` (`Actor.GetTransform` _returnvalue)))
  ;[0.2806 0.3331 1] Función que hace que pierda stats el jugador
  (`/Engine/EditorBlueprintResources/StandardMacros.IsValid` _returnvalue
    (:`Is Valid`
      (`AbilitySystemBlueprintLibrary.AddLooseGameplayTags` _returnvalue (`self.Gameplay Tags`))
      (bind _aspuff_ball (cast `PuffBall` _returnvalue))
      ;[1 1 1] Se activa animacion
      (set `PuffBall.StartingSpores` true _aspuff_ball)
      (`AbilityTask_WaitDelay.WaitDelay` 0.25
        (:`then`
          (`GameplayStatics.PlaySoundAtLocation` "/Game/Assets/Music/Enviroment/Hazards/S_PuffballInstant.S_PuffballInstant" _returnvalue_location (struct) 1.0 1.5 0.0 null null null null))
        (:`OnFinish`
          ;[0.2937 1 0.562] Llamo a Pufball
          (set `PuffBall.spawningSpores` true _aspuff_ball)
          (bind _returnvalue_2 (`Actor.K2_GetActorLocation` _aspuff_ball))
          ;[1 0.2674 0.6318] Spawneo en la posición guardada
          (`NiagaraFunctionLibrary.SpawnSystemAtLocation` "/Game/Assets/Actors/Hazards/PuffBall/VFX/NS_PuffBall_Instant.NS_PuffBall_Instant" _returnvalue_2 (struct) (4.0 4.0 4.0))
          ;[0.3364 0.1156 1] Colisión que activa el daño al jugador
          (bind (_asynctaskproxy _actor) (`AbilityTask_OnCollision.OnCollisionAbilityTask` "None" _returnvalue_2 (0.0 0.0 0.0) 200.0 (`self.Ignore Actors`))
            (:`OnCompleted`
              (set `PuffBall.StartingSpores` false _aspuff_ball)
              (set `PuffBall.spawningSpores` false _aspuff_ball)
              ;[0.2806 0.3331 1] Quito los efectos al jugador
              (`AbilitySystemBlueprintLibrary.RemoveLooseGameplayTags` _returnvalue (`self.Gameplay Tags`))
              (`self.K2_EndAbility`))
            (:`OnHit`
              ;[0.1747 1 0.9403] Llamo al player
              (bind _asplayer_character (cast `PlayerCharacter` _actor))
              (bind _returnvalue_3 (`AbilitySystemBlueprintLibrary.GetAbilitySystemComponent` _asplayer_character))
              ;[0.2567 0 1] Aplico habilidad al atributo del player
              (`AbilitySystemComponent.BP_ApplyGameplayEffectToTarget` :`self` _returnvalue_3 :`GameplayEffectClass` "/Game/Blueprints/EffectActors/Ammo1/GE_HealthHazardInstant.GE_HealthHazardInstant_C" :`Target` _returnvalue_3 :`Level` 1.0))))))
    (:`Is Not Valid`
      (`self.K2_EndAbility`))))

(event `self.K2_OnEndAbility`
  (params (bWasCancelled :type Boolean))
  (`AbilitySystemBlueprintLibrary.RemoveLooseGameplayTags` (`self.GetOwningActorFromActorInfo`) (`self.Gameplay Tags_1`)))