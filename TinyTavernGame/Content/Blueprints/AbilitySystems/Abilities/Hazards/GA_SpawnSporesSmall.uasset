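; Gameplay ability for a PuffBall hazard that releases a small spore cloud and poisons players caught in it.
; Activation adds loose tags, flags the puffball as starting and plays a DoOnce-gated sound and Niagara burst.
; After a short delay, a ticking, timed radius collision task applies GE_PoisonSmall to player characters it hits.
; Task completion clears the spore flags and tags, then ends the ability.
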(event `self.K2_ActivateAbility`
  (bind _returnvalue (`self.GetOwningActorFromActorInfo`))
  (bind _returnvalue_location (`KismetMathLibrary.BreakTransform` (`Actor.GetTransform` _returnvalue)))
  (`AbilitySystemBlueprintLibrary.AddLooseGameplayTags` _returnvalue (`self.Gameplay Tags`))
  (bind _aspuff_ball (cast `PuffBall` _returnvalue))
  (set `PuffBall.StartingSpores` true _aspuff_ball)
  (`AbilityTask_WaitDelay.WaitDelay` 0.4
    (:`then`
      (`/Engine/EditorBlueprintResources/StandardMacros.DoOnce` false
        (:`Completed`
          (`GameplayStatics.PlaySoundAtLocation` "/Game/Assets/Music/Enviroment/Hazards/S_Puffball.S_Puffball" _returnvalue_location (struct) 1.5 1.0 0.0 null null null null)
          (bind _returnvalue_2 (`Actor.K2_GetActorLocation` _aspuff_ball))
          (`NiagaraFunctionLibrary.SpawnSystemAtLocation` "/Game/Assets/Enviroment/VFX/PuffBall/NS_PuffBallSmall.NS_PuffBallSmall" _returnvalue_2))))
    (:`OnFinish`
      (set `PuffBall.spawningSpores` true _aspuff_ball)
      (bind (_asynctaskproxy _actor) (`AbilityTask_OnCollision.OnCollisionAbilityTask` "None" _returnvalue_2 (0.0 0.0 0.0) 150.0 (`self.Ignore Actors`) 2.5 true)
        (:`OnCompleted`
          (set `PuffBall.StartingSpores` false _aspuff_ball)
          (set `PuffBall.spawningSpores` false _aspuff_ball)
          (`AbilitySystemBlueprintLibrary.RemoveLooseGameplayTags` _returnvalue (`self.Gameplay Tags`))
          (`self.K2_EndAbility`))
        (:`OnHit`
          (bind _asplayer_character (cast `PlayerCharacter` _actor))
          (bind _returnvalue_3 (`AbilitySystemBlueprintLibrary.GetAbilitySystemComponent` _asplayer_character))
          (`AbilitySystemComponent.BP_ApplyGameplayEffectToTarget` :`self` _returnvalue_3 :`GameplayEffectClass` "/Game/Blueprints/AbilitySystems/Effects/Hazards/GE_PoisonSmall.GE_PoisonSmall_C" :`Target` _returnvalue_3 :`Level` 1.0))))))

(event `self.K2_OnEndAbility`
  (params (bWasCancelled :type Boolean))
  (`AbilitySystemBlueprintLibrary.RemoveLooseGameplayTags` (`self.GetOwningActorFromActorInfo`) (`self.Gameplay Tags_0`)))