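; Gameplay ability for the puffball hazard that releases a spore burst which poisons players caught in it.
; On activation it tags the owner, flags the puffball as starting spores and plays a one-time sound and Niagara burst.
; After a short delay, a ticking, timed OnCollision ability task checks a radius around it and applies GE_Poison to player characters hit.
; When the task completes, it clears the spore flags and ends, removing loose tags.
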(event `self.K2_ActivateAbility`
  (bind _returnvalue (`self.GetOwningActorFromActorInfo`))
  (`/Engine/EditorBlueprintResources/StandardMacros.IsValid` _returnvalue
    (:`Is Valid`
      (`AbilitySystemBlueprintLibrary.AddLooseGameplayTags` _returnvalue (`self.Gameplay Tags`))
      (bind _aspuff_ball (cast `PuffBall` _returnvalue))
      (set `PuffBall.StartingSpores` true _aspuff_ball)
      (`AbilityTask_WaitDelay.WaitDelay` 0.4
        (:`then`
          (`/Engine/EditorBlueprintResources/StandardMacros.DoOnce` false
            (:`Completed`
              (bind _returnvalue_2 (`Actor.K2_GetActorLocation` _aspuff_ball))
              (`GameplayStatics.PlaySoundAtLocation` "/Game/Assets/Music/Enviroment/Hazards/S_Puffball.S_Puffball" _returnvalue_2 (struct) 1.5 1.0 0.0 null null null null)
              (`NiagaraFunctionLibrary.SpawnSystemAtLocation` "/Game/Assets/Enviroment/VFX/PuffBall/NS_PuffBall.NS_PuffBall" _returnvalue_2 (struct) (1.2 1.2 1.2)))))
        (:`OnFinish`
          (set `PuffBall.spawningSpores` true _aspuff_ball)
          (bind (_asynctaskproxy _actor) (`AbilityTask_OnCollision.OnCollisionAbilityTask` "None" _returnvalue_2 (0.0 0.0 0.0) 275.0 (`self.Ignore Actors`) 3.0 true)
            (:`OnCompleted`
              (set `PuffBall.StartingSpores` false _aspuff_ball)
              (set `PuffBall.spawningSpores` false _aspuff_ball)
              (`self.K2_EndAbility`))
            (:`OnHit`
              (bind _asplayer_character (cast `PlayerCharacter` _actor))
              (bind _returnvalue_3 (`AbilitySystemBlueprintLibrary.GetAbilitySystemComponent` _asplayer_character))
              (`AbilitySystemComponent.BP_ApplyGameplayEffectToTarget` :`self` _returnvalue_3 :`GameplayEffectClass` "/Game/Blueprints/AbilitySystems/Effects/Hazards/GE_Poison.GE_Poison_C" :`Target` _returnvalue_3 :`Level` 2.0))))))
    (:`Is Not Valid`
      (`self.K2_EndAbility`))))

(event `self.K2_OnEndAbility`
  (params (bWasCancelled :type Boolean))
  (`self.EndAbility`))

(fn `EndAbility`
  (`AbilitySystemBlueprintLibrary.RemoveLooseGameplayTags` (`self.GetOwningActorFromActorInfo`) (`self.RemoveTag`))
  (`self.K2_EndAbility`))