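; Blood death effect actor that spawns gore and blood decals, presumably when a character dies.
; On BeginPlay it spawns BP_Organs at its location with random rotation and plays a force feedback rumble on the first player's controller.
; A particle data callback turns each received particle into a randomly sized blood decal, oriented against its velocity and given a lifespan and fade-out.
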(event `self.ReceiveBeginPlay`
  ;[0.07756 1 0] Begin Play
  (`|SpawnActorFromClass` "/Game/Blueprints/Character/Commons/BP_Organs.BP_Organs_C" (`KismetMathLibrary.MakeTransform` (`SceneComponent.K2_GetComponentLocation` (`self.DefaultSceneRoot`)) (`KismetMathLibrary.RandomRotator` true)) "Undefined" "MultiplyWithRoot" null null)
  (`PlayerController.K2_ClientPlayForceFeedback` (`GameplayStatics.GetPlayerController` 0) "/Game/Blueprints/Inputs/ForceFeedback/FF_GrillVibration.FF_GrillVibration" "None" false false false))

(event `self.ReceiveParticleData`
  (params (Data :type "Array of BasicParticleData Structure (by ref)") (NiagaraSystem :type "NiagaraSystem Object Reference") (SimulationPositionOffset :type "Vector Structure (by ref)"))
  (bind _decalsize (`self.DecalSize`))
  ;[0.7687 0.7912 1] Receive Particles Data
  (for _array_element Data
    (bind (_position _size _velocity) (break `BasicParticleData` _array_element))
    (bind _returnvalue (`GameplayStatics.SpawnDecalAtLocation` "/Game/Assets/Enemies/Commons/VFX/BLOODNGORE/MI_BloodDecal.MI_BloodDecal" (`KismetMathLibrary.Conv_DoubleToVector` (`KismetMathLibrary.Lerp` (* _decalsize 0.1) _decalsize (`KismetMathLibrary.RandomFloatInRange` 1.0 3.0))) _position (`KismetMathLibrary.Conv_VectorToRotator` (* _velocity -1.0)) 4.0))
    (`DecalComponent.SetFadeOut` _returnvalue 10.0 15.0 true)))

(fn `UserConstructionScript`)