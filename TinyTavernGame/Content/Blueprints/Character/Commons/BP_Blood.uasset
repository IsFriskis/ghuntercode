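; Blood effect actor that plays a Niagara blood system and leaves decals at the positions its particles report.
; On BeginPlay it registers itself as the Niagara export callback and sets the system's custom time dilation to offset the current global dilation.
; Each exported particle spawns a randomly sized blood decal, oriented against the particle's velocity, that fades out after a delay.
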(event `self.ReceiveBeginPlay`
  (bind _ns_blood (`self.NS_Blood`))
  (`NiagaraComponent.SetVariableObject` _ns_blood "BP_Blood" self)
  (`NiagaraComponent.SetCustomTimeDilation` _ns_blood (/ 1.0 (`GameplayStatics.GetGlobalTimeDilation`))))

(event `self.ReceiveParticleData`
  (params (Data :type "Array of BasicParticleData Structure (by ref)") (NiagaraSystem :type "NiagaraSystem Object Reference") (SimulationPositionOffset :type "Vector Structure (by ref)"))
  (bind _decalsize (`self.Decalsize`))
  (for _array_element Data
    (bind (_position _size _velocity) (break `BasicParticleData` _array_element))
    (bind _returnvalue (`GameplayStatics.SpawnDecalAtLocation` "/Game/Assets/Enemies/Commons/VFX/BLOODNGORE/MI_BloodDecal.MI_BloodDecal" (`KismetMathLibrary.Conv_DoubleToVector` (`KismetMathLibrary.Lerp` (* _decalsize (`KismetMathLibrary.RandomFloatInRange` 0.4 2.5)) _decalsize (`KismetMathLibrary.RandomFloatInRange` 0.0 1.0))) _position (`KismetMathLibrary.Conv_VectorToRotator` (* _velocity -1.0))))
    (`DecalComponent.SetFadeOut` _returnvalue 5.0 5.0 true)))

(fn `UserConstructionScript`)