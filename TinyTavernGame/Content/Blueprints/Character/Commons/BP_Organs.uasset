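; BP_Organs is a short-lived gore actor that displays a randomized set of scattered organs.
; On BeginPlay, each of its four ScatterGoreRigg components independently picks a skeletal mesh from SMOrgansArrayChoices, so duplicates can occur.
; A one-shot timer then fires CE_EndOrgans, which destroys the actor after 15 seconds.
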(event `self.ReceiveBeginPlay`
  (bind _outitem (`KismetArrayLibrary.Array_Random` (`self.SM_OrgansArrayChoices`)))
  ;[0 1 0.2364] Begin Play
  (`SkeletalMeshComponent.SetSkeletalMeshAsset` (`self.ScatterGore_rigg`) _outitem)
  (`SkeletalMeshComponent.SetSkeletalMeshAsset` (`self.ScatterGore_rigg1`) _outitem)
  (`SkeletalMeshComponent.SetSkeletalMeshAsset` (`self.ScatterGore_rigg2`) _outitem)
  (`SkeletalMeshComponent.SetSkeletalMeshAsset` (`self.ScatterGore_rigg3`) _outitem)
  (`KismetSystemLibrary.K2_SetTimerDelegate` (delegate `CE_EndOrgans`) 15.0))

(event `CE_EndOrgans`
  ;[0 1 0.2364] Begin Play
  (`self.K2_DestroyActor`))

(fn `UserConstructionScript`)