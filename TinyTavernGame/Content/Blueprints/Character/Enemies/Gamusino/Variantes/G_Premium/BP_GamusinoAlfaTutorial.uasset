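; Tutorial Alfa variant of the premium Gamusino enemy, extending its parent's BeginPlay with alert widget binding and a spawn material effect.
; On BeginPlay it registers itself as the Enemy of its WBP_AlertIndicator widget, stopping there if the cast fails.
; A timeline then animates the mesh's BurnDisappearance parameter and, on finish, swaps slot 0 to the premium Gamusino body material.
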(event `self.ReceiveBeginPlay`
  (bind _mesh (`self.Mesh`))
  (`parent.ReceiveBeginPlay`)
  (bind _aswbp_alert_indicator (cast `/Game/Blueprints/UI/HUD/3DHuds/WBP_AlertIndicator` (`WidgetComponent.GetWidget` (`self.WidgetAlerta`))))
  (set `/Game/Blueprints/UI/HUD/3DHuds/WBP_AlertIndicator.Enemy` self _aswbp_alert_indicator)
  (bind (_direction _newtrack_0) (`Timeline|Timeline`)
    (:`Update`
      (`MeshComponent.SetScalarParameterValueOnMaterials` _mesh "BurnDisappearance" _newtrack_0))
    (:`Finished`
      (`PrimitiveComponent.SetMaterial` _mesh 0 "/Game/Assets/Enemies/Gamusino/Variantes/Yeti/MI_cuerpogamusinopremium.MI_cuerpogamusinopremium"))))

(fn `UserConstructionScript`
  (`parent.UserConstructionScript`))