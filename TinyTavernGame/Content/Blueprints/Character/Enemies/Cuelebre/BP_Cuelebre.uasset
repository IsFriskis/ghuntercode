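; Cuelebre enemy that flies along a spline, optionally looping, and heals the player when killed by a dash attack.
; Body and wings play looping idle animations, with physics simulation enabled from a spine bone down.
; Tick moves the body mesh along the spline with fixed offsets.
; If OnDash is set, overlapping a dash-attacking player applies a GAS heal, plays death feedback, spawns a drop, reports the achievement and destroys the actor.
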(event `self.ReceiveBeginPlay`
  ;[0.2363 1 0] Begin Play
  (`SkeletalMeshComponent.SetAllBodiesPhysicsBlendWeight` (`self.Cuelebre`) 0.0 false)
  (`SkeletalMeshComponent.SetAllBodiesBelowSimulatePhysics` (`self.Cuelebre`) "spine05_c_twinSkn" true true)
  (`SkeletalMeshComponent.PlayAnimation` (`self.Cuelebre`) "/Game/Assets/Enemies/Cuelebre/Cuelebre_Idle.Cuelebre_Idle" true)
  (`SkeletalMeshComponent.PlayAnimation` (`self.Cuelebre_Alas`) "/Game/Assets/Enemies/Cuelebre/Cuelebre_Alas_Idle.Cuelebre_Alas_Idle" true))

(event `self.ReceiveTick`
  (params (DeltaSeconds :type "Float (single-precision)"))
  (bind _returnvalue (`SplineComponent.GetTransformAtDistanceAlongSpline` (`self.Spline`) (`self.Distance Along Spline`) "Local" false))
  ;[1 0.7891 0] Tick
  ;;[1 1 1] Follow Spline
  (if (!= (`self.Spline`) null)
    (set `self.Distance Along Spline` (+ (* DeltaSeconds (`self.Speed`)) (`self.Distance Along Spline`)))
    (`SceneComponent.K2_SetRelativeTransform` (`self.Cuelebre`) (`KismetMathLibrary.MakeTransform` (`KismetMathLibrary.MakeVector` (.x (.location _returnvalue)) (.y (.location _returnvalue)) (+ (.z (.location _returnvalue)) -90.0)) (`KismetMathLibrary.MakeRotator` (.roll (.rotation _returnvalue)) (.pitch (.rotation _returnvalue)) (+ (.yaw (.rotation _returnvalue)) -90.0)) (`SceneComponent.RelativeScale3D` (`self.Cuelebre`))) false false)
    (if (`self.Loop`)
      (if (< (`SplineComponent.GetSplineLength` (`self.Spline`)) (`self.Distance Along Spline`))
        (set `self.Distance Along Spline` 0.0)))))

(event `self.Capsule.OnComponentBeginOverlap`
  (params (OverlappedComponent :type "PrimitiveComponent Object Reference") (OtherActor :type "Actor Object Reference") (OtherComp :type "PrimitiveComponent Object Reference") (OtherBodyIndex :type Integer) (bFromSweep :type Boolean) (SweepResult :type "HitResult Structure (by ref)"))
  (bind _returnvalue (`SceneComponent.K2_GetComponentLocation` (`self.ChildActor`)))
  ;[1 1 1] Begin Overlap
  (if (`self.OnDash`)
    ;;[1 0.1354 0.1354] Cuando choca con el jugador dasheando explota y cura al jugador
    (bind _asplayer_character (cast `PlayerCharacter` OtherActor))
    (bind _returnvalue_2 (`AbilitySystemBlueprintLibrary.GetAbilitySystemComponent` _asplayer_character))
    (if (`GameplayTagAssetInterface.HasMatchingGameplayTag` _returnvalue_2 (struct :`TagName` "States.OnDashAttack"))
      (`AbilitySystemComponent.BP_ApplyGameplayEffectToTarget` :`self` _returnvalue_2 :`GameplayEffectClass` "/Game/Blueprints/EffectActors/Ammo1/GE_HealthHeal.GE_HealthHeal_C" :`Target` _returnvalue_2)
      (`NiagaraFunctionLibrary.SpawnSystemAtLocation` "/Game/Assets/Enemies/Commons/VFX/BLOODNGORE/NS_bLOODgreen.NS_bLOODgreen" (`SceneComponent.K2_GetComponentLocation` (`self.Cuelebre_Alas`)))
      (`PlayerController.K2_ClientPlayForceFeedback` (`GameplayStatics.GetPlayerController` 0) "/Game/Blueprints/Inputs/ForceFeedback/FF_GrillVibration.FF_GrillVibration" "None" false false false)
      (`GameplayStatics.PlaySoundAtLocation` "/Game/Assets/Music/Enemy/Gamusino/MS_DeathSplash.MS_DeathSplash" _returnvalue (struct) 1.0 1.0 0.0 null null null null)
      (`GameplayStatics.PlaySoundAtLocation` "/Game/Assets/Music/Enviroment/S_Curación.S_Curación" _returnvalue (struct) 1.0 1.0 0.5 null null null null)
      (`|SpawnActorFromClass` "/Game/Blueprints/Character/Enemies/Cuelebre/BP_CuelebreDrop.BP_CuelebreDrop_C" (`KismetMathLibrary.Conv_VectorToTransform` _returnvalue) "Undefined" "MultiplyWithRoot" null null)
      ;;[1 1 1] Achievement
      (bind _astt_game_instance (cast `TT_GameInstance` (`GameplayStatics.GetGameInstance`)))
      (`TT_GameInstance.FirstCuelebre` _astt_game_instance)
      (`self.K2_DestroyActor`))))

(fn `UserConstructionScript`)