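; Cucafera premium ghost enemy that passes cooking damage back to its Parent Cucafera when destroyed while cooked and vulnerable.
; On Destroyed, its boiled, fried or grilled tag becomes the SetByCaller tag for GE_CucaferaGhostDamage.
; The effect hits Parent and its GhostAlliesArray, scaled by each one's RawPoint and per-ghost share of TotalGhostsDamage.
; It also removes itself from its allies' lists, and hides its alert widget at BeginPlay.
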(event `self.ReceiveBeginPlay`
  (`parent.ReceiveBeginPlay`)
  (bind _aswbp_alert_indicator (cast `/Game/Blueprints/UI/HUD/3DHuds/WBP_AlertIndicator` (`WidgetComponent.GetWidget` (`self.WidgetAlerta_0`))))
  (set `/Game/Blueprints/UI/HUD/3DHuds/WBP_AlertIndicator.Enemy` self _aswbp_alert_indicator)
  (`Widget.SetVisibility` _aswbp_alert_indicator "Hidden"))

(event `self.ReceiveTick`
  (params (DeltaSeconds :type "Float (single-precision)"))
  (`parent.ReceiveTick` DeltaSeconds))

(event `self.ReceiveDestroyed`
  (bind _tag_containerghost (`self.Tag ContainerGhost`))
  (bind _tag_containerghost_2 (`self.Tag ContainerGhost`))
  (bind _parent (`self.Parent`))
  (bind _returnvalue (`AbilitySystemBlueprintLibrary.GetAbilitySystemComponent` _parent))
  (set `self.Tag ContainerGhost` (`GameplayTagAssetInterface.GetOwnedGameplayTags` (`AbilitySystemBlueprintLibrary.GetAbilitySystemComponent` self)))
  (if (and (`BlueprintGameplayTagLibrary.HasTag` _tag_containerghost (struct :`TagName` "States.Cook")) (`BlueprintGameplayTagLibrary.HasTag` _tag_containerghost (struct :`TagName` "States.Vulnerable")))
    (`AbilitySystemBlueprintLibrary.RemoveLooseGameplayTags` (`self.Parent`) (`self.CookTag`))
    (if (`BlueprintGameplayTagLibrary.HasTag` _tag_containerghost_2 (struct :`TagName` "States.Cook.Boiled") true)
      (`AbilitySystemBlueprintLibrary.AddLooseGameplayTags` null (`self.BoiledTag`))
      (set `self.CurrentCookingType` (struct :`TagName` "States.Cook.Boiled"))
      (`/Engine/EditorBlueprintResources/StandardMacros.IsValid` _returnvalue :!label _label
        (:`Is Valid`
          (bind _output_get (set `self.AmountDamage` (`KismetMathLibrary.FTrunc` (/ (* (/ (`EnemyCucafera.TotalGhostsDamage` _parent) (`self.Ghost_Num`)) (`EnemyBase.RawPoint` _parent)) 100.0))))
          (bind _returnvalue_2 (`AbilitySystemBlueprintLibrary.AssignTagSetByCallerMagnitude` (`AbilitySystemComponent.MakeOutgoingSpec` :`self` _returnvalue :`GameplayEffectClass` "/Game/Blueprints/AbilitySystems/Effects/Enemies/Cucafera/GE_CucaferaGhostDamage.GE_CucaferaGhostDamage_C") (`self.CurrentCookingType`) (`KismetMathLibrary.Conv_IntToDouble` _output_get)))
          (`AbilitySystemComponent.BP_ApplyGameplayEffectSpecToTarget` _returnvalue _returnvalue_2 _returnvalue)
          (for _array_element (`EnemyCucafera.GhostAlliesArray` _parent)
            (bind _asenemy_cucafera (cast `EnemyCucafera` _array_element))
            (bind _returnvalue_3 (`AbilitySystemBlueprintLibrary.GetAbilitySystemComponent` _asenemy_cucafera))
            (`/Engine/EditorBlueprintResources/StandardMacros.IsValid` _returnvalue_3
              (:`Is Valid`
                (bind _output_get_2 (set `self.AmountDamage` (`KismetMathLibrary.FTrunc` (/ (* (/ (`EnemyCucafera.TotalGhostsDamage` _asenemy_cucafera) (`self.Ghost_Num`)) (`EnemyBase.RawPoint` _asenemy_cucafera)) 100.0))))
                (bind _returnvalue_4 (`AbilitySystemBlueprintLibrary.AssignTagSetByCallerMagnitude` (`AbilitySystemComponent.MakeOutgoingSpec` :`self` _returnvalue_3 :`GameplayEffectClass` "/Game/Blueprints/AbilitySystems/Effects/Enemies/Cucafera/GE_CucaferaGhostDamage.GE_CucaferaGhostDamage_C") (`self.CurrentCookingType`) (`KismetMathLibrary.Conv_IntToDouble` _output_get_2)))
                (`AbilitySystemComponent.BP_ApplyGameplayEffectSpecToTarget` _returnvalue_3 _returnvalue_4 _returnvalue_3)
                (for _array_element_2 (`EnemyCucafera.GhostAlliesArray`)
                  (bind _asenemy_cucafera_2 (cast `EnemyCucafera` _array_element_2))
                  (`KismetArrayLibrary.Array_RemoveItem` (`EnemyCucafera.GhostAlliesArray` _asenemy_cucafera_2) self)))))))
      (elif (`BlueprintGameplayTagLibrary.HasTag` _tag_containerghost_2 (struct :`TagName` "States.Cook.Fried") true)
        (`AbilitySystemBlueprintLibrary.AddLooseGameplayTags` null (`self.FryTag`))
        (set `self.CurrentCookingType` (struct :`TagName` "States.Cook.Fried"))
        (goto _label)
        (elif (`BlueprintGameplayTagLibrary.HasTag` _tag_containerghost_2 (struct :`TagName` "States.Cook.Grilled") true)
          (`AbilitySystemBlueprintLibrary.AddLooseGameplayTags` null (`self.Grilled Tag`))
          (set `self.CurrentCookingType` (struct :`TagName` "States.Cook.Grilled"))
          (goto _label))))))

(fn `SetParent`
  (params (Parent :type "/Game/Blueprints/Character/Enemies/Cucafera/BP_CucaferaPremium Object Reference"))
  (set `self.Parent` Parent))

(fn `UserConstructionScript`
  (`parent.UserConstructionScript`))