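; BP_CucaferaPremium is the premium Cucafera enemy Blueprint, extending parent enemy behavior.
; BeginPlay links its alert indicator widget to itself.
; Tick polls gameplay tags while FirstHit is set, applying GE_CucaferaAttributes to itself and clearing the flag once it is Spectral and either Damaged or Alert.
; On destruction, it destroys every valid ghost ally in GhostAlliesArray.
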(event `self.ReceiveBeginPlay`
  (`parent.ReceiveBeginPlay`)
  (bind _aswbp_alert_indicator (cast `/Game/Blueprints/UI/HUD/3DHuds/WBP_AlertIndicator` (`WidgetComponent.GetWidget` (`self.WidgetAlerta_0`))))
  (set `/Game/Blueprints/UI/HUD/3DHuds/WBP_AlertIndicator.Enemy` self _aswbp_alert_indicator))

(event `self.ReceiveTick`
  (params (DeltaSeconds :type "Float (single-precision)"))
  (bind _returnvalue (`AbilitySystemBlueprintLibrary.GetAbilitySystemComponent` null))
  (bind _firsthit (`self.FirstHit`))
  (if _firsthit
    (if (or (and _firsthit (`GameplayTagAssetInterface.HasMatchingGameplayTag` _returnvalue (struct :`TagName` "States.Damaged")) (`GameplayTagAssetInterface.HasMatchingGameplayTag` _returnvalue (struct :`TagName` "Enemy.Cucafera.Spectral"))) (and (`GameplayTagAssetInterface.HasMatchingGameplayTag` _returnvalue (struct :`TagName` "States.Alert")) (`GameplayTagAssetInterface.HasMatchingGameplayTag` _returnvalue (struct :`TagName` "Enemy.Cucafera.Spectral"))))
      (set `self.FirstHit` false)
      (`AbilitySystemComponent.BP_ApplyGameplayEffectToSelf` :`self` (`AbilitySystemBlueprintLibrary.GetAbilitySystemComponent` null) :`GameplayEffectClass` "/Game/Blueprints/AbilitySystems/Effects/Enemies/Cucafera/GE_CucaferaAttributes.GE_CucaferaAttributes_C"))))

(event `self.ReceiveDestroyed`
  (for _array_element (`self.GhostAlliesArray`)
    (`/Engine/EditorBlueprintResources/StandardMacros.IsValid` _array_element
      (:`Is Valid`
        (`self.K2_DestroyActor` _array_element)))))

(fn `UserConstructionScript`)