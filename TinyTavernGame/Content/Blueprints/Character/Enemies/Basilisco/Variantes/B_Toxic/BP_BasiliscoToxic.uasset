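; Toxic variant of the Basilisco enemy, a child Blueprint that leaves its behavior to the parent class.
; On BeginPlay it runs the parent logic, then casts the WidgetAlerta component's widget to WBP_AlertIndicator and registers itself as that indicator's Enemy.
; The construction script only calls the parent, and the overlap and Tick events are disabled stubs, so the graphs hold no toxic-specific logic.
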(event `self.ReceiveBeginPlay`
  (`parent.ReceiveBeginPlay`)
  (bind _aswbp_alert_indicator (cast `/Game/Blueprints/UI/HUD/3DHuds/WBP_AlertIndicator` (`WidgetComponent.GetWidget` (`self.WidgetAlerta`))))
  (set `/Game/Blueprints/UI/HUD/3DHuds/WBP_AlertIndicator.Enemy` self _aswbp_alert_indicator))

(fn `UserConstructionScript`
  (`parent.UserConstructionScript`))