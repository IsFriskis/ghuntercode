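; BP_ToxicSpores is a temporary poison area for the toxic Basilisco enemy variant.
; On spawn it plays a Niagara toxic effect at its location, then destroys itself after ActiveTime.
; A sphere overlap caches the player and toggles InPoison on enter and exit.
; While InPoison is set, Tick applies GE_Poison through the player's own Ability System Component and shows the poison notification every frame.
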(event `self.ReceiveTick`
  (params (DeltaSeconds :type "Float (single-precision)"))
  (bind _as_player_character (`self.As Player Character`))
  (bind _returnvalue (`AbilitySystemBlueprintLibrary.GetAbilitySystemComponent` _as_player_character))
  (if (`self.InPoison`)
    (`AbilitySystemComponent.BP_ApplyGameplayEffectToTarget` :`self` _returnvalue :`GameplayEffectClass` "/Game/Blueprints/AbilitySystems/Effects/Hazards/GE_Poison.GE_Poison_C" :`Target` _returnvalue :`Level` 1.0)
    (`PlayerCharacter.DisplayNotificationPopUp` _as_player_character (struct :`TagName` "Notification.Poison"))))

(event `self.ReceiveBeginPlay`
  (`NiagaraFunctionLibrary.SpawnSystemAtLocation` "/Game/Assets/Enviroment/VFX/PuffBall/NS_ToxicBasilisco.NS_ToxicBasilisco" (`self.K2_GetActorLocation`))
  (`KismetSystemLibrary.Delay` (`self.ActiveTime`))
  (`self.K2_DestroyActor`))

(event `self.Sphere.OnComponentBeginOverlap`
  (params (OverlappedComponent :type "PrimitiveComponent Object Reference") (OtherActor :type "Actor Object Reference") (OtherComp :type "PrimitiveComponent Object Reference") (OtherBodyIndex :type Integer) (bFromSweep :type Boolean) (SweepResult :type "HitResult Structure (by ref)"))
  (bind _asplayer_character (cast `PlayerCharacter` OtherActor))
  (set `self.As Player Character` _asplayer_character)
  (set `self.InPoison` true))

(event `self.Sphere.OnComponentEndOverlap`
  (params (OverlappedComponent :type "PrimitiveComponent Object Reference") (OtherActor :type "Actor Object Reference") (OtherComp :type "PrimitiveComponent Object Reference") (OtherBodyIndex :type Integer))
  (cast `PlayerCharacter` OtherActor)
  (set `self.InPoison` false))

(fn `UserConstructionScript`)