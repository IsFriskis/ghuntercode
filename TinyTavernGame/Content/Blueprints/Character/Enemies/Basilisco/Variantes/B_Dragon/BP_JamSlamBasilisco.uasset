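; Falling fire projectile for the dragon Basilisco variant's JamSlam, exploding on impact to damage the player.
; Each Tick sweeps it straight down and traces below to place a landing indicator, lowering the offset when the trace hits the player.
; Impact spawns explosion VFX and sound, then enables hitbox collision for 0.2 seconds before destruction.
; Box overlap applies a damage GameplayEffect through the player's own Ability System Component.
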(event `self.ReceiveTick`
  (params (DeltaSeconds :type "Float (single-precision)"))
  (bind _returnvalue (`self.K2_GetActorLocation`))
  ;[1 1 1] Update projectile pos
  (bind _outhit (`KismetSystemLibrary.LineTraceSingle` :`Start` _returnvalue :`End` (+ _returnvalue (0.0 0.0 -800.0)) :`TraceChannel` "TraceTypeQuery1" :`DrawTime` 2.0))
  (cast `PlayerCharacter` (`.HitActor` (`GameplayStatics.BreakHitResult` _outhit))
    (:`then`
      (set `self.Height` -50.0))
    (:`CastFailed`
      (set `self.Height` 50.0)))
  (`SceneComponent.K2_SetWorldLocation` (`self.Indicator`) (`KismetMathLibrary.MakeVector` (.x (`.Location` (`GameplayStatics.BreakHitResult` _outhit))) (.y (`.Location` (`GameplayStatics.BreakHitResult` _outhit))) (+ (`self.Height`) (.z (`.Location` (`GameplayStatics.BreakHitResult` _outhit))))) false false)
  (`self.K2_SetActorTransform` (`KismetMathLibrary.MakeTransform` (+ (`self.K2_GetActorLocation`) (* (* DeltaSeconds (`self.Speed`)) (0.0 0.0 -1.0)))) true))

(event `self.Box.OnComponentBeginOverlap`
  (params (OverlappedComponent :type "PrimitiveComponent Object Reference") (OtherActor :type "Actor Object Reference") (OtherComp :type "PrimitiveComponent Object Reference") (OtherBodyIndex :type Integer) (bFromSweep :type Boolean) (SweepResult :type "HitResult Structure (by ref)"))
  ;[1 1 1] Hitbox
  (bind _asplayer_character (cast `PlayerCharacter` OtherActor))
  (bind _returnvalue (`AbilitySystemBlueprintLibrary.GetAbilitySystemComponent` _asplayer_character))
  (`AbilitySystemComponent.BP_ApplyGameplayEffectToTarget` :`self` _returnvalue :`GameplayEffectClass` "/Game/Blueprints/AbilitySystems/Effects/Damage/GE_Damage_2.GE_Damage_2_C" :`Target` _returnvalue))

(event `self.ProjectileCollision.OnComponentHit`
  (params (HitComponent :type "PrimitiveComponent Object Reference") (OtherActor :type "Actor Object Reference") (OtherComp :type "PrimitiveComponent Object Reference") (NormalImpulse :type "Vector Structure") (Hit :type "HitResult Structure (by ref)"))
  (bind (_bblockinghit _binitialoverlap _time _distance _location _impactpoint _normal _impactnormal) (`GameplayStatics.BreakHitResult` Hit))
  (bind (_returnvalue_roll _returnvalue_pitch _returnvalue_yaw) (`KismetMathLibrary.BreakRotator` (`KismetMathLibrary.Conv_VectorToRotator` _impactnormal)))
  ;[1 1 1] OnCollide SpawnNiagara and Hitbox
  (if (!= OtherActor (`self.HitObject`))
    (set `self.HitObject` OtherActor)
    (`NiagaraFunctionLibrary.SpawnSystemAtLocation` "/Game/Assets/Enemies/Basilisco/VFX/NS_FireExplosion.NS_FireExplosion" _impactpoint (`KismetMathLibrary.MakeRotator` _returnvalue_roll (+ _returnvalue_pitch -90.0) _returnvalue_yaw))
    (`GameplayStatics.PlaySoundAtLocation` "/Game/Assets/Music/Enemy/Basilisco/S_BasiliscoFireExplosion.S_BasiliscoFireExplosion" _impactpoint (struct) 1.0 1.0 0.0 null null null null)
    (`PrimitiveComponent.SetCollisionEnabled` (`self.ExplosionCollion`) "QueryAndPhysics")
    (`PrimitiveComponent.SetCollisionEnabled` (`self.Box`) "QueryAndPhysics")
    (`KismetSystemLibrary.Delay` 0.2)
    (`self.K2_DestroyActor`)))

(fn `UserConstructionScript`)