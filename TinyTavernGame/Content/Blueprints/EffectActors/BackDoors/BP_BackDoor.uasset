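; BP_BackDoor is an effect actor for a back door, providing the feedback when it activates.
; DoorActivate plays controller vibration and a scaled camera shake on player 0, activates the door audio and spawns a Niagara dust burst at the Scene component.
; DoorEnd disables collision on the door mesh.
; Both events are triggered from outside this Blueprint, which contains no door movement logic.
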(event `self.BP_DoorActivate`
  (bind _returnvalue (`GameplayStatics.GetPlayerController` 0))
  (bind _scene (`self.Scene`))
  (`PlayerController.K2_ClientPlayForceFeedback` _returnvalue "/Game/Blueprints/Inputs/FF_Vibration.FF_Vibration" "None" false false false)
  (`PlayerController.ClientStartCameraShake` :`self` _returnvalue :`Shake` "/Game/Blueprints/Actors/Adventure/Backdoors/BP_CameraBackdoorShake.BP_CameraBackdoorShake_C" :`Scale` 0.3 :`PlaySpace` "World")
  (`ActorComponent.Activate` (`self.BackDoorAudio`) false)
  (`NiagaraFunctionLibrary.SpawnSystemAtLocation` "/Game/Assets/Actors/Adventure/Statues/VFX/NS_StatueDust_B.NS_StatueDust_B" (`SceneComponent.K2_GetComponentLocation` _scene) (`SceneComponent.K2_GetComponentRotation` _scene)))

(event `self.BP_DoorEnd`
  (`PrimitiveComponent.SetCollisionEnabled` (`self.BackDoorMesh`) "NoCollision"))

(fn `UserConstructionScript`)