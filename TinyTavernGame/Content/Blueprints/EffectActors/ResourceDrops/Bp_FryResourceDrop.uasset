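; Fry resource drop pickup that a player character collects by overlapping its box.
; On overlap it reads the base values of a configurable current and max attribute from the player's Ability System Component.
; Only when both attributes exist and the current value is below max does it call PlayerOnOverlap, destroy itself and play a 2D collection sound, so a full player leaves the drop in place.
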(event `self.Box.OnComponentBeginOverlap`
  (params (OverlappedComponent :type "PrimitiveComponent Object Reference") (OtherActor :type "Actor Object Reference") (OtherComp :type "PrimitiveComponent Object Reference") (OtherBodyIndex :type Integer) (bFromSweep :type Boolean) (SweepResult :type "HitResult Structure (by ref)"))
  (bind _asplayer_character (cast `PlayerCharacter` OtherActor))
  (bind _returnvalue (`AbilitySystemBlueprintLibrary.GetAbilitySystemComponent` _asplayer_character))
  (bind (_bsuccessfullyfoundattribute _returnvalue_2) (`AbilitySystemBlueprintLibrary.GetFloatAttributeBaseFromAbilitySystemComponent` _returnvalue (`self.MaxAttribute`)))
  (if _bsuccessfullyfoundattribute
    (bind (_bsuccessfullyfoundattribute_2 _returnvalue_3) (`AbilitySystemBlueprintLibrary.GetFloatAttributeBaseFromAbilitySystemComponent` _returnvalue (`self.ValueAttribute`)))
    (if _bsuccessfullyfoundattribute_2
      (if (not (>= _returnvalue_3 _returnvalue_2))
        (`self.PlayerOnOverlap` _asplayer_character)
        (`self.K2_DestroyActor`)
        (`GameplayStatics.PlaySound2D` "/Game/Assets/Music/Player/S_ResourceCollection.S_ResourceCollection" 1.0 1.0 0.0 null null)))))

(fn `UserConstructionScript`)