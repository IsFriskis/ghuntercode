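; BP_PuffBallinstant is a puffball hazard actor that reacts when a player character enters or leaves its sphere trigger.
; Begin overlap adds loose gameplay tags, intended as player stat-loss effects, and end overlap removes them.
; Both calls target the hazard itself rather than the overlapping player, and only the removal is set to replicate.
; The construction script sets a fixed animation rate.
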(event `self.SphereTriggerShape.OnComponentBeginOverlap`
  (params (OverlappedComponent :type "PrimitiveComponent Object Reference") (OtherActor :type "Actor Object Reference") (OtherComp :type "PrimitiveComponent Object Reference") (OtherBodyIndex :type Integer) (bFromSweep :type Boolean) (SweepResult :type "HitResult Structure (by ref)"))
  ;[0.05306 0.2053 1] Entra al collider
  ;[1 0.06383 0.7308] Llamo al player
  (cast `PlayerCharacter` OtherActor)
  ;[0.2806 0.3331 1] Función que hace que pierda stats el jugador
  (`AbilitySystemBlueprintLibrary.AddLooseGameplayTags` self (`self.Gameplay Tags`)))

(event `self.SphereTriggerShape.OnComponentEndOverlap`
  (params (OverlappedComponent :type "PrimitiveComponent Object Reference") (OtherActor :type "Actor Object Reference") (OtherComp :type "PrimitiveComponent Object Reference") (OtherBodyIndex :type Integer))
  ;[0.05306 0.2053 1] Salgo dell collider
  ;[1 0.06383 0.7308] Llamo al player
  (cast `PlayerCharacter` OtherActor)
  ;[0.2806 0.3331 1] Quito los efectos al jugador
  (`AbilitySystemBlueprintLibrary.RemoveLooseGameplayTags` self (`self.Gameplay Tags`) true))

(fn `UserConstructionScript`
  (set `self.animRate` 4.0))