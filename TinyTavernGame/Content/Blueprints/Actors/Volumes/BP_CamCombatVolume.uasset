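; BP_CamCombatVolume is a volume that switches the level music between states when the player overlaps it.
; On BeginPlay it caches the first AmbientSound actor tagged "Music".
; On overlap, if the game instance's TriggerFantasyMusic differs from the volume's ToCombatCam, it fires the fantasy and tension toggle triggers on that audio component.
; It then flips the persistent flag, so repeat entries do not re-toggle.
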(event `self.ReceiveBeginPlay`
  (bind _outactors (`GameplayStatics.GetAllActorsOfClassWithTag` "/Script/Engine.AmbientSound" "Music"))
  (set `self.AmbientSoundBP` (`|GetArrayItem` _outactors)))

(event `self.ReceiveActorBeginOverlap`
  (params (OtherActor :type "Actor Object Reference"))
  (bind _audiocomponent (`AmbientSound.AudioComponent` (`self.AmbientSoundBP`)))
  (cast `PlayerCharacter` OtherActor)
  (bind _asbp_ttgame_instance (cast `/Game/Blueprints/Game/BP_TTGameInstance` (`GameplayStatics.GetGameInstance`)))
  (bind _triggerfantasymusic (`TT_GameInstance.TriggerFantasyMusic` _asbp_ttgame_instance))
  (if (not (== _triggerfantasymusic (`self.bToCombatCam`)))
    (`AudioParameterControllerInterface.SetTriggerParameter` _audiocomponent "ToggleFantasy")
    (`AudioParameterControllerInterface.SetTriggerParameter` _audiocomponent "ToggleTension")
    (set `TT_GameInstance.TriggerFantasyMusic` (not _triggerfantasymusic) _asbp_ttgame_instance)))

(fn `UserConstructionScript`)