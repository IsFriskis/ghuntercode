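; BP_FryResource is a harvestable world resource that gives the player fry ammo.
; A trigger tracks the player and highlights the mesh when melee tier suffices, though interaction only checks ammo capacity and the weapons-blocked tag.
; Interacting motion-warps the player into a skewer montage with timed VFX and a BP_DropFry spawn.
; When the montage ends, it restores the ranged weapon, applies the ammo GameplayEffect and destroys itself.
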(event `self.ReceiveBeginPlay`
  ;[0.03834 1 0] Begin Play
  (bind _astt_game_instance (cast `TT_GameInstance` (`GameplayStatics.GetGameInstance`)))
  (set `self.TTGameInstance` _astt_game_instance)
  (set `self.AmmoEffectToBeApplied` "/Game/Blueprints/AbilitySystems/Effects/Resources/GE_AddAmmoFry.GE_AddAmmoFry_C"))

(event `EnhancedInput|/Game/Blueprints/Inputs/InputActions/IA_Interact`
  (params (ActionValue :type Boolean) (ElapsedSeconds :type "Float (double-precision)") (TriggeredSeconds :type "Float (double-precision)") (InputAction :type "InputAction Object Reference" :default "/Game/Blueprints/Inputs/InputActions/IA_Interact.IA_Interact"))
  (bind _motionwarpinglocation (`self.MotionWarpingLocation`))
  (bind _player (`self.Player`))
  (bind _playerinside (`self.PlayerInside`))
  (bind _returnvalue (`AbilitySystemBlueprintLibrary.GetAbilitySystemComponent` (`self.Player`)))
  ;[1 0.9507 0] INTERACT
  (:`Started`
    (if _playerinside
      ;;[1 0.3294 0.8534] CUANDO PLAYER ESTÁ EN COLISON = TRUE
      (if (and _playerinside (< (`.ReturnValue` (`AbilitySystemBlueprintLibrary.GetFloatAttributeBaseFromAbilitySystemComponent` _returnvalue (`self.ValueAttribute`))) (`.ReturnValue` (`AbilitySystemBlueprintLibrary.GetFloatAttributeBaseFromAbilitySystemComponent` _returnvalue (`self.MaxAttribute`)))) (not (`GameplayTagAssetInterface.HasMatchingGameplayTag` _returnvalue (struct :`TagName` "States.WeaponsBlocked"))))
        (set `self.PlayerInside` false)
        ;;[0 0.09699 1] Play Montage, change mesh and disable any other action
        (`AbilitySystemBlueprintLibrary.AddLooseGameplayTags` _player (`self.WeaponsBlockedTag`))
        (`AbilitySystemBlueprintLibrary.RemoveLooseGameplayTags` _player (`self.AimingTag`))
        (`WeaponComponent.ChangeWeaponForDash` (`PlayerCharacter.WeaponComponent` _player))
        (`MotionWarpingComponent.AddOrUpdateWarpTarget` (`PlayerCharacter.PlayerMotionWarping` _player) (make `MotionWarpingTarget` "Cut" (`SceneComponent.K2_GetComponentLocation` _motionwarpinglocation) (`SceneComponent.K2_GetComponentRotation` _motionwarpinglocation)))
        (`|PlayMontage` (`Character.Mesh` (`self.Player`)) "/Game/Assets/Player/Ghunter/Anims/CollectResource/Skewer/AM_SkewerResource.AM_SkewerResource"
          (:`then`
            (`KismetSystemLibrary.Delay` 0.7)
            (`NiagaraFunctionLibrary.SpawnSystemAtLocation` "/Game/Assets/Actors/Resources/VFX/NS_ResourceFryBreak.NS_ResourceFryBreak" (`SceneComponent.GetSocketLocation` (`Character.Mesh` (`self.Player`)) "Melee_VFX_Socket"))
            (`KismetSystemLibrary.Delay` 0.15)
            (`|SpawnActorFromClass` "/Game/Assets/Actors/Resources/VFX/BP_DropFry.BP_DropFry_C" (`KismetMathLibrary.Conv_VectorToTransform` (`SceneComponent.K2_GetComponentLocation` (`self.MotionWarpingLocation`))) "Undefined" "MultiplyWithRoot" null null)
            (`GameplayStatics.PlaySoundAtLocation` "/Game/Assets/Weapons/Fried/S_ResourcePickUp.S_ResourcePickUp" (`self.K2_GetActorLocation`) (struct) 1.0 1.0 0.0 null null null null))
          (:`OnBlendOut`
            (`self.CE_EndResourceAnimation` :!label _label))
          (:`OnInterrupted`
            (goto _label)))
        (else
          ;;[1 0 0] Cannot pick Resource Sound
          (`GameplayStatics.PlaySoundAtLocation` null (`self.K2_GetActorLocation`) (struct) 1.0 1.0 0.0 null null null null)
          (`PlayerCharacter.DisplayNotificationPopUp` (`self.Player`) (struct :`TagName` "Notification.FullInventory")))))))

(event `CE_EndResourceAnimation`
  (bind _player (`self.Player`))
  ;[1 0.9507 0] INTERACT
  ;;[1 0 0] EndAnimation
  (`AbilitySystemBlueprintLibrary.RemoveLooseGameplayTags` _player (`self.WeaponsBlockedTag`))
  (`WeaponComponent.ChangeWeaponToRange` (`PlayerCharacter.WeaponComponent` _player))
  (`self.CE_AddAmmo`)
  (`self.K2_DestroyActor`))

(event `self.ResourceTrigger.OnComponentBeginOverlap`
  (params (OverlappedComponent :type "PrimitiveComponent Object Reference") (OtherActor :type "Actor Object Reference") (OtherComp :type "PrimitiveComponent Object Reference") (OtherBodyIndex :type Integer) (bFromSweep :type Boolean) (SweepResult :type "HitResult Structure (by ref)"))
  ;[0.9617 0.4084 1] PLAYE DETECTION
  (bind _asplayer_character (cast `PlayerCharacter` OtherActor))
  (set `self.PlayerInside` true)
  (set `self.Player` _asplayer_character)
  (bind _values (`BlueprintMapLibrary.Map_Values` (`TT_GameInstance.WeaponsLevel` (`self.TTGameInstance`))))
  (if (<= (`self.MeleeTierRequired`) (`KismetMathLibrary.Conv_ByteToInt` (`|GetArrayItem` _values)))
    (`MeshComponent.SetOverlayMaterial` (`self.ResourceSkeletalMesh`) (`self.HighlightMaterial`))))

(event `self.ResourceTrigger.OnComponentEndOverlap`
  (params (OverlappedComponent :type "PrimitiveComponent Object Reference") (OtherActor :type "Actor Object Reference") (OtherComp :type "PrimitiveComponent Object Reference") (OtherBodyIndex :type Integer))
  ;[0.9617 0.4084 1] PLAYE DETECTION
  (cast `PlayerCharacter` OtherActor)
  (set `self.PlayerInside` false)
  (`MeshComponent.SetOverlayMaterial` (`self.ResourceSkeletalMesh`) null))

(event `CE_AddAmmo`
  (bind _player (`self.Player`))
  (bind _returnvalue (`AbilitySystemBlueprintLibrary.GetAbilitySystemComponent` _player))
  (bind (_bsuccessfullyfoundattribute _returnvalue_2) (`AbilitySystemBlueprintLibrary.GetFloatAttributeBaseFromAbilitySystemComponent` _returnvalue (`self.MaxAttribute`)))
  (bind (_bsuccessfullyfoundattribute_2 _returnvalue_3) (`AbilitySystemBlueprintLibrary.GetFloatAttributeBaseFromAbilitySystemComponent` _returnvalue (`self.ValueAttribute`)))
  ;[1 0.1146 0.1146] AddAmmo
  (if _bsuccessfullyfoundattribute
    (if _bsuccessfullyfoundattribute_2
      (if (not (>= _returnvalue_3 _returnvalue_2))
        (`AbilitySystemComponent.BP_ApplyGameplayEffectToSelf` :`self` (`AbilitySystemBlueprintLibrary.GetAbilitySystemComponent` _player) :`GameplayEffectClass` (`self.AmmoEffectToBeApplied`))
        (`GameplayStatics.PlaySoundAtLocation` "/Game/Assets/Music/Player/S_ResourceCollection.S_ResourceCollection" (`self.K2_GetActorLocation`) (struct) 1.0 1.0 0.0 null null null null)))))

(fn `UserConstructionScript`)