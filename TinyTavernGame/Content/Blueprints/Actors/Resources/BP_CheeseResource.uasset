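; Harvestable cheese resource actor that the player slices with a melee montage to gain ammo.
; Overlap tracks the player and highlights the mesh if the melee tier suffices; interacting checks only ammo capacity and the WeaponsBlocked tag.
; Harvesting motion-warps the player, blocks weapons, then after a delay spawns VFX and a drop, restores the ranged weapon, applies an ammo GameplayEffect and destroys itself.
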(event `self.ReceiveBeginPlay`
  ;[0.1102 1 0] Begin Play
  (bind _astt_game_instance (cast `TT_GameInstance` (`GameplayStatics.GetGameInstance`)))
  (set `self.TTGameInstance` _astt_game_instance)
  (bind _aswbp_resource_widget (cast `/Game/Blueprints/UI/HUD/3DHuds/WBP_ResourceWidget` (`WidgetComponent.GetWidget` (`self.ResourceWidget`))))
  (`Image.SetBrushFromTexture` (`/Game/Blueprints/UI/HUD/3DHuds/WBP_ResourceWidget.MeleeImage` _aswbp_resource_widget) (`self.RequiredMeleeImage`) false))

(event `EnhancedInput|/Game/Blueprints/Inputs/InputActions/IA_Interact`
  (params (ActionValue :type Boolean) (ElapsedSeconds :type "Float (double-precision)") (TriggeredSeconds :type "Float (double-precision)") (InputAction :type "InputAction Object Reference" :default "/Game/Blueprints/Inputs/InputActions/IA_Interact.IA_Interact"))
  (bind _returnvalue (`self.K2_GetActorLocation`))
  (bind _player (`self.Player`))
  (bind _playerinside (`self.PlayerInside`))
  (bind _motionwarpinglocation (`self.MotionWarpingLocation`))
  (bind _returnvalue_2 (`AbilitySystemBlueprintLibrary.GetAbilitySystemComponent` (`self.Player`)))
  ;[1 0.9175 0] INTERACT
  (:`Started`
    (if _playerinside
      (if (and _playerinside (< (`.ReturnValue` (`AbilitySystemBlueprintLibrary.GetFloatAttributeBaseFromAbilitySystemComponent` _returnvalue_2 (`self.ValueAttribute`))) (`.ReturnValue` (`AbilitySystemBlueprintLibrary.GetFloatAttributeBaseFromAbilitySystemComponent` _returnvalue_2 (`self.MaxAttribute`)))) (not (`GameplayTagAssetInterface.HasMatchingGameplayTag` _returnvalue_2 (struct :`TagName` "States.WeaponsBlocked"))))
        (set `self.PlayerInside` false)
        ;;[0 0.09699 1] Play Montage, change mesh and disable any other action
        (`AbilitySystemBlueprintLibrary.AddLooseGameplayTags` _player (`self.WeaponsBlockedTag`))
        (`AbilitySystemBlueprintLibrary.RemoveLooseGameplayTags` _player (`self.AimingTag`))
        (`WeaponComponent.ChangeWeaponForDash` (`PlayerCharacter.WeaponComponent` _player))
        (`MotionWarpingComponent.AddOrUpdateWarpTarget` (`PlayerCharacter.PlayerMotionWarping` _player) (make `MotionWarpingTarget` "Cut" (`SceneComponent.K2_GetComponentLocation` _motionwarpinglocation) (`SceneComponent.K2_GetComponentRotation` _motionwarpinglocation)))
        (`|PlayMontage` (`Character.Mesh` (`self.Player`)) "/Game/Assets/Player/Ghunter/Anims/CollectResource/Slice/AM_SliceResource.AM_SliceResource"
          (:`then`
            (`KismetSystemLibrary.Delay` 0.55)
            (`NiagaraFunctionLibrary.SpawnSystemAtLocation` "/Game/Assets/Ingredients/Cheese/NS_CheeseBreak.NS_CheeseBreak" (`SceneComponent.GetSocketLocation` (`Character.Mesh` (`self.Player`)) "Melee_VFX_Socket"))
            (`|SpawnActorFromClass` "/Game/Blueprints/EffectActors/ResourceDrops/BP_CheeseResourceDrop.BP_CheeseResourceDrop_C" (`KismetMathLibrary.Conv_VectorToTransform` (`SceneComponent.K2_GetComponentLocation` (`self.ResourceSkeletalMesh`))) "Undefined" "MultiplyWithRoot" null null)
            (`GameplayStatics.PlaySoundAtLocation` "/Game/Assets/Music/Player/Ingredients/Cheese/MS_Cheese_Explosion.MS_Cheese_Explosion" _returnvalue (struct) 1.0 1.0 0.0 null null null null)
            (`self.CE_EndResourceAnimation`)
            (`GameplayStatics.PlaySoundAtLocation` "/Game/Assets/Music/Enviroment/Resources/S_CheeseHit.S_CheeseHit" _returnvalue (struct) 1.0 1.0 0.0 null null null null)
            (`self.K2_DestroyActor`)))
        (else
          ;;[1 0 0] Cannot pick Resource(Full Inventory)
          (`GameplayStatics.PlaySoundAtLocation` "/Game/Assets/Music/UI/S_Error.S_Error" (`self.K2_GetActorLocation`) (struct) 1.0 1.0 0.0 null null null null)
          (`PlayerCharacter.DisplayNotificationPopUp` (`self.Player`) (struct :`TagName` "Notification.FullInventory")))))))

(event `CE_EndResourceAnimation`
  (bind _player (`self.Player`))
  ;[1 0.9175 0] INTERACT
  ;;[1 0 0] EndAnimation
  (`AbilitySystemBlueprintLibrary.RemoveLooseGameplayTags` _player (`self.WeaponsBlockedTag`))
  (`WeaponComponent.ChangeWeaponToRange` (`PlayerCharacter.WeaponComponent` _player))
  (`self.Add ammo`))

(event `self.ReceiveActorBeginOverlap`
  (params (OtherActor :type "Actor Object Reference"))
  ;[0.9617 0.4084 1] PLAYER DETECTION
  (bind _asplayer_character (cast `PlayerCharacter` OtherActor))
  (set `self.PlayerInside` true)
  (set `self.Player` _asplayer_character)
  (bind _values (`BlueprintMapLibrary.Map_Values` (`TT_GameInstance.WeaponsLevel` (`self.TTGameInstance`))))
  (if (<= (`self.MeleeTierRequired`) (`KismetMathLibrary.Conv_ByteToInt` (`|GetArrayItem` _values)))
    (`MeshComponent.SetOverlayMaterial` (`self.ResourceSkeletalMesh`) (`self.HighlightMaterial`))))

(event `Add ammo`
  (bind _returnvalue (`AbilitySystemBlueprintLibrary.GetAbilitySystemComponent` (`self.Player`)))
  (bind (_bsuccessfullyfoundattribute _returnvalue_2) (`AbilitySystemBlueprintLibrary.GetFloatAttributeBaseFromAbilitySystemComponent` _returnvalue (`self.ValueAttribute`)))
  (bind (_bsuccessfullyfoundattribute_2 _returnvalue_3) (`AbilitySystemBlueprintLibrary.GetFloatAttributeBaseFromAbilitySystemComponent` _returnvalue (`self.MaxAttribute`)))
  ;[1 1 1] Comment
  (if _bsuccessfullyfoundattribute_2
    (if _bsuccessfullyfoundattribute
      (if (not (>= _returnvalue_2 _returnvalue_3))
        (`AbilitySystemComponent.BP_ApplyGameplayEffectToSelf` :`self` (`AbilitySystemBlueprintLibrary.GetAbilitySystemComponent` (`self.Player`)) :`GameplayEffectClass` (`self.Ammo Effect to be Applied`))
        (`GameplayStatics.PlaySoundAtLocation` "/Game/Assets/Music/Player/S_ResourceCollection.S_ResourceCollection" (`self.K2_GetActorLocation`) (struct) 1.0 1.0 0.0 null null null null)))))

(event `self.ReceiveActorEndOverlap`
  (params (OtherActor :type "Actor Object Reference"))
  ;[0.9617 0.4084 1] PLAYER DETECTION
  (cast `PlayerCharacter` OtherActor)
  (set `self.PlayerInside` false)
  (`MeshComponent.SetOverlayMaterial` (`self.ResourceSkeletalMesh`) null))

(fn `UserConstructionScript`)