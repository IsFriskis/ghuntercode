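; Harvestable grill resource pickup that the player slices to gain grill ammo.
; Overlap highlights the mesh and enables interaction, which checks GAS ammo attributes and the weapons-blocked tag, showing a full-inventory error on failure.
; On success, it blocks weapons, plays a motion-warped slice montage, spawns VFX and BP_DropGrill after a delay, restores the ranged weapon, applies the ammo GameplayEffect and destroys itself.
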(event `self.ReceiveBeginPlay`
  ;[0 1 0.06743] Begin Play
  ;;[1 1 1] Check Gavern Upgrade
  (cast `TT_GameInstance` (`GameplayStatics.GetGameInstance`))
  (set `self.AmmoEffectToBeApplied` "/Game/Blueprints/AbilitySystems/Effects/Resources/GE_AddAmmoGrill.GE_AddAmmoGrill_C"))

(event `EnhancedInput|/Game/Blueprints/Inputs/InputActions/IA_Interact`
  (params (ActionValue :type Boolean) (ElapsedSeconds :type "Float (double-precision)") (TriggeredSeconds :type "Float (double-precision)") (InputAction :type "InputAction Object Reference" :default "/Game/Blueprints/Inputs/InputActions/IA_Interact.IA_Interact"))
  (bind _player (`self.Player`))
  (bind _playerinside (`self.PlayerInside`))
  (bind _motionwarpinglocation (`self.MotionWarpingLocation`))
  (bind _returnvalue (`AbilitySystemBlueprintLibrary.GetAbilitySystemComponent` (`self.Player`)))
  ;[1 0.7786 0] Interaction
  ;;[0.5076 0.4447 1] BOTON INTERACTUAR
  (:`Started`
    (if _playerinside
      ;;[1 0.3294 0.8534] CUANDO PLAYER ESTÁ EN COLISON = TRUE
      (if (and _playerinside (< (`.ReturnValue` (`AbilitySystemBlueprintLibrary.GetFloatAttributeBaseFromAbilitySystemComponent` _returnvalue (`self.ValueAttribute`))) (`.ReturnValue` (`AbilitySystemBlueprintLibrary.GetFloatAttributeBaseFromAbilitySystemComponent` _returnvalue (`self.MaxAttribute`)))) (not (`GameplayTagAssetInterface.HasMatchingGameplayTag` _returnvalue (struct :`TagName` "States.WeaponsBlocked"))))
        (set `self.PlayerInside` false)
        ;;[0 0.09699 1] Play Montage, change mesh and disable any other action
        (`AbilitySystemBlueprintLibrary.AddLooseGameplayTags` _player (`self.WeaponsBlockedTag`))
        (`AbilitySystemBlueprintLibrary.RemoveLooseGameplayTags` _player (`self.AimingTag`))
        (`WeaponComponent.ChangeWeaponForDash` (`PlayerCharacter.WeaponComponent` _player))
        (`MotionWarpingComponent.AddOrUpdateWarpTarget` (`PlayerCharacter.PlayerMotionWarping` _player) (make `MotionWarpingTarget` "Cut" (`SceneComponent.K2_GetComponentLocation` _motionwarpinglocation) (`SceneComponent.K2_GetComponentRotation` _motionwarpinglocation)))
        (`|PlayMontage` (`Character.Mesh` (`self.Player`)) "/Game/Assets/Player/Ghunter/Anims/CollectResource/Slice/AM_SliceResource.AM_SliceResource"
          (:`then`
            (`KismetSystemLibrary.Delay` 0.55)
            (`NiagaraFunctionLibrary.SpawnSystemAtLocation` "/Game/Assets/Actors/Resources/VFX/NS_ResourceGrillDrop.NS_ResourceGrillDrop" (`SceneComponent.GetSocketLocation` (`Character.Mesh` (`self.Player`)) "Melee_VFX_Socket"))
            (`|SpawnActorFromClass` "/Game/Assets/Actors/Resources/VFX/BP_DropGrill.BP_DropGrill_C" (`KismetMathLibrary.Conv_VectorToTransform` (`SceneComponent.K2_GetComponentLocation` (`self.ResourceSkeletalMesh`))) "Undefined" "MultiplyWithRoot" null null)
            ;;[0.1183 0.4303 1] Activo el sonido del objeto
            (`GameplayStatics.PlaySoundAtLocation` "/Game/Assets/Weapons/Fried/S_ResourcePickUp.S_ResourcePickUp" (`self.K2_GetActorLocation`) (struct) 1.0 1.0 0.0 null null null null)
            (`self.CE_EndResourceAnimation`)
            (`MeshComponent.SetOverlayMaterial` (`self.ResourceSkeletalMesh`) null)
            (`self.K2_DestroyActor`)))
        (else
          ;;[1 0 0] Cannot pick Resource (Inventory Full)
          (`GameplayStatics.PlaySoundAtLocation` "/Game/Assets/Music/UI/S_Error.S_Error" (`self.K2_GetActorLocation`) (struct) 1.0 1.0 0.0 null null null null)
          (`PlayerCharacter.DisplayNotificationPopUp` (`self.Player`) (struct :`TagName` "Notification.FullInventory")))))))

(event `CE_EndResourceAnimation`
  (bind _player (`self.Player`))
  ;[1 0.7786 0] Interaction
  ;;[1 0 0] EndAnimation
  (`AbilitySystemBlueprintLibrary.RemoveLooseGameplayTags` _player (`self.WeaponsBlockedTag`))
  (`WeaponComponent.ChangeWeaponToRange` (`PlayerCharacter.WeaponComponent` _player))
  (`self.CE_AddAmmo`))

(event `self.ReceiveActorBeginOverlap`
  (params (OtherActor :type "Actor Object Reference"))
  ;[0.9617 0.4084 1] PLAYER DETECTION
  (bind _asplayer_character (cast `PlayerCharacter` OtherActor))
  (set `self.PlayerInside` true)
  (set `self.Player` _asplayer_character)
  (`MeshComponent.SetOverlayMaterial` (`self.ResourceSkeletalMesh`) "/Game/Assets/Enviroment/Resources/M_GrillHighlight.M_GrillHighlight"))

(event `self.ReceiveActorEndOverlap`
  (params (OtherActor :type "Actor Object Reference"))
  ;[0.9617 0.4084 1] PLAYER DETECTION
  (cast `PlayerCharacter` OtherActor)
  (set `self.PlayerInside` false)
  (`MeshComponent.SetOverlayMaterial` (`self.ResourceSkeletalMesh`) null))

(event `CE_AddAmmo`
  (bind _player (`self.Player`))
  (bind _returnvalue (`AbilitySystemBlueprintLibrary.GetAbilitySystemComponent` _player))
  (bind (_bsuccessfullyfoundattribute _returnvalue_2) (`AbilitySystemBlueprintLibrary.GetFloatAttributeBaseFromAbilitySystemComponent` _returnvalue (`self.MaxAttribute`)))
  (bind (_bsuccessfullyfoundattribute_2 _returnvalue_3) (`AbilitySystemBlueprintLibrary.GetFloatAttributeBaseFromAbilitySystemComponent` _returnvalue (`self.ValueAttribute`)))
  ;[1 0.1146 0.1146] AddAmmo
  (if _bsuccessfullyfoundattribute
    (if _bsuccessfullyfoundattribute_2
      (if (not (>= _returnvalue_3 _returnvalue_2))
        (`AbilitySystemComponent.BP_ApplyGameplayEffectToSelf` :`self` (`AbilitySystemBlueprintLibrary.GetAbilitySystemComponent` _player) :`GameplayEffectClass` (`self.AmmoEffectToBeApplied`))
        (`GameplayStatics.PlaySoundAtLocation` "/Game/Assets/Music/Player/S_ResourceCollection.S_ResourceCollection" (`self.K2_GetActorLocation`) (struct) 1.0 1.0 0.0 null null null null)))))

(fn `UserConstructionScript`)