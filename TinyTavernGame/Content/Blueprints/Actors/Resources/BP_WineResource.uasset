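; Wine resource pickup that the player breaks with a melee weapon to gain ammo.
; Overlap tracks the player and highlights the mesh if their melee tier suffices, while a widget shows the required weapon.
; Interact checks GAS ammo attributes, blocked-weapon tag and tier, showing an error notification on failure.
; Success plays a motion-warped skewer montage with break effects, blocking weapons until it ends, then applies the ammo GameplayEffect and destroys the actor.
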(event `self.ReceiveBeginPlay`
  ;[0.1102 1 0] Begin Play
  (bind _astt_game_instance (cast `TT_GameInstance` (`GameplayStatics.GetGameInstance`)))
  (set `self.TTGameInstance` _astt_game_instance)
  (bind _aswbp_resource_widget (cast `/Game/Blueprints/UI/HUD/3DHuds/WBP_ResourceWidget` (`WidgetComponent.GetWidget` (`self.ResourceWidget`))))
  (`Image.SetBrushFromTexture` (`/Game/Blueprints/UI/HUD/3DHuds/WBP_ResourceWidget.MeleeImage` _aswbp_resource_widget) (`self.RequiredMeleeImage`) false))

(event `EnhancedInput|/Game/Blueprints/Inputs/InputActions/IA_Interact`
  (params (ActionValue :type Boolean) (ElapsedSeconds :type "Float (double-precision)") (TriggeredSeconds :type "Float (double-precision)") (InputAction :type "InputAction Object Reference" :default "/Game/Blueprints/Inputs/InputActions/IA_Interact.IA_Interact"))
  (bind _player (`self.Player`))
  (bind _motionwarpinglocation (`self.MotionWarpingLocation`))
  (bind _playerinside (`self.PlayerInside`))
  (bind _returnvalue (`AbilitySystemBlueprintLibrary.GetAbilitySystemComponent` (`self.Player`)))
  ;[1 0.7206 0] INTERACT
  (:`Started`
    (if _playerinside
      (if (and _playerinside (< (`.ReturnValue` (`AbilitySystemBlueprintLibrary.GetFloatAttributeBaseFromAbilitySystemComponent` _returnvalue (`self.ValueAttribute`))) (`.ReturnValue` (`AbilitySystemBlueprintLibrary.GetFloatAttributeBaseFromAbilitySystemComponent` _returnvalue (`self.MaxAttribute`)))) (not (`GameplayTagAssetInterface.HasMatchingGameplayTag` _returnvalue (struct :`TagName` "States.WeaponsBlocked"))))
        (set `self.PlayerInside` false)
        (bind _values (`BlueprintMapLibrary.Map_Values` (`TT_GameInstance.WeaponsLevel` (`self.TTGameInstance`))))
        (if (<= (`self.MeleeTierRequired`) (`KismetMathLibrary.Conv_ByteToInt` (`|GetArrayItem` _values)))
          ;;[0 0.09699 1] Play Montage, change mesh and disable any other action
          (`AbilitySystemBlueprintLibrary.AddLooseGameplayTags` _player (`self.WeaponsBlockedTag`))
          (`AbilitySystemBlueprintLibrary.RemoveLooseGameplayTags` _player (`self.AimingTag`))
          (`WeaponComponent.ChangeWeaponForDash` (`PlayerCharacter.WeaponComponent` _player))
          (`MotionWarpingComponent.AddOrUpdateWarpTarget` (`PlayerCharacter.PlayerMotionWarping` _player) (make `MotionWarpingTarget` "Cut" (`SceneComponent.K2_GetComponentLocation` _motionwarpinglocation) (`SceneComponent.K2_GetComponentRotation` _motionwarpinglocation)))
          (`|PlayMontage` (`Character.Mesh` (`self.Player`)) "/Game/Assets/Player/Ghunter/Anims/CollectResource/Skewer/AM_SkewerResource.AM_SkewerResource"
            (:`then`
              (`KismetSystemLibrary.Delay` 0.6)
              (`NiagaraFunctionLibrary.SpawnSystemAtLocation` "/Game/Assets/Ingredients/Wine/NS_WineBreak.NS_WineBreak" (`self.K2_GetActorLocation`))
              (`NiagaraFunctionLibrary.SpawnSystemAtLocation` "/Game/Assets/Actors/Resources/VFX/NS_WineDrop.NS_WineDrop" (`self.K2_GetActorLocation`))
              (`GameplayStatics.PlaySoundAtLocation` "/Game/Assets/Music/Player/Ingredients/Wine/S_WineBreak.S_WineBreak" (`self.K2_GetActorLocation`) (struct) 1.0 1.0 0.0 null null null null))
            (:`OnBlendOut`
              (`self.CE_EndResourceAnimation` :!label _label))
            (:`OnInterrupted`
              (goto _label)))
          (else
            ;;[1 0 0] Cannot pick Resource(No Weapon)
            (`GameplayStatics.PlaySoundAtLocation` "/Game/Assets/Music/UI/S_Error.S_Error" (`self.K2_GetActorLocation`) (struct) 1.0 1.0 0.0 null null null null)
            (`PlayerCharacter.DisplayNotificationPopUp` (`self.Player`) (struct :`TagName` "Notification.NeedAnotherMelee"))))
        (else
          ;;[1 0 0] Cannot pick Resource(Full Inventory)
          (`GameplayStatics.PlaySoundAtLocation` "/Game/Assets/Music/UI/S_Error.S_Error" (`self.K2_GetActorLocation`) (struct) 1.0 1.0 0.0 null null null null)
          (`PlayerCharacter.DisplayNotificationPopUp` (`self.Player`) (struct :`TagName` "Notification.FullInventory")))))))

(event `CE_EndResourceAnimation`
  (bind _player (`self.Player`))
  ;[1 0.7206 0] INTERACT
  ;;[1 0 0] EndAnimation
  (`AbilitySystemBlueprintLibrary.RemoveLooseGameplayTags` _player (`self.WeaponsBlockedTag`))
  (`WeaponComponent.ChangeWeaponToRange` (`PlayerCharacter.WeaponComponent` _player))
  (`self.CE_AddAmmo`)
  (`self.K2_DestroyActor`))

(event `CE_AddAmmo`
  (bind _player (`self.Player`))
  (bind _returnvalue (`AbilitySystemBlueprintLibrary.GetAbilitySystemComponent` _player))
  (bind (_bsuccessfullyfoundattribute _returnvalue_2) (`AbilitySystemBlueprintLibrary.GetFloatAttributeBaseFromAbilitySystemComponent` _returnvalue (`self.ValueAttribute`)))
  (bind (_bsuccessfullyfoundattribute_2 _returnvalue_3) (`AbilitySystemBlueprintLibrary.GetFloatAttributeBaseFromAbilitySystemComponent` _returnvalue (`self.MaxAttribute`)))
  ;[1 1 1] Comment
  (if _bsuccessfullyfoundattribute_2
    (if _bsuccessfullyfoundattribute
      (if (not (>= _returnvalue_2 _returnvalue_3))
        (`AbilitySystemComponent.BP_ApplyGameplayEffectToSelf` :`self` (`AbilitySystemBlueprintLibrary.GetAbilitySystemComponent` _player) :`GameplayEffectClass` (`self.Ammo Effect to be Applied`))
        (`GameplayStatics.PlaySoundAtLocation` "/Game/Assets/Music/Player/S_ResourceCollection.S_ResourceCollection" (`self.K2_GetActorLocation`) (struct) 1.0 1.0 0.0 null null null null)))))

(event `self.ReceiveActorBeginOverlap`
  (params (OtherActor :type "Actor Object Reference"))
  ;[0.9617 0.4084 1] PLAYER DETECTION
  (bind _asplayer_character (cast `PlayerCharacter` OtherActor))
  (set `self.PlayerInside` true)
  (set `self.Player` _asplayer_character)
  (bind _values (`BlueprintMapLibrary.Map_Values` (`TT_GameInstance.WeaponsLevel` (`self.TTGameInstance`))))
  (if (<= (`self.MeleeTierRequired`) (`KismetMathLibrary.Conv_ByteToInt` (`|GetArrayItem` _values)))
    (`MeshComponent.SetOverlayMaterial` (`self.ResourceSkeletalMesh`) "/Game/Assets/Enviroment/Resources/M_WineHighlight.M_WineHighlight")))

(event `self.ReceiveActorEndOverlap`
  (params (OtherActor :type "Actor Object Reference"))
  ;[0.9617 0.4084 1] PLAYER DETECTION
  (cast `PlayerCharacter` OtherActor)
  (set `self.PlayerInside` false)
  (`MeshComponent.SetOverlayMaterial` (`self.ResourceSkeletalMesh`) null))

(fn `UserConstructionScript`)