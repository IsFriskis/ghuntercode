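; BP_GrillDropSpawner is a short-lived VFX actor that turns grill resource particles into dropped resource actors.
; It registers itself on the NSResourceGrill Niagara component as the particle data export target, on BeginPlay and in StartParticleGrill, which also activates the effect.
; The ParticleData callback, meant for particle collisions, spawns a BP_GrillResourceDrop with random yaw at each reported position.
; The spawner destroys itself three seconds after BeginPlay.
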(event `self.ReceiveBeginPlay`
  ;[0 1 0.9058] Seteo VFX que una vez llamado se destruye al pasar 3segs
  (`NiagaraComponent.SetVariableObject` (`self.NS_ResourceGrill`) "BP_GrillPickeable" self)
  (`KismetSystemLibrary.Delay` 3.0)
  (`self.K2_DestroyActor`))

(event `self.ReceiveParticleData`
  (params (Data :type "Array of BasicParticleData Structure (by ref)") (NiagaraSystem :type "NiagaraSystem Object Reference") (SimulationPositionOffset :type "Vector Structure (by ref)"))
  ;[1 0.1312 0.677] Cuando colisona suelto recurso
  (for _array_element Data
    (`|SpawnActorFromClass` "/Game/Blueprints/EffectActors/ResourceDrops/BP_GrillResourceDrop.BP_GrillResourceDrop_C" (`KismetMathLibrary.MakeTransform` (`.Position` (break `BasicParticleData` _array_element)) (`KismetMathLibrary.MakeRotator` 0.0 0.0 (`KismetMathLibrary.RandomFloatInRange` 0.0 360.0))) "AlwaysSpawn" "MultiplyWithRoot" null null)))

(fn `StartParticleGrill`
  (`NiagaraComponent.SetVariableObject` (`self.NS_ResourceGrill`) "BP_GrillPickeable" self)
  (`ActorComponent.Activate` (`self.NS_ResourceGrill`) false))

(fn `UserConstructionScript`)