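; BP_Statue is an adventure statue actor that provides the feedback for being solved.
; StatueCompleted activates the dust Niagara effect, plays the solve sound, turns off the shiny particles, and triggers camera shake and controller vibration on the first player.
; StatueAlreadyOpened only deactivates the shiny particles, setting the solved look without replaying the effects.
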(event `self.BP_StatueCompleted`
  (`|ExecutionSequence`
    (:`then_0`
      (`ActorComponent.Activate` (`self.NS_StatueDust`) false)
      (`GameplayStatics.PlaySound2D` "/Game/Assets/Music/Enviroment/Statues/S_StatueSolve.S_StatueSolve" 1.0 1.0 0.0 null null)
      (`ActorComponent.Deactivate` (`self.ShinyParticles`)))
    (:`then_1`
      (`PlayerController.ClientStartCameraShake` :`self` (`GameplayStatics.GetPlayerController` 0) :`Shake` "/Game/Blueprints/Actors/Adventure/Statues/BP_CameraStatueShake.BP_CameraStatueShake_C" :`Scale` 0.6 :`PlaySpace` "World")
      (`PlayerController.K2_ClientPlayForceFeedback` (`GameplayStatics.GetPlayerController` 0) "/Game/Blueprints/Inputs/FF_Vibration.FF_Vibration" "None" false false false))))

(event `self.BP_StatueAlreadyOpened`
  (`ActorComponent.Deactivate` (`self.ShinyParticles`)))

(fn `UserConstructionScript`)