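; Trigger actor in adventure levels that lets the player return to the tavern.
; It creates a return-to-tavern widget on begin play and plays its appear or disappear animation as anything enters or leaves its box.
; Pressing Interact while inside saves ammunition through the game instance and opens the TavernGym level by name.
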(event `self.ReceiveBeginPlay`
  ;[0 0.5 0.1085] Begin Play
  (bind _returnvalue (`|CreateWidget` "/Game/Blueprints/UI/HUD/WBP_ReturnToTavernUI.WBP_ReturnToTavernUI_C"))
  (bind _output_get (set `self.ReturnToTavernUI` _returnvalue))
  (`UserWidget.AddToViewport` _output_get 0))

(event `self.Box.OnComponentBeginOverlap`
  (params (OverlappedComponent :type "PrimitiveComponent Object Reference") (OtherActor :type "Actor Object Reference") (OtherComp :type "PrimitiveComponent Object Reference") (OtherBodyIndex :type Integer) (bFromSweep :type Boolean) (SweepResult :type "HitResult Structure (by ref)"))
  ;[0.5681 0.1562 1] Overlaps
  (set `self.IsInside` true)
  (`/Game/Blueprints/UI/HUD/WBP_ReturnToTavernUI.CE_AppearAnimation` (`self.ReturnToTavernUI`)))

(event `self.Box.OnComponentEndOverlap`
  (params (OverlappedComponent :type "PrimitiveComponent Object Reference") (OtherActor :type "Actor Object Reference") (OtherComp :type "PrimitiveComponent Object Reference") (OtherBodyIndex :type Integer))
  ;[0.5681 0.1562 1] Overlaps
  (set `self.IsInside` false)
  (`/Game/Blueprints/UI/HUD/WBP_ReturnToTavernUI.CE_DissapearAnimation` (`self.ReturnToTavernUI`)))

(event `EnhancedInput|/Game/Blueprints/Inputs/InputActions/IA_Interact`
  (params (ActionValue :type Boolean) (ElapsedSeconds :type "Float (double-precision)") (TriggeredSeconds :type "Float (double-precision)") (InputAction :type "InputAction Object Reference" :default "/Game/Blueprints/Inputs/InputActions/IA_Interact.IA_Interact"))
  ;[1 0.8273 0] Interact
  (:`Triggered`
    (bind _astt_game_instance (cast `TT_GameInstance` (`GameplayStatics.GetGameInstance`)))
    (if (`self.IsInside`)
      (`TT_GameInstance.SaveAmmunition` _astt_game_instance)
      (`GameplayStatics.OpenLevel` "TavernGym"))))

(fn `UserConstructionScript`)