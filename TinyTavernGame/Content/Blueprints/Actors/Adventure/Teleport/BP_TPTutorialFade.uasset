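; Trigger-box actor that takes the player out of the tutorial and into the TavernGym level behind a UI fade.
; The first player overlap plays the FadeOutTuto animation on the top-level WBP_AdventureUI widget and latches IsInside so it cannot retrigger.
; A short one-shot timer then opens the level by name, gated only by a cast to BP_TTGameInstance.
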(event `self.Box.OnComponentBeginOverlap`
  (params (OverlappedComponent :type "PrimitiveComponent Object Reference") (OtherActor :type "Actor Object Reference") (OtherComp :type "PrimitiveComponent Object Reference") (OtherBodyIndex :type Integer) (bFromSweep :type Boolean) (SweepResult :type "HitResult Structure (by ref)"))
  (if (not (`self.IsInside`))
    (cast `PlayerCharacter` OtherActor)
    (bind _foundwidgets (`WidgetBlueprintLibrary.GetAllWidgetsOfClass` "/Game/Blueprints/UI/HUD/AdventureUI/WBP_AdventureUI.WBP_AdventureUI_C"))
    (bind _output (`|GetArrayItem` _foundwidgets))
    ;[1 1 1] Visible Widget
    (`UserWidget.PlayAnimation` _output (`/Game/Blueprints/UI/HUD/AdventureUI/WBP_AdventureUI.FadeOutTuto` _output) 0.0 1 "Forward" 1.0 false)
    (`KismetSystemLibrary.K2_SetTimerDelegate` (delegate `CustomEvent`) 1.5)
    (set `self.IsInside` true)))

(event `CustomEvent`
  (cast `/Game/Blueprints/Game/BP_TTGameInstance` (`GameplayStatics.GetGameInstance`))
  (`GameplayStatics.OpenLevel` "TavernGym"))

(fn `UserConstructionScript`)