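; A single-use faeric healing circle that fully restores the player's health.
; Overlap toggles an interact widget, and interacting requires being inside, below max health, with no shield or weapon-blocking tag.
; Healing applies a GAS effect, clears weapons, blocks dashing and plays a motion-warped montage with VFX, sound, rumble and an achievement call.
; When the montage completes, the ranged weapon returns, dash unblocks and the circle effects shut off.
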(event `self.ReceiveBeginPlay`
  (`Widget.SetVisibility` (`WidgetComponent.GetWidget` (`self.Widget`)) "Hidden"))

(event `self.ReceiveActorBeginOverlap`
  (params (OtherActor :type "Actor Object Reference"))
  (bind _returnvalue (`WidgetComponent.GetWidget` (`self.Widget`)))
  (if (not (`self.used`))
    (bind _asplayer_character (cast `PlayerCharacter` OtherActor))
    (set `self.PlayerCharacter` _asplayer_character)
    ;[1 1 1] Visible Widget
    (set `self.IsInside` true)
    (if (!= _returnvalue null)
      (`Widget.SetVisibility` _returnvalue "Visible"))))

(event `self.ReceiveActorEndOverlap`
  (params (OtherActor :type "Actor Object Reference"))
  (bind _returnvalue (`WidgetComponent.GetWidget` (`self.Widget`)))
  (cast `PlayerCharacter` OtherActor)
  (set `self.IsInside` false)
  ;[1 1 1] Hide Widget
  (if (!= _returnvalue null)
    (`Widget.SetVisibility` _returnvalue "Hidden")))

(event `EnhancedInput|/Game/Blueprints/Inputs/InputActions/IA_Interact`
  (params (ActionValue :type Boolean) (ElapsedSeconds :type "Float (double-precision)") (TriggeredSeconds :type "Float (double-precision)") (InputAction :type "InputAction Object Reference" :default "/Game/Blueprints/Inputs/InputActions/IA_Interact.IA_Interact"))
  (bind _playercharacter (`self.PlayerCharacter`))
  (bind _motionwarping (`self.MotionWarping`))
  (bind _playercharacter_2 (`self.PlayerCharacter`))
  (bind _playercharacter_3 (`self.PlayerCharacter`))
  (bind _returnvalue (`AbilitySystemBlueprintLibrary.GetAbilitySystemComponent` (`self.PlayerCharacter`)))
  (bind _mesh (`Character.Mesh` (`self.PlayerCharacter`)))
  (:`Started`
    (`/Engine/EditorBlueprintResources/StandardMacros.IsValid` _playercharacter_3
      (:`Is Valid`
        (if (`GameplayTagAssetInterface.HasMatchingGameplayTag` (`AbilitySystemBlueprintLibrary.GetAbilitySystemComponent` _playercharacter_3) (struct :`TagName` "States.WeaponsBlocked"))
          _
          (elif (`self.IsInside`)
            (if (and (not (`self.used`)) (< (`.ReturnValue` (`AbilitySystemBlueprintLibrary.GetFloatAttributeBaseFromAbilitySystemComponent` _returnvalue (`self.ValueAttribute`))) (`.ReturnValue` (`AbilitySystemBlueprintLibrary.GetFloatAttributeBaseFromAbilitySystemComponent` _returnvalue (`self.MaxAttribute`)))) (not (`GameplayTagAssetInterface.HasMatchingGameplayTag` _returnvalue (struct :`TagName` "States.PlayerShield"))))
              (`WeaponComponent.ClearWeapons` (`PlayerCharacter.WeaponComponent` _playercharacter_2))
              (`AbilitySystemComponent.BP_ApplyGameplayEffectToSelf` :`self` (`AbilitySystemBlueprintLibrary.GetAbilitySystemComponent` _playercharacter_2) :`GameplayEffectClass` "/Game/Blueprints/EffectActors/Ammo1/GE_HealthFullHeal.GE_HealthFullHeal_C" :`Level` 1.0)
              (`ActorComponent.Activate` (`self.NS_faericcircle2`) true)
              (`MotionWarpingComponent.AddOrUpdateWarpTarget` (`PlayerCharacter.PlayerMotionWarping` (`self.PlayerCharacter`)) (make `MotionWarpingTarget` "Heal" (`SceneComponent.K2_GetComponentLocation` _motionwarping) (`SceneComponent.K2_GetComponentRotation` _motionwarping)))
              (`AbilitySystemBlueprintLibrary.AddLooseGameplayTags` _playercharacter (`self.BlockDash`))
              (`|PlayMontage` (`Character.Mesh` _playercharacter) "/Game/Assets/Player/Ghunter/Anims/AM_GhunterHeal.AM_GhunterHeal"
                (:`then`
                  (`NiagaraFunctionLibrary.SpawnSystemAttached` "/Game/Assets/VFX/NS_Healing.NS_Healing" _mesh "None" (0.0 0.0 0.0) (struct) "KeepRelativeOffset")
                  (set `self.used` true)
                  (`GameplayStatics.PlaySoundAtLocation` "/Game/Assets/Music/Enviroment/S_Curación.S_Curación" (`SceneComponent.K2_GetComponentLocation` _mesh) (struct) 1.0 1.0 0.5 null null null null)
                  (`PlayerController.K2_ClientPlayForceFeedback` (`GameplayStatics.GetPlayerController` 0) "/Game/Blueprints/Inputs/FF_HealVibration.FF_HealVibration" "None" false false false)
                  ;[1 1 1] Achievement
                  (bind _astt_game_instance (cast `TT_GameInstance` (`GameplayStatics.GetGameInstance`)))
                  (`TT_GameInstance.UsedAHealingCircle` _astt_game_instance))
                (:`OnCompleted`
                  (`WeaponComponent.ChangeWeaponToRange` (`PlayerCharacter.WeaponComponent` (`self.PlayerCharacter`)))
                  (`AbilitySystemBlueprintLibrary.RemoveLooseGameplayTags` (`self.PlayerCharacter`) (`self.BlockDash`))
                  (`ActorComponent.Deactivate` (`self.NS_faericcircle2`))
                  (`ActorComponent.Deactivate` (`self.NS_faericcircle`)))))))))))

(fn `UserConstructionScript`)