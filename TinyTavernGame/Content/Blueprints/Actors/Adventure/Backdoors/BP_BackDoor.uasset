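; BP_BackDoor is a one-use lever that opens a back door in adventure areas.
; Overlap shows a prompt widget, and interacting inside disables input, hides the player's weapon and motion-warps them into a lever-pull montage.
; After a delay, dust and sound play while timelines dissolve the lever through a material parameter and move the referenced door actor along Z.
; The lever then destroys itself.
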(event `self.ReceiveActorBeginOverlap`
  (params (OtherActor :type "Actor Object Reference"))
  (if (not (`self.used`))
    (bind _asplayer_character (cast `PlayerCharacter` OtherActor))
    (set `self.Player` _asplayer_character)
    (set `self.IsInside` true)
    ;[1 1 1] Visible Widget
    (`UserWidget.SetColorAndOpacity` (`WidgetComponent.GetWidget` (`self.Widget`)) (make `LinearColor` 1.0 1.0 1.0 1.0))))

(event `self.ReceiveActorEndOverlap`
  (params (OtherActor :type "Actor Object Reference"))
  (cast `PlayerCharacter` OtherActor)
  (set `self.IsInside` false)
  ;[1 1 1] Hide Widget
  (`UserWidget.SetColorAndOpacity` (`WidgetComponent.GetWidget` (`self.Widget`)) (make `LinearColor` 0.0) :!label _label))

(event `EnhancedInput|/Game/Blueprints/Inputs/InputActions/IA_Interact`
  (params (ActionValue :type Boolean) (ElapsedSeconds :type "Float (double-precision)") (TriggeredSeconds :type "Float (double-precision)") (InputAction :type "InputAction Object Reference" :default "/Game/Blueprints/Inputs/InputActions/IA_Interact.IA_Interact"))
  (bind _scene (`self.Scene`))
  (bind _door (`self.Door`))
  (bind _player (`self.Player`))
  (bind _weaponskeletalmesh (`PlayerCharacter.WeaponSkeletalMesh` _player))
  ;[1 0.5597 0.4189] Cuando el jugador interactua y esta dentro del area desactivo los inputs para este BP (y evitar que vuelva a interactuar)
  (:`Triggered`
    (if (`self.IsInside`)
      (`self.DisableInput` null)
      (`|ExecutionSequence`
        (:`then_0`
          (goto _label))
        (:`then_1`
          (`SceneComponent.SetVisibility` _weaponskeletalmesh false false)
          (`MotionWarpingComponent.AddOrUpdateWarpTarget` (`PlayerCharacter.PlayerMotionWarping` _player) (make `MotionWarpingTarget` "WarpTarget" (`SceneComponent.K2_GetComponentLocation` _scene) (`SceneComponent.K2_GetComponentRotation` _scene)))
          (`|PlayMontage` (`Character.Mesh` _player) "/Game/Assets/Player/Ghunter/Anims/Ghunter_Palanca_Montage.Ghunter_Palanca_Montage"
            (:`then`
              (`SkeletalMeshComponent.PlayAnimation` (`self.SkeletalMesh`) "/Game/Assets/Actors/Adventure/Backdoor/Palancanew_Anim.Palancanew_Anim" false)
              (`KismetSystemLibrary.Delay` 2.0)
              (`NiagaraFunctionLibrary.SpawnSystemAtLocation` "/Game/Assets/Actors/Adventure/Statues/VFX/NS_StatueDust_B.NS_StatueDust_B" (+ (`self.K2_GetActorLocation` (`self.Door`)) (0.0 -200.0 0.0)) (struct :`Yaw` 90.0))
              (`GameplayStatics.PlaySoundAtLocation` "/Game/Assets/Music/Enviroment/Statues/S_StatueMove.S_StatueMove" (`self.K2_GetActorLocation`) (struct) 1.0 1.0 0.0 null null null null)
              ;[1 0.4769 0.5872] Con otro Timeline cambio el valor de una variable del material para que se disuelva la estatua de abajo a arriba
              (bind (_direction _newtrack_0) (`Timeline|Timeline_0`)
                (:`Update`
                  (`MeshComponent.SetScalarParameterValueOnMaterials` (`self.Palanca`) "BurnDisappearance" _newtrack_0)
                  ;[0.8448 0.4893 1] En un timeline reduzco un valor para lla posicion Z de bloqueador
                  (bind (_direction_2 _newtrack_0_2) (`Timeline|Timeline`)
                    (:`Update`
                      ;[1 0.849 0.396] En cada Update bajo al bloqueador por el nuevo vector con el valor de la timeline
                      (`self.K2_SetActorLocation` _door (+ (`self.K2_GetActorLocation` _door) (`KismetMathLibrary.MakeVector` 0.0 0.0 _newtrack_0_2)) false false))
                    (:`Finished`
                      ;[0.8743 0.5276 1] Cuando termina la timeline desgtruyo al bloqueador y me destruyo
                      (set `self.used` true)
                      (`self.K2_DestroyActor`))))))
            (:`OnCompleted`
              (`SceneComponent.SetVisibility` _weaponskeletalmesh true false))))))))

(fn `UserConstructionScript`)