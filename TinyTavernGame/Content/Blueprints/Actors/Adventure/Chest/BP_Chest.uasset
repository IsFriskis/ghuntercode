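; Adventure chest actor that the player opens to receive a relic and see the chest UI.
; Trigger overlap caches the player and applies a highlight overlay, which is cleared when the overlap ends.
; ChestFinished motion-warps the player into an opening montage, hides weapons and plays the lid animation, with montage notifies timing the relic and UI reveals.
; ChestAlreadyOpened hides the mesh and deactivates the Niagara effect.
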(event `self.BP_ChestFinished`
  (bind _player (`self.Player`))
  (bind _motionwarping (`self.MotionWarping`))
  ;[1 0.2137 0] Chest Finished
  ;;[1 1 1] Sound
  (`GameplayStatics.PlaySoundAtLocation` "/Game/Assets/Music/Enviroment/Chest/S_ChestOpen.S_ChestOpen" (`self.K2_GetActorLocation`) (struct) 1.0 1.0 0.0 null null null null)
  ;;[1 1 1] Motion Warping
  (`MotionWarpingComponent.AddOrUpdateWarpTarget` (`PlayerCharacter.PlayerMotionWarping` _player) (make `MotionWarpingTarget` "ChestWarp" (`SceneComponent.K2_GetComponentLocation` _motionwarping) (`SceneComponent.K2_GetComponentRotation` _motionwarping)))
  ;;[1 1 1] Hide Weapon, Open Chest Animation, Show Chest UI in middle of animation
  (`WeaponComponent.ClearWeapons` (`PlayerCharacter.WeaponComponent` (`self.Player`)))
  (bind _notifyname (`|PlayMontage` (`Character.Mesh` _player) (`self.ChestMontage`))
    (:`then`
      (`SkeletalMeshComponent.PlayAnimation` (`self.SkeletalMesh`) "/Game/Assets/Actors/Adventure/Chest/Chest_Open.Chest_Open" false)
      (`ActorComponent.Deactivate` (`self.NS_Chest`)))
    (:`OnNotifyBegin`
      (if (== _notifyname "GetRelic")
        (`self.BP_ShowRelic`)
        (else
          (`WeaponComponent.ClearWeapons` (`PlayerCharacter.WeaponComponent` (`self.Player`))))))
    (:`OnNotifyEnd`
      (if (not (== _notifyname "GetRelic"))
        (`self.ShowChestUI`)))))

(event `self.ChestTrigger.OnComponentBeginOverlap`
  (params (OverlappedComponent :type "PrimitiveComponent Object Reference") (OtherActor :type "Actor Object Reference") (OtherComp :type "PrimitiveComponent Object Reference") (OtherBodyIndex :type Integer) (bFromSweep :type Boolean) (SweepResult :type "HitResult Structure (by ref)"))
  ;[1 0.383 0.0367] Overlaps
  (bind _asplayer_character (cast `PlayerCharacter` OtherActor))
  (set `self.Player` _asplayer_character)
  (`MeshComponent.SetOverlayMaterial` (`self.SkeletalMesh`) "/Game/Assets/Enviroment/Resources/M_InteractHighlight.M_InteractHighlight"))

(event `self.ReceiveActorEndOverlap`
  (params (OtherActor :type "Actor Object Reference"))
  ;[1 0.383 0.0367] Overlaps
  (cast `PlayerCharacter` OtherActor)
  (`MeshComponent.SetOverlayMaterial` (`self.SkeletalMesh`) null))

(event `self.BP_ChestAlreadyOpened`
  ;[1 1 1] Chest Already Opened
  (`SceneComponent.SetVisibility` (`self.SkeletalMesh`) false false)
  (`ActorComponent.Deactivate` (`self.NS_Chest`)))

(fn `UserConstructionScript`)