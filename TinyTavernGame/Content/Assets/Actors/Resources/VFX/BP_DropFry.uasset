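; BP_DropFry is a resource-drop VFX actor whose Niagara particles track the player character.
; It registers itself as the Niagara particle export callback and feeds the system a point above the player mesh every tick.
; When any exported particle comes near the player mesh, it raises the system-wide Force variable.
; The actor destroys itself when the system finishes or deactivates.
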(event `self.ReceiveBeginPlay`
  ;[0 1 0.06743] Begin Play
  (`NiagaraComponent.SetVariableObject` (`self.Niagara`) "ParticleCall" self))

(event `self.ReceiveParticleData`
  (params (Data :type "Array of BasicParticleData Structure (by ref)") (NiagaraSystem :type "NiagaraSystem Object Reference") (SimulationPositionOffset :type "Vector Structure (by ref)"))
  ;[1 1 1] Receive ParticleData
  (for _array_element Data
    (if (< (`KismetMathLibrary.VSize` (- (break `BasicParticleData` _array_element) (`SceneComponent.K2_GetComponentLocation` (`Character.Mesh` (`GameplayStatics.GetPlayerCharacter` 0))))) 50.0)
      (`NiagaraComponent.SetNiagaraVariableFloat` (`self.Niagara`) "Force" 2.0))))

(event `self.ReceiveTick`
  (params (DeltaSeconds :type "Float (single-precision)"))
  ;[0.1785 0.1427 1] Tick
  (`NiagaraComponent.SetVariableVec3` (`self.Niagara`) "ActorLocation" (+ (`SceneComponent.K2_GetComponentLocation` (`Character.Mesh` (`GameplayStatics.GetPlayerCharacter` 0))) (0.0 0.0 150.0))))

(event `self.Niagara.OnSystemFinished`
  (params (PSystem :type "NiagaraComponent Object Reference"))
  ;[1 1 1] Destroy
  (`self.K2_DestroyActor` :!label _label))

(event `self.Niagara.OnComponentDeactivated`
  (params (Component :type "ActorComponent Object Reference"))
  ;[1 1 1] Destroy
  (goto _label))

(fn `UserConstructionScript`)