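; BP_Turnip is an actor that moves a turnip mesh along a spline, apparently as a soup ingredient in the environment.
; Each tick it advances a distance by Speed and places the turnip at that local spline point, lowered by a fixed vertical offset.
; Only position follows the path; when Loop is set, the distance resets to the start after passing the spline's end.
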(event `self.ReceiveTick`
  (params (DeltaSeconds :type "Float (single-precision)"))
  (bind _returnvalue (`SplineComponent.GetTransformAtDistanceAlongSpline` (`self.Spline`) (`self.Distance Along Spline`) "Local" false))
  ;[1 1 1] Follow Spline
  (set `self.Distance Along Spline` (+ (* DeltaSeconds (`self.Speed`)) (`self.Distance Along Spline`)))
  (`SceneComponent.K2_SetRelativeLocation` (`self.Turnip`) (`KismetMathLibrary.MakeVector` (.x (.location _returnvalue)) (.y (.location _returnvalue)) (+ (.z (.location _returnvalue)) -90.0)) false false)
  (if (`self.Loop`)
    (if (< (`SplineComponent.GetSplineLength` (`self.Spline`)) (`self.Distance Along Spline`))
      (set `self.Distance Along Spline` 0.0))))

(fn `UserConstructionScript`)